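; BP_AssembleWorkbench is an assembly workbench actor whose interaction box stays disabled until enough parts are unlocked.
; BeginPlay turns off the box's collision, and each UnlockParts call adds an entry to 零件数据 (parts data), enabling collision once 零件数量 (parts count) is reached.
; The construction script places and sizes the box from the BOXTe transform.
; The player overlap handlers are empty stubs, so no assembly logic exists here.
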(event OnComponentBeginOverlap(Box)
  (params (OverlappedComponent :type Primitive%20Component%20Object%20Reference) (OtherActor :type Actor%20Object%20Reference) (OtherComp :type Primitive%20Component%20Object%20Reference) (OtherBodyIndex :type Integer) (bFromSweep :type Boolean) (SweepResult :type Hit%20Result%20Structure%20%28by%20ref%29))
  (if (== OtherActor (Game|GetPlayerCharacter 0))
    _))

(event OnComponentEndOverlap(Box)
  (params (OverlappedComponent :type Primitive%20Component%20Object%20Reference) (OtherActor :type Actor%20Object%20Reference) (OtherComp :type Primitive%20Component%20Object%20Reference) (OtherBodyIndex :type Integer))
  (if (== OtherActor (Game|GetPlayerCharacter 0))
    _))

(event EventBeginPlay
  (Collision|SetCollisionEnabled (Variables|Default|GetBox) "NoCollision"))

(event Collision|EventActorBeginOverlap
  (params (OtherActor :type Actor%20Object%20Reference)))

(event EventTick
  (params (DeltaSeconds :type Float%20%28single-precision%29)))

(event EventUnlockParts
  (Utilities|Array|Add (Variables|Default|Get零件数据) true)
  (if (>= (Utilities|Array|Length (Variables|Default|Get零件数据)) (Variables|Default|Get零件数量))
    (Collision|SetCollisionEnabled (Variables|Default|GetBox) "QueryAndPhysics")))

(fn ConstructionScript
  (bind _box_te (Variables|Default|GetBOX%20Te))
  (bind (_location _rotation _scale) (Math|Transform|BreakTransform _box_te))
  (Transformation|SetRelativeLocation (Variables|Default|GetBox) _location false false)
  (Components|Box|SetBoxExtent (Variables|Default|GetBox) (* _scale "10.000000,10.000000,10.000000") true))