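; BP_CameraAccessories is a placeable accessory actor that takes over the player's view while the player stands inside its trigger Box.
; Overlap begin on the Box sets the actor as the player controller's view target, and overlap end returns the view to the player character.
; The construction script applies the configurable accessory mesh, hides StaticMesh and positions the Box from NewLocation.
; The custom event 显示内容 (show content) is an empty stub.
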(event OnComponentBeginOverlap(Box)
  (params (OverlappedComponent :type Primitive%20Component%20Object%20Reference) (OtherActor :type Actor%20Object%20Reference) (OtherComp :type Primitive%20Component%20Object%20Reference) (OtherBodyIndex :type Integer) (bFromSweep :type Boolean) (SweepResult :type Hit%20Result%20Structure%20%28by%20ref%29))
  (if (== OtherActor (Game|GetPlayerCharacter 0))
    (Game|Player|SetViewTargetwithBlend (Game|GetPlayerController 0) self 0.0 "VTBlend_Linear" 0.0 false)))

(event OnComponentEndOverlap(Box)
  (params (OverlappedComponent :type Primitive%20Component%20Object%20Reference) (OtherActor :type Actor%20Object%20Reference) (OtherComp :type Primitive%20Component%20Object%20Reference) (OtherBodyIndex :type Integer))
  (if (== OtherActor (Game|GetPlayerCharacter 0))
    (Game|Player|SetViewTargetwithBlend (Game|GetPlayerController 0) (Game|GetPlayerCharacter 0) 0.0 "VTBlend_Linear" 0.0 false)))

(event EventBeginPlay)

(event Collision|EventActorBeginOverlap
  (params (OtherActor :type Actor%20Object%20Reference)))

(event EventTick
  (params (DeltaSeconds :type Float%20%28single-precision%29)))

(event Event显示内容)

(fn ConstructionScript
  (Components|StaticMesh|SetStaticMesh (Variables|Default|GetAccessories%20Static%20Mesh) (Variables|Default|GetAccessories%20Mesh))
  (Rendering|SetVisibility (Variables|Default|GetStaticMesh) false false)
  (Transformation|SetRelativeLocation (Variables|Default|GetBox) (Variables|Default|GetNew%20Location) false false))