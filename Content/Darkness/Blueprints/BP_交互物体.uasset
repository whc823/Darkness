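; BP_交互物体 is an interactable item actor with a configurable mesh, a world-space prompt and an item content widget.
; Timelines scale a tip mesh and mouse prompt widget, each reverse able to hand off to the other.
; Tick yaws the prompt widget toward the player pawn.
; An optional BP_Ligst sound actor spawns at BeginPlay; 显示内容 destroys it and fills WBP_物品内容 with item content.
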(event Custom|显示内容
  (bind _aswbp_物品内容 (Utilities|Casting|CastToWBP_物品内容 (UserInterface|GetWidget (Variables|Default|GetWidget1)))
    (:then
      (Default|更新物品内容 _aswbp_物品内容 (Variables|Default|Get物品内容)))
    (:CastFailed
      _))
  (Utilities|IsValid (Variables|Default|Get音效对象)
    (:Is%20Valid
      (Actor|DestroyActor (Variables|Default|Get音效对象)))))

(event Custom|Show%20Tips%20Animation
  (if (not (Variables|Default|GetMouse%20Model？))
    (bind (_direction _新建轨道_0) (Timeline|Tips%20Animation Play)
      (:Update
        (Development|PrintString (Utilities|String|ToString(Float) _新建轨道_0) true true "(R=0.000000,G=0.660000,B=1.000000,A=1.000000)" 2312.0)
        (Transformation|SetRelativeScale3D (Variables|Default|GetTips%20Statcic%20Mesh) (Math|Vector|Lerp(Vector) "0, 0, 0" (Variables|Default|Get提示控件默认缩放) _新建轨道_0)))
      (:Finished
        (switch Utilities|FlowControl|Switch|SwitchonETimelineDirection _direction
          (:Backward
            (if (Variables|Default|GetSwitch%20to%20Mouse)
              (Rendering|SetVisibility (Variables|Default|GetWidget) true true)
              (Rendering|SetVisibility (Variables|Default|GetTips%20Statcic%20Mesh) false false)
              (CallFunction|ShowMouseAnimation))))))))

(event Custom|Hide%20Tips%20Animation
  (params (Switch%20To%20Mouse%20 :type Boolean))
  (Variables|Default|SetSwitch%20to%20Mouse Switch%20To%20Mouse%20)
  (if (not (Variables|Default|GetMouse%20Model？))
    (if (Variables|Default|GetSwitch%20to%20Mouse)
      (Variables|Default|SetMouse%20Model？ true)
      (bind (_direction _新建轨道_0) (Timeline|Tips%20Animation Reverse)
        (:Update
          (Development|PrintString (Utilities|String|ToString(Float) _新建轨道_0) true true "(R=0.000000,G=0.660000,B=1.000000,A=1.000000)" 2312.0)
          (Transformation|SetRelativeScale3D (Variables|Default|GetTips%20Statcic%20Mesh) (Math|Vector|Lerp(Vector) "0, 0, 0" (Variables|Default|Get提示控件默认缩放) _新建轨道_0)))
        (:Finished
          (switch Utilities|FlowControl|Switch|SwitchonETimelineDirection _direction
            (:Backward
              (if (Variables|Default|GetSwitch%20to%20Mouse)
                (Rendering|SetVisibility (Variables|Default|GetWidget) true true)
                (Rendering|SetVisibility (Variables|Default|GetTips%20Statcic%20Mesh) false false)
                (CallFunction|ShowMouseAnimation))))))
      (else
        (Timeline|Tips%20Animation Reverse)))))

(event Custom|Hide%20Mouse%20Animation
  (Variables|Default|SetMouse%20Model？ false)
  (bind (_direction _新建轨道_0) (Timeline|Mouse%20Animation Reverse)
    (:Update
      (Transformation|SetRelativeScale3D (Variables|Default|GetWidget) (Math|Vector|Lerp(Vector) "0, 0, 0" (Variables|Default|Get提示控件默认缩放) _新建轨道_0)))
    (:Finished
      (switch Utilities|FlowControl|Switch|SwitchonETimelineDirection _direction
        (:Backward
          (Rendering|SetVisibility (Variables|Default|GetWidget) false false)
          (Rendering|SetVisibility (Variables|Default|GetTips%20Statcic%20Mesh) true true)
          (CallFunction|ShowTipsAnimation))))))

(event Custom|Show%20Mouse%20Animation
  (bind (_direction _新建轨道_0) (Timeline|Mouse%20Animation Play)
    (:Update
      (Transformation|SetRelativeScale3D (Variables|Default|GetWidget) (Math|Vector|Lerp(Vector) "0, 0, 0" (Variables|Default|Get提示控件默认缩放) _新建轨道_0)))
    (:Finished
      (switch Utilities|FlowControl|Switch|SwitchonETimelineDirection _direction
        (:Backward
          (Rendering|SetVisibility (Variables|Default|GetWidget) false false)
          (Rendering|SetVisibility (Variables|Default|GetTips%20Statcic%20Mesh) true true)
          (CallFunction|ShowTipsAnimation))))))

(event EventBeginPlay
  (Variables|Default|Set提示控件默认缩放 (Variables|/Script/Engine.SceneComponent|GetRelativeScale3D (Variables|Default|GetTips%20Statcic%20Mesh)))
  (Transformation|SetRelativeScale3D (Variables|Default|GetTips%20Statcic%20Mesh) "0, 0, 0")
  (Rendering|SetVisibility (Variables|Default|GetWidget) false false)
  (if (Variables|Default|Get拥有默认音效)
    (CallFunction|生成音效)))

(event Collision|EventActorBeginOverlap
  (params (OtherActor :type Actor%20Object%20Reference)))

(event EventTick
  (params (DeltaSeconds :type Float%20%28single-precision%29))
  (Transformation|SetWorldRotation (Variables|Default|GetWidget) (Math|Rotator|MakeRotator 0.0 0.0 (.Yaw (Math|Rotator|BreakRotator (Math|Rotator|FindLookatRotation (Transformation|GetWorldLocation (Variables|Default|GetWidget)) (Transformation|GetActorLocation (Game|Player|GetPlayerPawn 0)))))) false false))

(fn ConstructionScript
  (Transformation|SetRelativeLocation (Variables|Default|GetTips%20Statcic%20Mesh) (Variables|Default|GetWidget%20Location) false false)
  (Transformation|SetRelativeTransform (Variables|Default|GetWidget1) (Variables|Default|Get物品内容变换) false false)
  (Components|StaticMesh|SetStaticMesh (Variables|Default|GetStaticMesh) (Variables|Default|Get物品模型))
  (Transformation|SetRelativeLocation (Variables|Default|GetSound%20Location%20Cmp) (Variables|Default|GetSound%20Location) false false))

(fn 更新图标
  (params (图像 :type Texture%202D%20Object%20Reference))
  (bind _aswbp_tips_widget (Utilities|Casting|CastToWBP_TipsWidget (UserInterface|GetWidget (Variables|Default|GetWidget))))
  (Default|更新图标 _aswbp_tips_widget 图像))

(fn 生成音效
  (bind _returnvalue (Game|SpawnActorfromClass "/Game/Darkness/Blueprints/BP_Ligst.BP_Ligst_C" (Math|Transform|MakeTransform (Transformation|GetWorldLocation (Variables|Default|GetSound%20Location%20Cmp))) "AlwaysSpawn" "MultiplyWithRoot" 0 (Variables|Default|Get音效) 0))
  (Variables|Default|Set音效对象 _returnvalue))