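; BP_AssembleCamera is a camera assembly target with slots for body, lens, card cover and memory card.
; A preset part overlapping its box is allowed to install, and the mesh matching its PartID has its material override cleared.
; Leaving before installation revokes permission and applies a translucent ghost material.
; The part's install notification unbinds itself and clears that mesh's override again, through a shared helper that sets every material slot.
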(event OnComponentBeginOverlap(Box)
  (params (OverlappedComponent :type Primitive%20Component%20Object%20Reference) (OtherActor :type Actor%20Object%20Reference) (OtherComp :type Primitive%20Component%20Object%20Reference) (OtherBodyIndex :type Integer) (bFromSweep :type Boolean) (SweepResult :type Hit%20Result%20Structure%20%28by%20ref%29))
  (bind _asbp_item_preset_part (Utilities|Casting|CastToBP_Item_PresetPart OtherActor))
  (Variables|/Game/DarknessGame/Blueprint/ItemActor/BP_Item_PresetPart.BP_Item_PresetPart_C|SetAllow%20Installation _asbp_item_preset_part true)
  (CallFunction|设置物体材质 (Utilities|Select :Index (Variables|/Game/DarknessGame/Blueprint/ItemActor/BP_Item_PresetPart.BP_Item_PresetPart_C|GetPart%20ID _asbp_item_preset_part) :Option%200 (Variables|Default|GetStatic%20Mesh%20Camera%20Body) :Option%201 (Variables|Default|GetStatic%20Mesh%20%20Camera%20Lens) :Option%202 (Variables|Default|GetStatic%20Mesh%20Cmaera%20Card%20Cover) :Option%203 (Variables|Default|GetStatic%20Mesh%20Camera%20Memory%20Card)))
  (EventDispatchers|AssignInstallingOntifiction _asbp_item_preset_part (delegate Custom|Installing%20Ontifiction_事件)))

(event OnComponentEndOverlap(Box)
  (params (OverlappedComponent :type Primitive%20Component%20Object%20Reference) (OtherActor :type Actor%20Object%20Reference) (OtherComp :type Primitive%20Component%20Object%20Reference) (OtherBodyIndex :type Integer))
  (bind _asbp_item_preset_part (Utilities|Casting|CastToBP_Item_PresetPart OtherActor))
  (if (not (Variables|/Game/DarknessGame/Blueprint/ItemActor/BP_Item_PresetPart.BP_Item_PresetPart_C|GetInstalling _asbp_item_preset_part))
    (Variables|/Game/DarknessGame/Blueprint/ItemActor/BP_Item_PresetPart.BP_Item_PresetPart_C|SetAllow%20Installation _asbp_item_preset_part false)
    (CallFunction|设置物体材质 (Utilities|Select :Index (Variables|/Game/DarknessGame/Blueprint/ItemActor/BP_Item_PresetPart.BP_Item_PresetPart_C|GetPart%20ID _asbp_item_preset_part) :Option%200 (Variables|Default|GetStatic%20Mesh%20Camera%20Body) :Option%201 (Variables|Default|GetStatic%20Mesh%20%20Camera%20Lens) :Option%202 (Variables|Default|GetStatic%20Mesh%20Cmaera%20Card%20Cover) :Option%203 (Variables|Default|GetStatic%20Mesh%20Camera%20Memory%20Card)) "/Game/DarknessGame/ArtAssets/Materials/M_TranslucentMaterial_Inst.M_TranslucentMaterial_Inst")))

(event Custom|Installing%20Ontifiction_事件
  (params (Prese%20Part%20Actor :type BP%20Item%20Preset%20Part%20Object%20Reference))
  (EventDispatchers|UnbindallEventsfromInstallingOntifiction Prese%20Part%20Actor)
  (CallFunction|设置物体材质 (Utilities|Select :Index (Variables|/Game/DarknessGame/Blueprint/ItemActor/BP_Item_PresetPart.BP_Item_PresetPart_C|GetPart%20ID Prese%20Part%20Actor) :Option%200 (Variables|Default|GetStatic%20Mesh%20Camera%20Body) :Option%201 (Variables|Default|GetStatic%20Mesh%20%20Camera%20Lens) :Option%202 (Variables|Default|GetStatic%20Mesh%20Cmaera%20Card%20Cover) :Option%203 (Variables|Default|GetStatic%20Mesh%20Camera%20Memory%20Card))))

(event EventBeginPlay)

(event Collision|EventActorBeginOverlap
  (params (OtherActor :type Actor%20Object%20Reference)))

(event EventTick
  (params (DeltaSeconds :type Float%20%28single-precision%29)))

(fn ConstructionScript)

(fn 设置物体材质
  (params (Static%20Mesh :type Mesh%20Component%20Object%20Reference) (New%20Material :type Material%20Interface%20Object%20Reference))
  (for (_ _array_index) (Rendering|Material|GetMaterials Static%20Mesh)
    (Rendering|Material|SetMaterial Static%20Mesh _array_index New%20Material)))