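; BP_Hand is a mouse-driven 3D hand that reveals and touches objects, placed by deprojecting the cursor and facing along the camera's forward direction.
; On BeginPlay it attaches a collision-free BP_WorldChanger sphere, which a timeline grows or shrinks during detection.
; A looping timer sphere-traces forward, scaled by that sphere, sending touch messages to the nearest hit and clearing on a miss.
; It also keeps a duplicate-free list of collected part actors.
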(event EventBeginPlay
  (bind _returnvalue (Transformation|GetActorTransform))
  ;[0.15 0.15 0.15 0.5] 生成探测效果球 类 并使用变量进行保存 并附加到 组件上
  (bind _returnvalue_2 (Game|SpawnActorfromClass "/Game/DarknessGame/Blueprint/SphereMaskBlueprints/BP_WorldChanger.BP_WorldChanger_C" (Math|Transform|MakeTransform (.location _returnvalue) (.rotation _returnvalue) "0.100000,0.100000,0.100000") "AlwaysSpawn" "MultiplyWithRoot" 0 0))
  (bind _output_get (Variables|BaseData|Set显示描边球体 _returnvalue_2))
  (Transformation|AttachComponentToComponent _output_get (Variables|Default|GetDetection) "None" "SnapToTarget" "SnapToTarget" "KeepWorld" true)
  ;[0.15 0.15 0.15 0.5] 设置探测球的碰撞为关闭 避免影响后续功能、
  (Collision|SetActorEnableCollision (Variables|BaseData|Get显示描边球体) false)
  ;[0.15 0.15 0.15 0.5] 设置探测球初始值为 0
  (Transformation|SetActorScale3D (Variables|BaseData|Get显示描边球体) "0, 0, 0")
  ;[0.15 0.15 0.15 0.5] 手部探测定时器
  (Utilities|Time|SetTimerbyFunctionName 0 "Hand Touch Funtion" 0.1 true))

(event Collision|EventActorBeginOverlap
  (params (OtherActor :type Actor%20Object%20Reference)))

(event EventTick
  (params (DeltaSeconds :type Float%20%28single-precision%29)))

(event EventHandDetectionEvent
  (params (End%20Detection :type Boolean) (Maximum%20Detection%20Range :type Float%20%28double-precision%29))
  ;[0.4115 0.4115 0.4115] 手部探测范围缩放功能实现
  (if (not End%20Detection)
    (bind _新建轨道_0 (Timeline|时间轴 Play)
      (:Update
        (Transformation|SetActorScale3D (Variables|BaseData|Get显示描边球体) (Math|Vector|Lerp(Vector) "0, 0, 0" (Math|Conversions|ToVector(Float) Maximum%20Detection%20Range) _新建轨道_0))))
    (else
      (Timeline|时间轴 Reverse))))

(fn ConstructionScript)

(fn FilterNearestDistanceFunction
  (params (Filtered%20Data :type Array%20of%20Hit%20Result%20Structures))
  ;[0.15 0.15 0.15 0.5] 计算 数据中距离手 最近的物体计算方法
  (for _array_element Filtered%20Data
    ;;[0.15 0.15 0.15 0.5] 获取扫描到的物体 位置和自己手部的位置 做对比 保存最小距离 初始最小距离用一个比较大的值作为初始值 确保第一个 就是最短距离
    (if (< (Math|Vector|Distance(Vector) (Transformation|GetWorldLocation (Variables|Default|GetHadn%20Static%20Mesh)) (Transformation|GetActorLocation (.HitActor (Collision|BreakHitResult _array_element)))) (LocalVariables|Get距离))
      (LocalVariables|Set距离 (Math|Vector|Distance(Vector) (Transformation|GetWorldLocation (Variables|Default|GetHadn%20Static%20Mesh)) (Transformation|GetActorLocation (.HitActor (Collision|BreakHitResult _array_element)))))
      (LocalVariables|Set当前最近的的物体 (.HitActor (Collision|BreakHitResult _array_element)))))
  ;[0.15 0.15 0.15 0.5] 返回计算得到的Actor
  (return (LocalVariables|Get当前最近的的物体)))

(fn HandTouchFuntion
  (bind _显示描边球体 (Variables|BaseData|Get显示描边球体))
  (bind _arrow1 (Variables|Default|GetArrow1))
  (bind _returnvalue (Transformation|GetWorldLocation _arrow1))
  (bind _returnvalue_2 (Transformation|GetActorScale3D _显示描边球体))
  (bind _x (Math|Vector|BreakVector _returnvalue_2))
  ;[0.15 0.15 0.15 0.5] 计算手部触摸范围
  (bind (_outhits _returnvalue_3) (Collision|MultiSphereTraceForObjects _returnvalue (+ _returnvalue (* (* (Math|Vector|GetForwardVector (Variables|Default|GetArrow1)) (Variables|基本数据|GetHand%20Touch%20Range)) _x)) (* 5.0 _x) (Utilities|Array|MakeArray "ObjectTypeQuery7") false 0 "ForOneFrame"))
  (if _returnvalue_3
    (Variables|基本数据|SetHand%20Touched%20Actor (CallFunction|FilterNearestDistanceFunction _outhits))
    (Class|IAItemCommunicationInterfaces|TriggerTouchEvent(Message) (Variables|基本数据|GetHand%20Touched%20Actor) true)
    (else
      (Utilities|IsValid (Variables|基本数据|GetHand%20Touched%20Actor)
        (:Is%20Valid
          (Class|IAItemCommunicationInterfaces|TriggerTouchEvent(Message) (Variables|基本数据|GetHand%20Touched%20Actor) false)
          (Variables|基本数据|SetHand%20Touched%20Actor 0))
        (:Is%20Not%20Valid
          (Variables|基本数据|SetHand%20Touched%20Actor 0))))))

(fn GetHandTouchItem
  (return (Variables|基本数据|GetHand%20Touched%20Actor)))

(fn GetPart
  (params (Part%20Actor :type Actor%20Object%20Reference))
  (Utilities|IsValid Part%20Actor
    (:Is%20Valid
      (LocalVariables|Set已拥有该零件 false)
      (for _array_element (Variables|Default|GetPart%20Actro%20Data)
        (if (== _array_element Part%20Actor)
          (LocalVariables|Set已拥有该零件 true)))
      (if (not (LocalVariables|Get已拥有该零件))
        (Utilities|Array|Add (Variables|Default|GetPart%20Actro%20Data) Part%20Actor)
        (return (Variables|Default|GetPart%20Actro%20Data))))
    (:Is%20Not%20Valid
      (return (Variables|Default|GetPart%20Actro%20Data)))))

(fn SynchronizeHandDistance
  (params (Hand%20Distance :type Float%20%28double-precision%29))
  (bind _returnvalue (Game|GetPlayerController 0))
  (bind _returnvalue_2 (Game|GetPlayerController 0))
  (bind (_worldlocation _worlddirection) (Game|Player|ConvertMouseLocationToWorldSpace _returnvalue_2))
  (bind _playercameramanager (Variables|/Script/Engine.PlayerController|GetPlayerCameraManager _returnvalue))
  (bind _returnvalue_3 (Transformation|GetActorLocation _playercameramanager))
  ;[0.15 0.15 0.15 0.5] 获取鼠标位置 同步到手（鼠标为2d 手为3d）讲鼠标2d位置 转换到 游戏空间位置 并实时计算 手在游戏空间中的位置 和旋转
  ;;[0.15 0.15 0.15 0.5] 设置位置
  (Transformation|SetActorLocation (+ _worldlocation (* _worlddirection (Math|Conversions|ToVector(Float) Hand%20Distance))) false false)
  ;;[0.15 0.15 0.15 0.5] 设置旋转
  (Transformation|SetActorRotation (Math|Rotator|MakeRotator 0.0 0.0 (.Yaw (Math|Rotator|BreakRotator (Math|Rotator|FindLookatRotation _returnvalue_3 (+ _returnvalue_3 (* (Transformation|GetActorForwardVector _playercameramanager) Hand%20Distance)))))))
  (return true))