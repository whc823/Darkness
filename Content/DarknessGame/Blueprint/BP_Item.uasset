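; BP_Item is an item actor that pairs a configurable mesh with a tips indicator component.
; The construction script applies the mesh and scale, overrides every material slot with M_detection, then positions the tips component and sets its style.
; On Tick, when the tips component shows its second tips mesh, it yaws to face the player pawn.
; A timeline driving the tips component is present but never runs.
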(event EventBeginPlay)

(event Collision|EventActorBeginOverlap
  (params (OtherActor :type Actor%20Object%20Reference)))

(event EventTick
  (params (DeltaSeconds :type Float%20%28single-precision%29))
  (if (== (Variables|/Script/Engine.StaticMeshComponent|GetStaticMesh (Variables|Default|GetCBP_ItemTipsComponent)) "/Game/DarknessGame/ArtAssets/Mesh/SM_SM_TipsStaticMesh02.SM_SM_TipsStaticMesh02")
    (Transformation|SetWorldRotation (Variables|Default|GetCBP_ItemTipsComponent) (Math|Rotator|MakeRotator 0.0 0.0 (.Yaw (Math|Rotator|BreakRotator (Math|Rotator|FindLookatRotation (Transformation|GetWorldLocation (Variables|Default|GetCBP_ItemTipsComponent)) (Transformation|GetActorLocation (Game|Player|GetPlayerPawn 0)))))) false false)))

(fn ConstructionScript
  (Components|StaticMesh|SetStaticMesh (Variables|Default|GetItem%20Static%20Mesh) (Variables|ItemData|GetItem%20Mesh))
  (for (_ _array_index) (Rendering|Material|GetMaterials (Variables|Default|GetItem%20Static%20Mesh))
    (Rendering|Material|SetMaterial (Variables|Default|GetItem%20Static%20Mesh) _array_index "/Game/m_detection.m_detection"))
  (Transformation|SetRelativeScale3D (Variables|Default|GetItem%20Static%20Mesh) (Math|Conversions|ToVector(Float) (Variables|ItemData|GetItem%20Size)))
  (Transformation|SetRelativeLocation (Variables|Default|GetCBP_ItemTipsComponent) (Variables|ItemData|GetItem%20Tips%20Location) false false)
  (Default|SetTipsStyle (Variables|Default|GetCBP_ItemTipsComponent) false))