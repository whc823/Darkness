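; BP_SoundLigst is an interactable sound-emitting actor with a 3D Niagara icon and an on-screen indicator.
; On BeginPlay it plays its assigned sound and adds a WBP_Indicator widget targeting itself to the viewport.
; Each Tick yaws the icon toward the player pawn with a 90-degree offset, keeping pitch and roll.
; Its interaction event removes the indicator and destroys the actor.
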(event OnAudioFinished(Audio))

(event Custom|进行交互
  (Widget|RemovefromParent (Variables|Default|GetWBP_Indicator))
  (Variables|Default|SetWBP_Indicator 0)
  (Actor|DestroyActor))

(event EventBeginPlay
  (Audio|Components|Audio|SetSound (Variables|Default|GetAudio) (Variables|Default|Get音效))
  (Audio|Components|Audio|Play (Variables|Default|GetAudio) 0.0)
  (bind _returnvalue (UserInterface|CreateWidget "/Game/DarknessGame/Blueprint/UMG/WBP_Indicator.WBP_Indicator_C" 0 self))
  (bind _output_get (Variables|Default|SetWBP_Indicator _returnvalue))
  (UserInterface|Viewport|AddtoViewport _output_get 0))

(event Collision|EventActorBeginOverlap
  (params (OtherActor :type Actor%20Object%20Reference)))

(event EventTick
  (params (DeltaSeconds :type Float%20%28single-precision%29))
  (bind _ns_icon3d_ting (Variables|Default|GetNS_Icon3D_Ting))
  (bind _returnvalue (Transformation|GetWorldRotation _ns_icon3d_ting))
  ;[0.15 0.15 0.15 0.5] 为了 保证特效一直面向相机
  (Transformation|SetWorldRotation (Variables|Default|GetNS_Icon3D_Ting) (Math|Rotator|MakeRotator (.roll _returnvalue) (.pitch _returnvalue) (+ (.yaw (Math|Rotator|FindLookatRotation (Transformation|GetActorLocation) (Transformation|GetActorLocation (Game|Player|GetPlayerPawn 0)))) -9e+01)) false false))

(fn ConstructionScript)