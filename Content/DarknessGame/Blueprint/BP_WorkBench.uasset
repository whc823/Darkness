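; BP_WorkBench is a workbench where the player assembles a camera from parts.
; The construction script places the trigger box, view spring arm, part points and assembly-camera transform; BeginPlay spawns BP_AssembleCamera there.
; Player overlap blends the view to the bench, swaps the hand mesh and, given enough part data, spawns preset parts once.
; While inside, axis input yaws the assembly-camera actor; leaving restores view and hand.
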(event OnComponentBeginOverlap(EnterWorkbenchRangeBox)
  (params (OverlappedComponent :type Primitive%20Component%20Object%20Reference) (OtherActor :type Actor%20Object%20Reference) (OtherComp :type Primitive%20Component%20Object%20Reference) (OtherBodyIndex :type Integer) (bFromSweep :type Boolean) (SweepResult :type Hit%20Result%20Structure%20%28by%20ref%29))
  (if (Actor|ActorHasTag OtherActor "Player")
    (Game|Player|SetViewTargetwithBlend (Game|GetPlayerController 0) self (Variables|CameraData|GetCamera%20Blend%20Time) (Variables|CameraData|GetCamera%20Blend%20Function) 0.0 false)
    (Variables|Default|SetPlayer%20Enter true)
    (bind _hand_actor (Class|IBPControllerCommunicationInterface|GetHandActor(Message) (Game|GetPlayerController 0)))
    (Class|HandDataandMerhodCommunicationInterface|SetHandMesh(Message) _hand_actor "/Game/DarknessGame/ArtAssets/Mesh/SM_MaterialSphere.SM_MaterialSphere")
    (bind _part_actor_data (Class|HandDataandMerhodCommunicationInterface|GetPart(Message) _hand_actor))
    (Variables|PartData|SetPart%20Actor%20Data _part_actor_data)
    (Development|PrintString "获取到手部 拿到数据" true true "(R=0.000000,G=0.660000,B=1.000000,A=1.000000)" 231.0)
    (if (>= (Utilities|Array|Length (Variables|PartData|GetPart%20Actor%20Data)) (Utilities|Array|Length (Variables|PartData|GetPart%20Location%20Data)))
      (Utilities|FlowControl|DoOnce false
        (:Completed
          (for (_array_element _array_index) (Variables|Default|GetPart%20Location%20Component%20Data)
            (Game|SpawnActorfromClass "/Game/DarknessGame/Blueprint/ItemActor/BP_Item_PresetPart.BP_Item_PresetPart_C" (Math|Transform|MakeTransform (.Location (Math|Transform|BreakTransform (Transformation|GetWorldTransform _array_element))) (.Rotation (Math|Transform|BreakTransform (Transformation|GetWorldTransform _array_element))) "1.000000,1.000000,1.000000") "AlwaysSpawn" "MultiplyWithRoot" 0 _array_index (Utilities|Select :Index _array_index :Option%200 "/Game/DarknessGame/ArtAssets/Mesh/Level_1_Assets/相机.相机" :Option%201 "/Game/DarknessGame/ArtAssets/Mesh/Level_1_Assets/镜头.镜头" :Option%202 "/Game/DarknessGame/ArtAssets/Mesh/Level_1_Assets/盖子.盖子" :Option%203 "/Game/DarknessGame/ArtAssets/Mesh/Level_1_Assets/内存卡01.内存卡01") 1.0 "0.000000,0.000000,50.000000" 3e+02 0 0))))
      (else
        (Development|PrintString "零件数量错误！！！！！" true true "(R=0.000000,G=0.660000,B=1.000000,A=1.000000)" 231.0)))))

(event OnComponentEndOverlap(EnterWorkbenchRangeBox)
  (params (OverlappedComponent :type Primitive%20Component%20Object%20Reference) (OtherActor :type Actor%20Object%20Reference) (OtherComp :type Primitive%20Component%20Object%20Reference) (OtherBodyIndex :type Integer))
  (if (Actor|ActorHasTag OtherActor "Player")
    (Game|Player|SetViewTargetwithBlend (Game|GetPlayerController 0) (Game|Player|GetPlayerPawn 0) (Variables|CameraData|GetCamera%20Blend%20Time) (Variables|CameraData|GetCamera%20Blend%20Function) 0.0 false)
    (Variables|Default|SetPlayer%20Enter false)
    (bind _hand_actor (Class|IBPControllerCommunicationInterface|GetHandActor(Message) (Game|GetPlayerController 0)))
    (Class|HandDataandMerhodCommunicationInterface|SetHandMesh(Message) _hand_actor "/Game/DarknessGame/ArtAssets/Mesh/Hand/hand.hand")))

(event EventBeginPlay
  (bind _returnvalue (Game|SpawnActorfromClass "/Game/DarknessGame/Blueprint/BP_AssembleCamera.BP_AssembleCamera_C" (Transformation|GetWorldTransform (Variables|Default|GetAssecmble%20Camera%20Transform%20Comp)) "AlwaysSpawn" "MultiplyWithRoot" 0 0))
  (Variables|Default|SetAssemble%20Camera%20Actor _returnvalue))

(event Collision|EventActorBeginOverlap
  (params (OtherActor :type Actor%20Object%20Reference)))

(event EventTick
  (params (DeltaSeconds :type Float%20%28single-precision%29))
  (if (Variables|Default|GetPlayer%20Enter)
    (Class|Actor|AddActorWorldRotation (Variables|Default|GetAssemble%20Camera%20Actor) (Math|Rotator|MakeRotator 0.0 0.0 (* (Class|Actor|GetInputAxisKeyValue) -1.0)))))

(fn ConstructionScript
  (bind _assemble_cmaera_transform (Variables|Default|GetAssemble%20Cmaera%20Transform))
  (bind _work_bench_camera_data (Variables|CameraData|GetWork%20Bench%20Camera%20Data))
  (bind (_location _rotation) (Math|Transform|BreakTransform _work_bench_camera_data))
  (bind (_location_2 _rotation_2 _scale) (Math|Transform|BreakTransform _assemble_cmaera_transform))
  (Components|Box|SetBoxExtent (Variables|Default|GetEnter%20Workbench%20Range%20Box) (Math|Conversions|ToVector(Float) (Variables|EnterRangeData|GetEnter%20Workbench%20Range%20Size)) true)
  (Transformation|SetRelativeLocation (Variables|Default|GetEnter%20Workbench%20Range%20Box) (Variables|EnterRangeData|GetEnter%20Workbench%20Range%20Location) false false)
  (Transformation|SetRelativeLocation (Variables|Default|GetSpringArm) _location false false)
  (Transformation|SetWorldRotation (Variables|Default|GetSpringArm) _rotation false false)
  (Variables|/Script/Engine.SpringArmComponent|SetTargetArmLength (Variables|Default|GetSpringArm) (Variables|CameraData|GetWorl%20Bench%20Camera%20Distance))
  (for _array_element (Variables|PartData|GetPart%20Location%20Data)
    (bind _returnvalue (AddComponent|AddSceneComponent false (Math|Transform|MakeTransform _array_element "0, 0, 0" "1.000000,1.000000,1.000000")))
    (Utilities|Array|Add (Variables|Default|GetPart%20Location%20Component%20Data) _returnvalue))
  (bind _returnvalue_2 (AddComponent|AddSceneComponent false (Math|Transform|MakeTransform _location_2 _rotation_2 _scale)))
  (Variables|Default|SetAssecmble%20Camera%20Transform%20Comp _returnvalue_2))