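; Static mesh component that serves as an item tip marker, with a switchable interaction look.
; It stores its initial relative scale at BeginPlay.
; SetTipsStyle swaps mesh and material based on the InteractionTips flag.
; NewFunction scales the marker from zero to that stored size by Alpha, but its Index branch uses a fixed zero alpha, so it always restores full size.
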(event EventBeginPlay
  (Variables|Default|Set初始大小 (Variables|Default|GetRelativeScale3D)))

(event EventTick
  (params (DeltaSeconds :type Float%20%28single-precision%29)))

(fn SetTipsStyle
  (params (Interaction%20Tips :type Boolean))
  (Components|StaticMesh|SetStaticMesh (select Interaction%20Tips "/Game/DarknessGame/ArtAssets/Mesh/SM_SM_TipsStaticMesh02.SM_SM_TipsStaticMesh02" "/Game/DarknessGame/ArtAssets/Mesh/SM_TipsStaticMesh01.SM_TipsStaticMesh01"))
  (Rendering|Material|SetMaterial 0 (select Interaction%20Tips "/Game/DarknessGame/ArtAssets/Materials/M_ItemTipsMaterial.M_ItemTipsMaterial" "/Game/DarknessGame/ArtAssets/Materials/M_Basic_Wall.M_Basic_Wall")))

(fn NewFunction
  (params (Alpha :type Float%20%28single-precision%29) (Index :type Boolean))
  (Transformation|SetRelativeScale3D (select Index (Math|Vector|Lerp(Vector) (Variables|Default|Get初始大小) "0, 0, 0" 0.0) (Math|Vector|Lerp(Vector) "0, 0, 0" (Variables|Default|Get初始大小) Alpha))))