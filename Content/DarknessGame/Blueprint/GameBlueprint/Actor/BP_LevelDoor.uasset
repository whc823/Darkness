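; Clickable level door actor that either ends the game or sends the player to another level, depending on the game instance's clear flag.
; When cleared, a timeline swings it open, then the view blends to the door, BP_Hand hides and the game-over widget appears.
; Otherwise a locked sound, camera animation and falling monologue chain into SwitchGameLevels.
; A prompt scales in on player overlap, swaps triangle/mouse meshes on touch, and yaws toward the player as a mouse.
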(event OnComponentBeginOverlap(Box)
  (params (OverlappedComponent :type Primitive%20Component%20Object%20Reference) (OtherActor :type Actor%20Object%20Reference) (OtherComp :type Primitive%20Component%20Object%20Reference) (OtherBodyIndex :type Integer) (bFromSweep :type Boolean) (SweepResult :type Hit%20Result%20Structure%20%28by%20ref%29))
  ;[0.15 0.15 0.15 0.5] 玩家进入提示范围进行提示
  (if (Actor|ActorHasTag OtherActor "Player")
    (CallFunction|StartAnimationEvent)))

(event OnComponentEndOverlap(Box)
  (params (OverlappedComponent :type Primitive%20Component%20Object%20Reference) (OtherActor :type Actor%20Object%20Reference) (OtherComp :type Primitive%20Component%20Object%20Reference) (OtherBodyIndex :type Integer))
  ;[0.15 0.15 0.15 0.5] 玩家进入提示范围进行提示
  (if (Actor|ActorHasTag OtherActor "Player")
    (CallFunction|ReverseAnimationEnvetn)))

(event Custom|End%20Touch%20%20Prompt%20Completeion
  ;[0.15 0.15 0.15 0.5] 手部触摸 显示交互提示逻辑
  ;;[0.15 0.15 0.15 0.5] 鼠标变成三角形的过程逻辑
  (EventDispatchers|UnbindallEventsfromAnimtionCompletionNotification)
  (CallFunction|SetTipsStyle false)
  (CallFunction|StartAnimationEvent))

(event Custom|Show%20Triangle
  ;[0.15 0.15 0.15 0.5] 手部触摸 显示交互提示逻辑
  ;;[0.15 0.15 0.15 0.5] 鼠标变成三角形的过程逻辑
  (CallFunction|ReverseAnimationEnvetn)
  (EventDispatchers|AssignAnimtionCompletionNotification (delegate Custom|End%20Touch%20%20Prompt%20Completeion))
  ;;[0.15 0.15 0.15 0.5] 三角形变成鼠标的过程逻辑
  (Utilities|FlowControl|DoOnce false) ; enters at Reset
)

(event Custom|Camer%20Animation%20Over_事件
  (bind _hud (CallFunction|GetGameHUD))
  (Default|PlayPlayerInnerMonologue _hud "Wait— am I falling?! Ahhhhhhhhh/")
  (EventDispatchers|AssignCompletePlayerInnerMonologue _hud (delegate Custom|Complete%20Player%20Inner%20Monologue_事件)))

(event Custom|Start%20Animation%20Event
  (bind _item_tips_component (Variables|Default|GetItem%20Tips%20Component))
  ;[0.15 0.15 0.15 0.5] 提示动画
  (if (Variables|Default|Get运行许可)
    (bind _新建轨道_0 (Timeline|时间轴 PlayFromStart)
      (:Update
        (Utilities|IsValid _item_tips_component
          (:Is%20Valid
            (Transformation|SetRelativeScale3D _item_tips_component (Math|Vector|Lerp(Vector) "0, 0, 0" (Math|Conversions|ToVector(Float) (Variables|Default|GetInitial%20Tips%20Size)) _新建轨道_0)))))
      (:Finished
        (Default|CallAnimtionCompletionNotification)))))

(event Custom|Complete%20Player%20Inner%20Monologue_事件
  (CallFunction|SwitchGameLevels "NewEnumerator3"))

(event Custom|Start%20Touch%20Prompt%20Completeion
  ;[0.15 0.15 0.15 0.5] 手部触摸 显示交互提示逻辑
  ;;[0.15 0.15 0.15 0.5] 三角形变成鼠标的过程逻辑
  (EventDispatchers|UnbindallEventsfromAnimtionCompletionNotification)
  (CallFunction|SetTipsStyle true)
  (CallFunction|StartAnimationEvent))

(event Custom|Reverse%20Animation%20Envetn
  (bind _item_tips_component (Variables|Default|GetItem%20Tips%20Component))
  ;[0.15 0.15 0.15 0.5] 提示动画
  (if (Variables|Default|Get运行许可)
    (bind _新建轨道_0 (Timeline|时间轴 ReverseFromEnd)
      (:Update
        (Utilities|IsValid _item_tips_component
          (:Is%20Valid
            (Transformation|SetRelativeScale3D _item_tips_component (Math|Vector|Lerp(Vector) "0, 0, 0" (Math|Conversions|ToVector(Float) (Variables|Default|GetInitial%20Tips%20Size)) _新建轨道_0)))))
      (:Finished
        (Default|CallAnimtionCompletionNotification)))))

(event Custom|CustomEvent
  (CallFunction|SwitchGameLevels "NewEnumerator3"))

(event Custom|Show%20Mouse
  ;[0.15 0.15 0.15 0.5] 手部触摸 显示交互提示逻辑
  ;;[0.15 0.15 0.15 0.5] 三角形变成鼠标的过程逻辑
  (CallFunction|ReverseAnimationEnvetn)
  (EventDispatchers|BindEventtoAnimtionCompletionNotification (delegate Custom|Start%20Touch%20Prompt%20Completeion))
  ;;[0.15 0.15 0.15 0.5] 鼠标变成三角形的过程逻辑
  (Utilities|FlowControl|DoOnce false) ; enters at Reset
)

(event EventBeginPlay
  (bind _asbp_darkenss_game_instance (Utilities|Casting|CastToBP_DarkenssGameInstance (Game|GetGameInstance)))
  (Variables|Default|SetDarkenss%20Game%20Instance _asbp_darkenss_game_instance)
  (Transformation|SetRelativeScale3D (Variables|Default|GetItem%20Tips%20Component) "0, 0, 0"))

(event Collision|EventActorBeginOverlap
  (params (OtherActor :type Actor%20Object%20Reference)))

(event EventTick
  (params (DeltaSeconds :type Float%20%28single-precision%29))
  (if (== (Variables|/Script/Engine.StaticMeshComponent|GetStaticMesh (Variables|Default|GetItem%20Tips%20Component)) "/Game/DarknessGame/ArtAssets/Mesh/SM_SM_TipsStaticMesh02.SM_SM_TipsStaticMesh02")
    (Transformation|SetWorldRotation (Variables|Default|GetItem%20Tips%20Component) (Math|Rotator|MakeRotator 0.0 0.0 (.Yaw (Math|Rotator|BreakRotator (Math|Rotator|FindLookatRotation (Transformation|GetWorldLocation (Variables|Default|GetItem%20Tips%20Component)) (Transformation|GetActorLocation (Game|Player|GetPlayerPawn 0)))))) false false)))

(event EventTriggerTouchEvent
  (params (Trigger :type Boolean))
  ;[0.15 0.15 0.15 0.5] 手部触摸 显示交互提示逻辑
  (if (Variables|Default|Get运行许可)
    (if Trigger
      ;;[0.15 0.15 0.15 0.5] 三角形变成鼠标的过程逻辑
      (Utilities|FlowControl|DoOnce false :!label _label
        (:Completed
          (CallFunction|ReverseAnimationEnvetn)
          (EventDispatchers|BindEventtoAnimtionCompletionNotification (delegate Custom|Start%20Touch%20Prompt%20Completeion))
          (goto _label_2 Reset)))
      (else
        ;;[0.15 0.15 0.15 0.5] 鼠标变成三角形的过程逻辑
        (Utilities|FlowControl|DoOnce false :!label _label_2
          (:Completed
            (CallFunction|ReverseAnimationEnvetn)
            (EventDispatchers|AssignAnimtionCompletionNotification (delegate Custom|End%20Touch%20%20Prompt%20Completeion))
            (goto _label Reset)))))))

(event EventMouseClickEvent
  (params (Hand%20Actor :type Actor%20Object%20Reference))
  (if (Variables|/Game/DarknessGame/Blueprint/GameBlueprint/BP_DarkenssGameInstance.BP_DarkenssGameInstance_C|Get通关 (Variables|Default|GetDarkenss%20Game%20Instance))
    (Audio|PlaySound2D "/Game/D_SFX/门/门打开.门打开" 1.0 1.0 0.0 0 0)
    (bind _新建轨道_0 (Timeline|Open%20The%20Door%20Animation PlayFromStart)
      (:Update
        (Transformation|SetRelativeRotation (Variables|Default|GetSM_Doorway_Door) (Math|Rotator|MakeRotator 0.0 0.0 _新建轨道_0) false false))
      (:Finished
        (Game|Player|SetViewTargetwithBlend (Game|GetPlayerController 0) self 5.0 "VTBlend_Linear" 0.0 false)
        (bind _returnvalue (Actor|GetActorOfClass "/Game/DarknessGame/Blueprint/GameBlueprint/Actor/BP_Hand.BP_Hand_C"))
        (Rendering|SetActorHiddenInGame _returnvalue true)
        (Utilities|FlowControl|Delay 5.0)
        (bind _returnvalue_2 (UserInterface|CreateWidget "/Game/DarknessGame/Blueprint/GameBlueprint/Actor/WBP_GameOverTips.WBP_GameOverTips_C"))
        (UserInterface|Viewport|AddtoViewport _returnvalue_2 0)))
    (else
      (Audio|PlaySound2D "/Game/D_SFX/门/门上锁.门上锁" 1.0 1.0 0.0 0 0)
      (bind _player_character (CallFunction|PlayPlayerCameraAniatmion true))
      (EventDispatchers|AssignCamerAnimationOver _player_character (delegate Custom|Camer%20Animation%20Over_事件)))))

(fn ConstructionScript
  (Transformation|SetRelativeTransform (Variables|Default|GetCamera) (Variables|Default|GetCamera%20Location) false false)
  (Transformation|SetRelativeLocation (Variables|Default|GetItem%20Tips%20Component) (Variables|Default|GetItem%20Tips%20Location) false false)
  (CallFunction|SetTipsStyle false)
  (Components|Box|SetBoxExtent (Variables|Default|GetBox) (Math|Conversions|ToVector(Float) (Variables|Default|GetPerception%20Player%20Range)) true))

(fn SetTipsStyle
  (params (Interaction%20Tips :type Boolean))
  (Utilities|IsValid (Variables|Default|GetItem%20Tips%20Component)
    (:Is%20Valid
      (Components|StaticMesh|SetStaticMesh (Variables|Default|GetItem%20Tips%20Component) (select Interaction%20Tips "/Game/DarknessGame/ArtAssets/Mesh/SM_SM_TipsStaticMesh02.SM_SM_TipsStaticMesh02" "/Game/DarknessGame/ArtAssets/Mesh/SM_TipsStaticMesh01.SM_TipsStaticMesh01"))
      (Rendering|Material|SetMaterial (Variables|Default|GetItem%20Tips%20Component) 0 (select Interaction%20Tips "/Game/DarknessGame/ArtAssets/Materials/M_ItemTipsMaterial.M_ItemTipsMaterial" "/Game/DarknessGame/ArtAssets/Materials/M_Basic_Wall.M_Basic_Wall")))))

(fn GetItemData
  (return "" ""))