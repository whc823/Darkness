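; Combination safe that the player opens by clicking left, right, reset and handle parts.
; While a character is inside its sphere, controller click notifications feed the hand's hit component tag into timeline-driven button and wheel animations.
; Turns are stored as booleans and checked against the correct sequence at the handle.
; Opening swings the door, may play a first-time monologue, updates matching items and saves the unlock in the GameInstance, reopening on BeginPlay.
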(event OnComponentBeginOverlap(Sphere_0)
  (params (OverlappedComponent :type Primitive%20Component%20Object%20Reference) (OtherActor :type Actor%20Object%20Reference) (OtherComp :type Primitive%20Component%20Object%20Reference) (OtherBodyIndex :type Integer) (bFromSweep :type Boolean) (SweepResult :type Hit%20Result%20Structure%20%28by%20ref%29))
  ;[0.15 0.15 0.15 0.5] 进入密码箱范围 绑定鼠标左键按键通知
  (Utilities|Casting|CastToCharacter OtherActor)
  (bind _asbp_darkenss_player_controller (Utilities|Casting|CastToBP_DarkenssPlayerController (Game|GetPlayerController 0)))
  (EventDispatchers|AssignLeftClickNotification _asbp_darkenss_player_controller (delegate Custom|Left%20Click%20Notification_事件))
  (EventDispatchers|AssignUpLeftClickNotification _asbp_darkenss_player_controller (delegate Custom|Up%20Left%20Click%20Notification_事件)))

(event OnComponentEndOverlap(Sphere_0)
  (params (OverlappedComponent :type Primitive%20Component%20Object%20Reference) (OtherActor :type Actor%20Object%20Reference) (OtherComp :type Primitive%20Component%20Object%20Reference) (OtherBodyIndex :type Integer))
  ;[0.15 0.15 0.15 0.5] 进入密码箱范围 绑定鼠标左键按键通知
  (Utilities|Casting|CastToCharacter OtherActor)
  (bind _asbp_darkenss_player_controller (Utilities|Casting|CastToBP_DarkenssPlayerController (Game|GetPlayerController 0)))
  (EventDispatchers|UnbindallEventsfromLeftClickNotification _asbp_darkenss_player_controller)
  (EventDispatchers|UnbindallEventsfromUpLeftClickNotification _asbp_darkenss_player_controller))

(event Custom|Left%20Click%20Notification_事件
  (params (Hand :type Actor%20Object%20Reference))
  ;[0.15 0.15 0.15 0.5] 密码旋转逻辑
  (Utilities|FlowControl|DoOnce false
    (:Completed
      (if (not (Variables|Default|GetAnimationing?))
        (bind _hit_compcont (Class|HandDataandMerhodCommunicationInterface|GetHandTouchItem(Message) Hand))
        (Utilities|IsValid _hit_compcont
          (:Is%20Valid
            (if (Components|ComponentHasTag _hit_compcont "向左")
              (CallFunction|ButtonAnimation (Variables|Default|GetLeft%20Buttion) true true false)
              (Utilities|Array|Add (Variables|Default|Get密码内容) true)
              (Audio|PlaySound2D "/Game/D_SFX/保险箱/保险箱点击按钮.保险箱点击按钮" 1.0 1.0 0.0 0 0)
              (elif (Components|ComponentHasTag _hit_compcont "向右")
                (CallFunction|ButtonAnimation (Variables|Default|GetRight%20Button) true false false)
                (Utilities|Array|Add (Variables|Default|Get密码内容) false)
                (Audio|PlaySound2D "/Game/D_SFX/保险箱/保险箱点击按钮.保险箱点击按钮" 1.0 1.0 0.0 0 0)
                (elif (Components|ComponentHasTag _hit_compcont "重置")
                  (CallFunction|ButtonAnimation (Variables|Default|Get立方体_001) false false true)
                  (Utilities|Array|Clear (Variables|Default|Get密码内容))
                  (Audio|PlaySound2D "/Game/D_SFX/保险箱/保险箱点击按钮.保险箱点击按钮" 1.0 1.0 0.0 0 0)
                  (elif (Components|ComponentHasTag _hit_compcont "门把手")
                    (Variables|Default|Set密码错误 false)
                    (for (_array_element _array_index) (Variables|Default|Get密码内容)
                      (if (!= (Utilities|Array|Get(acopy) (Variables|Default|Get正确密码) _array_index) _array_element)
                        (Variables|Default|Set密码错误 true)))
                    (if (!= (Utilities|Array|Length (Variables|Default|Get密码内容)) (Utilities|Array|Length (Variables|Default|Get正确密码)))
                      (Variables|Default|Set密码错误 true))
                    (if (Variables|Default|Get密码错误)
                      (Audio|PlaySound2D "/Game/D_SFX/保险箱/保险箱_机关盒子上锁.保险箱_机关盒子上锁" 1.0 1.0 0.0 0 0)
                      (else
                        (CallFunction|Open)
                        (Audio|PlaySound2D "/Game/D_SFX/保险箱/保险箱打开.保险箱打开" 1.0 1.0 0.0 0 0)))
                    (Utilities|Array|Clear (Variables|Default|Get密码内容))))))))))))

(event Custom|Open
  ;[0.15 0.15 0.15 0.5] 开门动画逻辑
  (bind _新建轨道_1 (Timeline|Open%20Lock%20Box%20Door%20Animation PlayFromStart)
    (:Update
      (Transformation|SetRelativeRotation (Variables|Default|GetLockBox%20Door) (Math|Rotator|Lerp(Rotator) "0, 0, 0" "0.000000,-90.000000,0.000000" _新建轨道_1) false false))
    (:Finished
      (Collision|SetActorEnableCollision false)
      (bind _asbp_darkenss_game_instance (Utilities|Casting|CastToBP_DarkenssGameInstance (Game|GetGameInstance)))
      (if (Variables|/Game/DarknessGame/Blueprint/GameBlueprint/BP_DarkenssGameInstance.BP_DarkenssGameInstance_C|Get第一次任务 _asbp_darkenss_game_instance)
        (bind _outactors (Actor|GetAllActorsOfClass "/Game/DarknessGame/Blueprint/GameBlueprint/ItemActor/BP_Item.BP_Item_C"))
        (for _array_element _outactors
          (if (Utilities|Enum|Equal(Enum) (.ItemType (Utilities|Struct|BreakItemStruct (Variables|/Game/DarknessGame/Blueprint/GameBlueprint/ItemActor/BP_Item.BP_Item_C|GetItem%20Data _array_element))) "NewEnumerator6")
            (Default|刷新物体交互状态 _array_element false false)
            (Default|SpawnSoundFunction _array_element)))
        (bind _asbp_darkenss_game_instance_2 (Utilities|Casting|CastToBP_DarkenssGameInstance (Game|GetGameInstance)))
        (Variables|/Game/DarknessGame/Blueprint/GameBlueprint/BP_DarkenssGameInstance.BP_DarkenssGameInstance_C|SetUnlocked%20Safe _asbp_darkenss_game_instance_2 true)
        (else
          (Variables|/Game/DarknessGame/Blueprint/GameBlueprint/BP_DarkenssGameInstance.BP_DarkenssGameInstance_C|Set第一次任务 _asbp_darkenss_game_instance true)
          (bind _asbp_darkenss_player_pawn (Utilities|Casting|CastToBP_DarkenssPlayerPawn (Game|GetPlayerCharacter 0)))
          (Default|内心独白 _asbp_darkenss_player_pawn "Who would put a phone inside a safe/" "(R=1.000000,G=1.000000,B=1.000000,A=1.000000)")
          (EventDispatchers|Assign完成动画 (Variables|/Game/DarknessGame/Blueprint/GameBlueprint/BP_DarkenssPlayerPawn.BP_DarkenssPlayerPawn_C|Get内心独白控件 _asbp_darkenss_player_pawn) (delegate Custom|完成动画_事件)))))))

(event Custom|已开启密码箱
  ;[0.15 0.15 0.15 0.5] 进入密码箱范围 绑定鼠标左键按键通知
  (bind _asbp_darkenss_player_controller (Utilities|Casting|CastToBP_DarkenssPlayerController (Game|GetPlayerController 0)))
  (EventDispatchers|UnbindallEventsfromLeftClickNotification _asbp_darkenss_player_controller)
  (EventDispatchers|UnbindallEventsfromUpLeftClickNotification _asbp_darkenss_player_controller))

(event Custom|Up%20Left%20Click%20Notification_事件
  ;[0.15 0.15 0.15 0.5] 密码旋转逻辑
  (Utilities|FlowControl|DoOnce false) ; enters at Reset
)

(event Custom|完成动画_事件
  (bind _outactors (Actor|GetAllActorsOfClass "/Game/DarknessGame/Blueprint/GameBlueprint/ItemActor/BP_Item.BP_Item_C"))
  (for _array_element _outactors
    (if (Utilities|Enum|Equal(Enum) (.ItemType (Utilities|Struct|BreakItemStruct (Variables|/Game/DarknessGame/Blueprint/GameBlueprint/ItemActor/BP_Item.BP_Item_C|GetItem%20Data _array_element))) "NewEnumerator6")
      (Default|刷新物体交互状态 _array_element false false)
      (Default|SpawnSoundFunction _array_element)))
  (bind _asbp_darkenss_game_instance (Utilities|Casting|CastToBP_DarkenssGameInstance (Game|GetGameInstance)))
  (Variables|/Game/DarknessGame/Blueprint/GameBlueprint/BP_DarkenssGameInstance.BP_DarkenssGameInstance_C|SetUnlocked%20Safe _asbp_darkenss_game_instance true))

(event EventBeginPlay
  (bind _asbp_darkenss_game_instance (Utilities|Casting|CastToBP_DarkenssGameInstance (Game|GetGameInstance)))
  (if (Variables|/Game/DarknessGame/Blueprint/GameBlueprint/BP_DarkenssGameInstance.BP_DarkenssGameInstance_C|GetUnlocked%20Safe _asbp_darkenss_game_instance)
    (CallFunction|Open)))

(event Collision|EventActorBeginOverlap
  (params (OtherActor :type Actor%20Object%20Reference)))

(event Custom|Button%20Animation
  (params (Button :type Primitive%20Component%20Object%20Reference) (Password%20Wheel :type Boolean) (Left%20Password%20Wheel :type Boolean) (Reset%20Password%20Wheel :type Boolean))
  (Variables|Default|SetAnimationing? true)
  (Variables|Default|SetAnimation%20Start%20Location (Variables|/Script/Engine.SceneComponent|GetRelativeLocation Button))
  (bind _新建轨道_1 (Timeline|Animation%20Timer%20Lner PlayFromStart)
    (:Update
      (Transformation|SetRelativeLocation Button (Math|Vector|Lerp(Vector) (Variables|Default|GetAnimation%20Start%20Location) (- (Variables|Default|GetAnimation%20Start%20Location) "0.000000,1.000000,0.000000") _新建轨道_1) false false))
    (:Finished
      (if Password%20Wheel
        (CallFunction|PasswordWheelAnimation Left%20Password%20Wheel)
        (elif Reset%20Password%20Wheel
          (CallFunction|ResetPasswordWheelAnimation)
          (else
            (Variables|Default|SetAnimationing? false)))))))

(event Custom|Password%20Wheel%20Animation
  (params (Left%20Password%20Wheel :type Boolean))
  (bind _returnvalue (select Left%20Password%20Wheel 1e+01 -1e+01))
  (Variables|Default|Set密码轮旋转 (+ (Variables|Default|Get密码轮旋转) _returnvalue))
  (bind _新建轨道_0 (Timeline|时间轴 PlayFromStart)
    (:Update
      (Transformation|SetRelativeRotation (Variables|Default|GetPassword%20Wheel) (Math|Rotator|MakeRotator 0.0 (Math|Float|Lerp (- (Variables|Default|Get密码轮旋转) _returnvalue) (Variables|Default|Get密码轮旋转) _新建轨道_0) 0.0) false false))
    (:Finished
      (Variables|Default|SetAnimationing? false))))

(event Custom|Reset%20Password%20Wheel%20Animation
  (bind _新建轨道_0 (Timeline|Reset%20Password%20Wheel%20Animation%20Lener PlayFromStart)
    (:Update
      (Transformation|SetRelativeRotation (Variables|Default|GetPassword%20Wheel) (Math|Rotator|MakeRotator 0.0 (Math|Float|Lerp (Variables|Default|Get密码轮旋转) 0.0 _新建轨道_0) 0.0) false false))
    (:Finished
      (Variables|Default|Set密码轮旋转 0.0)
      (Variables|Default|SetAnimationing? false))))

(fn ConstructionScript
  (Transformation|SetRelativeTransform (Variables|Default|GetSpawn%20Phone) (Variables|Default|GetSpawn%20Phone%20Transform) false false))