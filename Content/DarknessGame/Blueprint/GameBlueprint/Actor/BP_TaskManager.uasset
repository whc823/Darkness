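; Story task actor that shows a character mesh and dialogue widget for its TaskEnum, driving narrative progression.
; When the dialogue completes, it hides the mesh and plays a task-specific inner monologue on the player pawn, chained through completion delegates.
; Camera and mechanism tasks then play a camera animation and second monologue before opening the next level.
; Other tasks unlock the matching BP_Item, with a sound for Oreo, then destroy the actor.
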(event Custom|完成文字交互_事件
  (Rendering|SetVisibility (Variables|Default|GetStaticMesh) false false)
  (Utilities|FlowControl|Delay 2.0)
  (bind _asbp_darkenss_player_pawn (Utilities|Casting|CastToBP_DarkenssPlayerPawn (Game|GetPlayerCharacter 0)))
  (Default|内心独白 _asbp_darkenss_player_pawn (Utilities|Select :Index (Variables|Default|GetTaskEnum) :NewEnumerator0 "" :NewEnumerator1 "God, John! Let a blind guy take care of Oreo? You can’t be serious/Guess I’d better find her first/" :NewEnumerator2 "Of course I can recognize your voice, Ellie/How could I ever forget/" :NewEnumerator3 "...Dad/Why do those words sound so familiar/And those gifts, from John and Ellie— I remember them/But why do all these memories feel so… blurry/" :NewEnumerator4 "I love you too, mom/It’s always been me— ignoring everything/Shutting it all out, refusing to accept what happened/The puzzle box… it’s been a while/") "(R=1.000000,G=1.000000,B=1.000000,A=1.000000)")
  (EventDispatchers|Assign完成动画 (Variables|/Game/DarknessGame/Blueprint/GameBlueprint/BP_DarkenssPlayerPawn.BP_DarkenssPlayerPawn_C|Get内心独白控件 _asbp_darkenss_player_pawn) (delegate Custom|完成动画_事件)))

(event Custom|完成动画_事件
  (bind _taskenum (Variables|Default|GetTaskEnum))
  (if (Utilities|Enum|Equal(Enum) (Variables|Default|GetTaskEnum) "NewEnumerator4")
    (bind _asbp_darkenss_player_pawn (Utilities|Casting|CastToBP_DarkenssPlayerPawn (Game|GetPlayerCharacter 0)))
    (Default|StartCameraAnimation _asbp_darkenss_player_pawn)
    (EventDispatchers|AssignCamerAnimationOver _asbp_darkenss_player_pawn (delegate Custom|CustomEvent))
    (elif (Utilities|Enum|Equal(Enum) (Variables|Default|GetTaskEnum) "NewEnumerator3")
      (bind _asbp_darkenss_player_pawn_2 (Utilities|Casting|CastToBP_DarkenssPlayerPawn (Game|GetPlayerCharacter 0)))
      (Default|StartCameraAnimation _asbp_darkenss_player_pawn_2)
      (EventDispatchers|AssignCamerAnimationOver _asbp_darkenss_player_pawn_2 (delegate Custom|Camer%20Animation%20Over_事件))
      (else
        (bind _outactors (Actor|GetAllActorsOfClass "/Game/DarknessGame/Blueprint/GameBlueprint/ItemActor/BP_Item.BP_Item_C"))
        (for _array_element _outactors
          (bind _item_table_data (Default|GetItemData _array_element))
          (if (== (.rowname _item_table_data) (select (Utilities|Enum|Equal(Enum) _taskenum "NewEnumerator2") "留声机2" (Utilities|String|EnumtoString _taskenum)))
            (Default|刷新物体交互状态 _array_element false false)
            (if (Utilities|Enum|Equal(Enum) (Variables|Default|GetTaskEnum) "NewEnumerator1")
              (Default|SpawnSoundFunction _array_element))))
        (Actor|DestroyActor)))))

(event Custom|CustomEvent
  (bind _asbp_darkenss_player_pawn (Utilities|Casting|CastToBP_DarkenssPlayerPawn (Game|GetPlayerCharacter 0)))
  (Default|内心独白 _asbp_darkenss_player_pawn "Where will you take me this time/ 
 
What kind of answer will you show me/" "(R=1.000000,G=1.000000,B=1.000000,A=1.000000)")
  (EventDispatchers|Assign完成动画 (Variables|/Game/DarknessGame/Blueprint/GameBlueprint/BP_DarkenssPlayerPawn.BP_DarkenssPlayerPawn_C|Get内心独白控件 _asbp_darkenss_player_pawn) (delegate Custom|CustomEvent_1)))

(event Custom|CustomEvent_1
  (Game|OpenLevel(byName) "MechanismBoxTestMap"))

(event Custom|Camer%20Animation%20Over_事件
  (bind _asbp_darkenss_player_pawn (Utilities|Casting|CastToBP_DarkenssPlayerPawn (Game|GetPlayerCharacter 0)))
  (Default|内心独白 _asbp_darkenss_player_pawn "We are doing this again?!/" "(R=1.000000,G=1.000000,B=1.000000,A=1.000000)")
  (EventDispatchers|Assign完成动画 (Variables|/Game/DarknessGame/Blueprint/GameBlueprint/BP_DarkenssPlayerPawn.BP_DarkenssPlayerPawn_C|Get内心独白控件 _asbp_darkenss_player_pawn) (delegate Custom|完成动画_事件_0)))

(event Custom|完成动画_事件_0
  (Game|OpenLevel(byName) "Level_Bedroom"))

(event EventBeginPlay
  (Components|StaticMesh|SetStaticMesh (Variables|Default|GetStaticMesh) (Utilities|Select :Index (Variables|Default|GetTaskEnum) :NewEnumerator0 0 :NewEnumerator1 "/Game/DarknessGame/ArtAssets/Mesh/Level_2_Assets/人像.人像" :NewEnumerator2 "/Game/DarknessGame/ArtAssets/Mesh/Level_2_Assets/Girl2_2.Girl2_2" :NewEnumerator3 "/Game/DarknessGame/ArtAssets/Mesh/Level_2_Assets/Man.Man" :NewEnumerator4 "/Game/DarknessGame/ArtAssets/Mesh/Level_2_Assets/girl.girl"))
  (bind _aswbp_物品内容 (Utilities|Casting|CastToWBP_物品内容 (UserInterface|GetWidget (Variables|Default|GetStory%20Content%20Widget))))
  (Default|更新物品内容 _aswbp_物品内容 (.Value (Utilities|Map|Find (Variables|Default|GetTask%20Data) (Variables|Default|GetTaskEnum))))
  (EventDispatchers|Assign完成文字交互 _aswbp_物品内容 (delegate Custom|完成文字交互_事件))
  (if (Utilities|Enum|Equal(Enum) (Variables|Default|GetTaskEnum) "NewEnumerator2")
    (Audio|PlaySound2D "/Game/D_SFX/BGM/Livingroom.Livingroom" 1.0 1.0 0.0 0 0)))

(fn ConstructionScript)