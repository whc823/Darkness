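; Workbench actor where the player brings collected parts for assembly, blending the view to its camera while the player is inside its trigger box.
; Entry or a part-collected event reads the hand actor's part data and respawns preview BP_Items at construction-script-built slots.
; A full set also spawns or reveals BP_AssembleCamera, which left-click input yaws while the player is inside.
; Exit or completion restores player view and clears previews; completion also disables the trigger.
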(event OnComponentBeginOverlap(EnterWorkbenchRangeBox)
  (params (OverlappedComponent :type Primitive%20Component%20Object%20Reference) (OtherActor :type Actor%20Object%20Reference) (OtherComp :type Primitive%20Component%20Object%20Reference) (OtherBodyIndex :type Integer) (bFromSweep :type Boolean) (SweepResult :type Hit%20Result%20Structure%20%28by%20ref%29))
  (if (Actor|ActorHasTag OtherActor "Player")
    (Game|Player|SetViewTargetwithBlend (Game|GetPlayerController 0) self (Variables|CameraData|GetCamera%20Blend%20Time) (Variables|CameraData|GetCamera%20Blend%20Function) 0.0 false)
    (Variables|Default|SetPlayer%20Enter true)
    ;[0.15 0.15 0.15 0.5] 音效提示Actor 是否存在 存在则删除
    (Utilities|IsValid (Variables|Default|GetSound%20Lighst%20Actor)
      (:Is%20Valid
        (Actor|DestroyActor (Variables|Default|GetSound%20Lighst%20Actor))
        (Variables|Default|SetSound%20Lighst%20Actor 0))
      (:Is%20Not%20Valid
        _))
    ;[0.15 0.15 0.15 0.5] 获取手部 零件数据
    (Utilities|Array|Clear (Variables|PartData|GetPart%20Data))
    (bind _hand_actor (Class|IBPControllerCommunicationInterface|GetHandActor(Message) (Game|GetPlayerController 0)))
    (Class|HandDataandMerhodCommunicationInterface|SetHandMesh(Message) _hand_actor "/Game/DarknessGame/ArtAssets/Mesh/SM_MaterialSphere.SM_MaterialSphere")
    (bind _part_actor_data (Class|HandDataandMerhodCommunicationInterface|GetPart(Message) _hand_actor))
    (Variables|PartData|SetPart%20Data _part_actor_data)
    (Development|PrintString "获取到手部 拿到数据" true true "(R=0.000000,G=0.660000,B=1.000000,A=1.000000)" 231.0)
    (if (>= (Utilities|Array|Length (Variables|PartData|GetPart%20Data)) (Utilities|Array|Length (Variables|PartData|GetPart%20Location%20Data)))
      ;[0.15 0.15 0.15 0.5] 拥有完整的零件 生成预设体 并绑定完成拼装通知
      (Utilities|IsValid (Variables|Default|GetAssemble%20Camera%20Actor)
        (:Is%20Valid
          (Rendering|SetActorHiddenInGame (Variables|Default|GetAssemble%20Camera%20Actor) false)
          ;[0.15 0.15 0.15 0.5] 清空数据 确保数据为最新数据
          (for _array_element (Variables|Default|GetSpawn%20Preset%20Actor%20Data) :!label _label
            (Utilities|IsValid _array_element
              (:Is%20Valid
                (Actor|DestroyActor _array_element))))
          (Utilities|Array|Clear (Variables|Default|GetSpawn%20Preset%20Actor%20Data))
          ;[0.15 0.15 0.15 0.5] 生成组装零件
          (for (_array_element_2 _array_index) (Variables|PartData|GetPart%20Data)
            (bind _returnvalue (Game|SpawnActorfromClass "/Game/DarknessGame/Blueprint/GameBlueprint/ItemActor/BP_Item.BP_Item_C" (Math|Transform|MakeTransform (.Location (Math|Transform|BreakTransform (Transformation|GetWorldTransform (Utilities|Array|Get(acopy) (Variables|Default|GetPart%20Location%20Component%20Data) _array_index)))) (.Rotation (Math|Transform|BreakTransform (Transformation|GetWorldTransform (Utilities|Array|Get(acopy) (Variables|Default|GetPart%20Location%20Component%20Data) _array_index)))) "1.000000,1.000000,1.000000") "AlwaysSpawn" "MultiplyWithRoot" 0 (Utilities|Struct|MakeDataTableRowHandle 0 "None") (Utilities|Struct|MakeItemStruct (.ItemStaticMehs (Utilities|Struct|BreakItemStruct _array_element_2)) (Utilities|Enum|LiteralenumItemTypeEnum "NewEnumerator5") (.ItemStroyContent (Utilities|Struct|BreakItemStruct _array_element_2)) (.SoundStroy (Utilities|Struct|BreakItemStruct _array_element_2)) (.PartID (Utilities|Struct|BreakItemStruct _array_element_2))) 1.0 "0.000000,0.000000,50.000000" 5e+02 "0.000000,0.000000,0.000000|0.000000,0.000000,-0.000000|1.000000,1.000000,1.000000" false false 0))
            (Utilities|Array|Add (Variables|Default|GetSpawn%20Preset%20Actor%20Data) _returnvalue)))
        (:Is%20Not%20Valid
          (bind _returnvalue_2 (Game|SpawnActorfromClass "/Game/DarknessGame/Blueprint/GameBlueprint/Actor/BP_AssembleCamera.BP_AssembleCamera_C" (Transformation|GetWorldTransform (Variables|Default|GetAssecmble%20Camera%20Transform%20Comp)) "AlwaysSpawn" "MultiplyWithRoot" 0 0))
          (EventDispatchers|AssignCompleteAssemblyNotification _returnvalue_2 (delegate Custom|Complete%20Assembly%20Notification_事件))
          (Variables|Default|SetAssemble%20Camera%20Actor _returnvalue_2)
          (Utilities|FlowControl|Sequence
            (:then_0
              ;[0.15 0.15 0.15 0.5] 生成音效提示对象
              (Utilities|FlowControl|DoOnce false
                (:Completed
                  (bind _returnvalue_3 (Game|SpawnActorfromClass "/Game/DarknessGame/Blueprint/GameBlueprint/Actor/BP_SoundLigst.BP_SoundLigst_C" (Math|Transform|MakeTransform (Transformation|GetActorLocation (Variables|Default|GetAssemble%20Camera%20Actor)) "0, 0, 0" "1.000000,1.000000,1.000000") "AlwaysSpawn" "MultiplyWithRoot" 0 "/Game/DarknessGame/ArtAssets/Sound/视频游戏的声音效果___拾取硬币_Freesound1.视频游戏的声音效果___拾取硬币_Freesound1" 0))
                  (Variables|Default|SetSound%20Lighst%20Actor _returnvalue_3))))
            (:then_1
              (goto _label)))))
      (else
        (Development|PrintString "零件数量错误！！！！！" true true "(R=0.000000,G=0.660000,B=1.000000,A=1.000000)" 231.0)
        (goto _label)))))

(event OnComponentEndOverlap(EnterWorkbenchRangeBox)
  (params (OverlappedComponent :type Primitive%20Component%20Object%20Reference) (OtherActor :type Actor%20Object%20Reference) (OtherComp :type Primitive%20Component%20Object%20Reference) (OtherBodyIndex :type Integer))
  (if (Actor|ActorHasTag OtherActor "Player")
    (Game|Player|SetViewTargetwithBlend (Game|GetPlayerController 0) (Game|Player|GetPlayerPawn 0) (Variables|CameraData|GetCamera%20Blend%20Time) (Variables|CameraData|GetCamera%20Blend%20Function) 0.0 false)
    (Variables|Default|SetPlayer%20Enter false)
    (bind _hand_actor (Class|IBPControllerCommunicationInterface|GetHandActor(Message) (Game|GetPlayerController 0)))
    (Class|HandDataandMerhodCommunicationInterface|SetHandMesh(Message) _hand_actor "/Game/DarknessGame/ArtAssets/Mesh/Hand/hand.hand")
    ;[0.15 0.15 0.15 0.5] 每次离开 工作台 删除零件 确保不会出现多个零件的情况
    (for _array_element (Variables|Default|GetSpawn%20Preset%20Actor%20Data)
      (Utilities|IsValid _array_element
        (:Is%20Valid
          (Actor|DestroyActor _array_element))))
    (Utilities|Array|Clear (Variables|Default|GetSpawn%20Preset%20Actor%20Data))))

(event Custom|Complete%20Assembly%20Notification_事件
  ;[0.15 0.15 0.15 0.5] 完成拼装后执行逻辑
  (Collision|SetCollisionEnabled (Variables|Default|GetEnter%20Workbench%20Range%20Box) "NoCollision")
  (CallFunction|ReturntoPlayerControl))

(event Custom|Return%20to%20Player%20Control
  ;[0.15 0.15 0.15 0.5] 返回玩家事件
  (Game|Player|SetViewTargetwithBlend (Game|GetPlayerController 0) (Game|Player|GetPlayerPawn 0) (Variables|CameraData|GetCamera%20Blend%20Time) (Variables|CameraData|GetCamera%20Blend%20Function) 0.0 false)
  (Variables|Default|SetPlayer%20Enter false)
  (bind _hand_actor (Class|IBPControllerCommunicationInterface|GetHandActor(Message) (Game|GetPlayerController 0)))
  (Class|HandDataandMerhodCommunicationInterface|SetHandMesh(Message) _hand_actor "/Game/DarknessGame/ArtAssets/Mesh/Hand/hand.hand")
  ;[0.15 0.15 0.15 0.5] 每次离开 工作台 删除零件 确保不会出现多个零件的情况
  (for _array_element (Variables|Default|GetSpawn%20Preset%20Actor%20Data)
    (Utilities|IsValid _array_element
      (:Is%20Valid
        (Actor|DestroyActor _array_element))))
  (Utilities|Array|Clear (Variables|Default|GetSpawn%20Preset%20Actor%20Data)))

(event Custom|Collect%20part%20notifications%20Event
  ;[0.15 0.15 0.15 0.5] 收集零件通知 每收集一个零件则通知一次
  (Utilities|Array|Clear (Variables|PartData|GetPart%20Data))
  (bind _hand_actor (Class|IBPControllerCommunicationInterface|GetHandActor(Message) (Game|GetPlayerController 0)))
  (bind _part_actor_data (Class|HandDataandMerhodCommunicationInterface|GetPart(Message) _hand_actor))
  (Variables|PartData|SetPart%20Data _part_actor_data)
  (Development|PrintString "获取到手部 拿到数据" true true "(R=0.000000,G=0.660000,B=1.000000,A=1.000000)" 231.0)
  (if (>= (Utilities|Array|Length (Variables|PartData|GetPart%20Data)) (Utilities|Array|Length (Variables|PartData|GetPart%20Location%20Data)))
    ;[0.15 0.15 0.15 0.5] 拥有完整的零件 生成预设体 并绑定完成拼装通知
    (Utilities|IsValid (Variables|Default|GetAssemble%20Camera%20Actor)
      (:Is%20Valid
        (Rendering|SetActorHiddenInGame (Variables|Default|GetAssemble%20Camera%20Actor) false)
        ;[0.15 0.15 0.15 0.5] 清空数据 确保数据为最新数据
        (for _array_element (Variables|Default|GetSpawn%20Preset%20Actor%20Data) :!label _label
          (Utilities|IsValid _array_element
            (:Is%20Valid
              (Actor|DestroyActor _array_element))))
        (Utilities|Array|Clear (Variables|Default|GetSpawn%20Preset%20Actor%20Data))
        ;[0.15 0.15 0.15 0.5] 生成组装零件
        (for (_array_element_2 _array_index) (Variables|PartData|GetPart%20Data)
          (bind _returnvalue (Game|SpawnActorfromClass "/Game/DarknessGame/Blueprint/GameBlueprint/ItemActor/BP_Item.BP_Item_C" (Math|Transform|MakeTransform (.Location (Math|Transform|BreakTransform (Transformation|GetWorldTransform (Utilities|Array|Get(acopy) (Variables|Default|GetPart%20Location%20Component%20Data) _array_index)))) (.Rotation (Math|Transform|BreakTransform (Transformation|GetWorldTransform (Utilities|Array|Get(acopy) (Variables|Default|GetPart%20Location%20Component%20Data) _array_index)))) "1.000000,1.000000,1.000000") "AlwaysSpawn" "MultiplyWithRoot" 0 (Utilities|Struct|MakeDataTableRowHandle 0 "None") (Utilities|Struct|MakeItemStruct (.ItemStaticMehs (Utilities|Struct|BreakItemStruct _array_element_2)) (Utilities|Enum|LiteralenumItemTypeEnum "NewEnumerator5") (.ItemStroyContent (Utilities|Struct|BreakItemStruct _array_element_2)) (.SoundStroy (Utilities|Struct|BreakItemStruct _array_element_2)) (.PartID (Utilities|Struct|BreakItemStruct _array_element_2))) 1.0 "0.000000,0.000000,50.000000" 5e+02 "0.000000,0.000000,0.000000|0.000000,0.000000,-0.000000|1.000000,1.000000,1.000000" false false 0))
          (Utilities|Array|Add (Variables|Default|GetSpawn%20Preset%20Actor%20Data) _returnvalue)))
      (:Is%20Not%20Valid
        (bind _returnvalue_2 (Game|SpawnActorfromClass "/Game/DarknessGame/Blueprint/GameBlueprint/Actor/BP_AssembleCamera.BP_AssembleCamera_C" (Transformation|GetWorldTransform (Variables|Default|GetAssecmble%20Camera%20Transform%20Comp)) "AlwaysSpawn" "MultiplyWithRoot" 0 0))
        (EventDispatchers|AssignCompleteAssemblyNotification _returnvalue_2 (delegate Custom|Complete%20Assembly%20Notification_事件))
        (Variables|Default|SetAssemble%20Camera%20Actor _returnvalue_2)
        (Utilities|FlowControl|Sequence
          (:then_0
            ;[0.15 0.15 0.15 0.5] 生成音效提示对象
            (Utilities|FlowControl|DoOnce false
              (:Completed
                (bind _returnvalue_3 (Game|SpawnActorfromClass "/Game/DarknessGame/Blueprint/GameBlueprint/Actor/BP_SoundLigst.BP_SoundLigst_C" (Math|Transform|MakeTransform (Transformation|GetActorLocation (Variables|Default|GetAssemble%20Camera%20Actor)) "0, 0, 0" "1.000000,1.000000,1.000000") "AlwaysSpawn" "MultiplyWithRoot" 0 "/Game/DarknessGame/ArtAssets/Sound/视频游戏的声音效果___拾取硬币_Freesound1.视频游戏的声音效果___拾取硬币_Freesound1" 0))
                (Variables|Default|SetSound%20Lighst%20Actor _returnvalue_3))))
          (:then_1
            (goto _label)))))
    (else
      (Development|PrintString "零件数量错误！！！！！" true true "(R=0.000000,G=0.660000,B=1.000000,A=1.000000)" 231.0)
      (goto _label))))

(event Custom|Left%20Click%20Notification_事件
  (params (Hand :type Actor%20Object%20Reference))
  (bind _assemble_camera_actor (Variables|Default|GetAssemble%20Camera%20Actor))
  (if (Variables|Default|GetPlayer%20Enter)
    (Utilities|IsValid _assemble_camera_actor
      (:Is%20Valid
        (Class|Actor|AddActorWorldRotation _assemble_camera_actor (Math|Rotator|MakeRotator 0.0 0.0 (* (Class|Actor|GetInputAxisKeyValue) -2.0)))))))

(event EventBeginPlay
  (bind _asbp_darkenss_player_controller (Utilities|Casting|CastToBP_DarkenssPlayerController (Game|GetPlayerController 0)))
  (EventDispatchers|AssignLeftClickNotification _asbp_darkenss_player_controller (delegate Custom|Left%20Click%20Notification_事件)))

(event EventTick
  (params (DeltaSeconds :type Float%20%28single-precision%29)))

(fn ConstructionScript
  (bind _assemble_cmaera_transform (Variables|Default|GetAssemble%20Cmaera%20Transform))
  (bind _work_bench_camera_data (Variables|CameraData|GetWork%20Bench%20Camera%20Data))
  (bind (_location _rotation) (Math|Transform|BreakTransform _work_bench_camera_data))
  (bind (_location_2 _rotation_2 _scale) (Math|Transform|BreakTransform _assemble_cmaera_transform))
  (Components|Box|SetBoxExtent (Variables|Default|GetEnter%20Workbench%20Range%20Box) (Math|Conversions|ToVector(Float) (Variables|EnterRangeData|GetEnter%20Workbench%20Range%20Size)) true)
  (Transformation|SetRelativeLocation (Variables|Default|GetEnter%20Workbench%20Range%20Box) (Variables|EnterRangeData|GetEnter%20Workbench%20Range%20Location) false false)
  (Transformation|SetRelativeLocation (Variables|Default|GetSpringArm) _location false false)
  (Transformation|SetWorldRotation (Variables|Default|GetSpringArm) _rotation false false)
  (Variables|/Script/Engine.SpringArmComponent|SetTargetArmLength (Variables|Default|GetSpringArm) (Variables|CameraData|GetWorl%20Bench%20Camera%20Distance))
  (for _array_element (Variables|PartData|GetPart%20Location%20Data)
    (bind _returnvalue (AddComponent|AddSceneComponent false (Math|Transform|MakeTransform _array_element "0, 0, 0" "1.000000,1.000000,1.000000")))
    (Utilities|Array|Add (Variables|Default|GetPart%20Location%20Component%20Data) _returnvalue))
  (bind _returnvalue_2 (AddComponent|AddSceneComponent false (Math|Transform|MakeTransform _location_2 _rotation_2 _scale)))
  (Variables|Default|SetAssecmble%20Camera%20Transform%20Comp _returnvalue_2))