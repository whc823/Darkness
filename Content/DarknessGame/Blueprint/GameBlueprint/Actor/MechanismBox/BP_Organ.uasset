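; BP_Organ is the data-table-driven interactable puzzle piece of the mechanism box: drawers, levers, rune slots, runes and a level-ending portrait.
; Its OrganDataTable row sets mesh, monologue, sound and tip behavior, with a scaling tip mesh that swaps style on touch.
; Clicks branch on row name to slide, pull or fly spawned runes into sockets.
; Row names and tags drive further BP_Organ spawns and task reports to BP_OrganColleront.
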(event Custom|Camer%20Animation%20Over_事件
  (EventDispatchers|UnbindallEventsfromCamerAnimationOver (stale Custom|完成动画_事件 _asbp_darkenss_player_pawn))
  (bind _asbp_darkenss_game_instance (Utilities|Casting|CastToBP_DarkenssGameInstance (Game|GetGameInstance)))
  (Variables|/Game/DarknessGame/Blueprint/GameBlueprint/BP_DarkenssGameInstance.BP_DarkenssGameInstance_C|Set通关 _asbp_darkenss_game_instance true)
  (Game|OpenLevel(byName) "Level_Hallway"))

(event Custom|End%20Touch%20%20Prompt%20Completeion
  ;[0.15 0.15 0.15 0.5] 交互提示内容
  (EventDispatchers|UnbindallEventsfromAnimtionCompletionNotification)
  (CallFunction|SetTipsStyle false)
  (CallFunction|StartAnimationEvent))

(event Custom|Start%20Animation%20Event
  (bind _item_tips_component (Variables|Default|GetItem%20Tips%20Component))
  ;[0.15 0.15 0.15 0.5] 交互提示内容
  (Utilities|IsValid (Variables|Default|GetItem%20Tips%20Component)
    (:Is%20Valid
      (bind _新建轨道_0 (Timeline|时间轴 Play)
        (:Update
          (Utilities|IsValid _item_tips_component
            (:Is%20Valid
              (Transformation|SetRelativeScale3D _item_tips_component (Math|Vector|Lerp(Vector) "0, 0, 0" "1.000000,1.000000,1.000000" _新建轨道_0)))))
        (:Finished
          (Default|CallAnimtionCompletionNotification))))))

(event Custom|Start%20Touch%20Prompt%20Completeion
  ;[0.15 0.15 0.15 0.5] 交互提示内容
  (EventDispatchers|UnbindallEventsfromAnimtionCompletionNotification)
  (CallFunction|SetTipsStyle true)
  (CallFunction|StartAnimationEvent))

(event Custom|Reverse%20Animation%20Envetn
  (bind _item_tips_component (Variables|Default|GetItem%20Tips%20Component))
  ;[0.15 0.15 0.15 0.5] 交互提示内容
  (Utilities|IsValid (Variables|Default|GetItem%20Tips%20Component)
    (:Is%20Valid
      (bind _新建轨道_0 (Timeline|时间轴 Reverse)
        (:Update
          (Utilities|IsValid _item_tips_component
            (:Is%20Valid
              (Transformation|SetRelativeScale3D _item_tips_component (Math|Vector|Lerp(Vector) "0, 0, 0" "1.000000,1.000000,1.000000" _新建轨道_0)))))
        (:Finished
          (Default|CallAnimtionCompletionNotification))))))

(event Custom|完成动画_事件
  (bind _tags (Variables|Actor|GetTags))
  (EventDispatchers|UnbindallEventsfrom完成动画 (Variables|/Game/DarknessGame/Blueprint/GameBlueprint/BP_DarkenssPlayerPawn.BP_DarkenssPlayerPawn_C|Get内心独白控件 (stale EventMouseClickEvent _asbp_darkenss_player_pawn_2)))
  (if (> (Utilities|Array|Length _tags) 0)
    (switch name (Utilities|Array|Get(acopy) _tags)
      (:符文1
        (Default|SubmitDecryptionTask (Variables|Default|GetOrgan%20Collercton) (Utilities|Enum|LiteralenumDecryptionTaskEnum "NewEnumerator1") true)
        (Audio|SpawnSound2D "/Game/D_SFX/交互/获取道具音效.获取道具音效" 1.0 1.0 0.0 0 :!label _label)
        (Actor|DestroyActor))
      (:符文2
        (Default|SubmitDecryptionTask (Variables|Default|GetOrgan%20Collercton) (Utilities|Enum|LiteralenumDecryptionTaskEnum "NewEnumerator3") true)
        (goto _label))
      (:符文3
        (Default|SubmitDecryptionTask (Variables|Default|GetOrgan%20Collercton) (Utilities|Enum|LiteralenumDecryptionTaskEnum "NewEnumerator6") true)
        (goto _label))
      (:人像
        (bind _asbp_darkenss_player_pawn (Utilities|Casting|CastToBP_DarkenssPlayerPawn (Game|GetPlayerCharacter 0)))
        (Default|StartCameraAnimation _asbp_darkenss_player_pawn)
        (EventDispatchers|AssignCamerAnimationOver _asbp_darkenss_player_pawn (delegate Custom|Camer%20Animation%20Over_事件))))))

(event Custom|Audio%20Finished_事件
  (Actor|DestroyActor (Variables|Default|GetSound%20Actor))
  (Variables|Default|SetSound%20Actor 0))

(event EventBeginPlay
  (bind _organ_data (Variables|Default|GetOrgan%20Data))
  (bind (_mesh _content _nocontent _startanimation) (Utilities|Struct|BreakOrganDataStruct _organ_data))
  (Transformation|SetRelativeScale3D (Variables|Default|GetItem%20Tips%20Component) "0, 0, 0")
  (Variables|Drawer|SetDrawer%20Initial%20Postion (Transformation|GetActorLocation))
  (bind _returnvalue (Actor|GetActorOfClass "/Game/DarknessGame/Blueprint/GameBlueprint/Actor/MechanismBox/BP_OrganColleront.BP_OrganColleront_C"))
  (Variables|Default|SetOrgan%20Collercton _returnvalue)
  (if _nocontent
    (Components|DestroyComponent (Variables|Default|GetItem%20Tips%20Component))
    (Variables|Default|SetItem%20Tips%20Component 0))
  (Utilities|FlowControl|Delay 0.2)
  (if _startanimation
    (CallFunction|AnimationEvent))
  (if (.SoundTips (Utilities|Struct|BreakOrganDataStruct (Variables|Default|GetOrgan%20Data)))
    (bind _returnvalue_2 (Game|SpawnActorfromClass "/Game/DarknessGame/Blueprint/GameBlueprint/Actor/BP_SoundLigst.BP_SoundLigst_C" (Math|Transform|MakeTransform (Transformation|GetSocketLocation (Variables|Default|GetStaticMesh) "Socket") "0, 0, 0" "1.000000,1.000000,1.000000") "AlwaysSpawn" "MultiplyWithRoot" 0 "/Engine/EngineSounds/1kSineTonePing.1kSineTonePing" 0))
    (Variables|Default|SetSound%20Actor _returnvalue_2)
    (EventDispatchers|AssignAudioFinished _returnvalue_2 (delegate Custom|Audio%20Finished_事件))))

(event Collision|EventActorBeginOverlap
  (params (OtherActor :type Actor%20Object%20Reference)))

(event EventTick
  (params (DeltaSeconds :type Float%20%28single-precision%29))
  ;[0.15 0.15 0.15 0.5] 交互提示内容
  (Utilities|IsValid (Variables|Default|GetItem%20Tips%20Component)
    (:Is%20Valid
      (if (== (Variables|/Script/Engine.StaticMeshComponent|GetStaticMesh (Variables|Default|GetItem%20Tips%20Component)) "/Game/DarknessGame/ArtAssets/Mesh/SM_SM_TipsStaticMesh02.SM_SM_TipsStaticMesh02")
        (Transformation|SetWorldRotation (Variables|Default|GetItem%20Tips%20Component) (Math|Rotator|MakeRotator 0.0 0.0 (.Yaw (Math|Rotator|BreakRotator (Math|Rotator|FindLookatRotation (Transformation|GetWorldLocation (Variables|Default|GetItem%20Tips%20Component)) (Transformation|GetActorLocation (Game|Player|GetPlayerPawn 0)))))) false false)))))

(event EventTriggerTouchEvent
  (params (Trigger :type Boolean))
  ;[0.15 0.15 0.15 0.5] 交互提示内容
  (if Trigger
    (Utilities|FlowControl|DoOnce false :!label _label
      (:Completed
        (CallFunction|ReverseAnimationEnvetn)
        (EventDispatchers|AssignAnimtionCompletionNotification (delegate Custom|Start%20Touch%20Prompt%20Completeion))
        (goto _label_2 Reset)))
    (else
      (Utilities|FlowControl|DoOnce false :!label _label_2
        (:Completed
          (CallFunction|ReverseAnimationEnvetn)
          (EventDispatchers|AssignAnimtionCompletionNotification (delegate Custom|End%20Touch%20%20Prompt%20Completeion))
          (goto _label Reset))))))

(event EventMouseClickEvent
  (params (Hand%20Actor :type Actor%20Object%20Reference))
  (bind _organ_collercton (Variables|Default|GetOrgan%20Collercton))
  (bind _unlock_organ_box (Variables|/Game/DarknessGame/Blueprint/GameBlueprint/Actor/MechanismBox/BP_OrganColleront.BP_OrganColleront_C|GetUnlock%20Organ%20Box _organ_collercton))
  (if (Variables|Default|GetUnlock%20Required)
    (bind _asbp_darkenss_player_pawn (Utilities|Casting|CastToBP_DarkenssPlayerPawn (Game|GetPlayerCharacter 0)))
    (Default|内心独白 _asbp_darkenss_player_pawn "锁住了！/" "(R=1.000000,G=1.000000,B=1.000000,A=1.000000)")
    (Audio|PlaySound2D "/Game/D_SFX/保险箱/保险箱_机关盒子上锁.保险箱_机关盒子上锁" 1.0 1.0 0.0 0 0)
    (else
      (Utilities|FlowControl|Sequence
        (:then_0
          (Utilities|IsValid (Variables|Default|GetItem%20Tips%20Component)
            (:Is%20Valid
              (Components|DestroyComponent (Variables|Default|GetItem%20Tips%20Component))
              (Variables|Default|SetItem%20Tips%20Component 0)
              (bind _asbp_darkenss_player_pawn_2 (Utilities|Casting|CastToBP_DarkenssPlayerPawn (Game|GetPlayerCharacter 0)))
              (Default|内心独白 _asbp_darkenss_player_pawn_2 (.Content (Utilities|Struct|BreakOrganDataStruct (Variables|Default|GetOrgan%20Data))) "(R=1.000000,G=1.000000,B=1.000000,A=1.000000)")
              (EventDispatchers|Assign完成动画 (Variables|/Game/DarknessGame/Blueprint/GameBlueprint/BP_DarkenssPlayerPawn.BP_DarkenssPlayerPawn_C|Get内心独白控件 _asbp_darkenss_player_pawn_2) (delegate Custom|完成动画_事件)))))
        (:then_1
          (switch name (.RowName (Utilities|Struct|BreakDataTableRowHandle (Variables|Default|GetItem%20Table%20Data)))
            (:抽屉
              (Utilities|FlowControl|DoOnce false
                (:Completed
                  (Audio|PlaySound2D "/Game/D_SFX/机关盒子/抽屉拉开.抽屉拉开" 1.0 1.0 0.0 0 0)
                  (CallFunction|AnimationEvent))))
            (:符文插槽
              (if (.Value (Utilities|Map|Find _unlock_organ_box "NewEnumerator6"))
                (Utilities|FlowControl|DoOnce false
                  (:Completed
                    (bind _returnvalue (Game|SpawnActorfromClass "BP_Organ_C" (Math|Transform|MakeTransform (.location (Transformation|GetActorTransform (Game|GetPlayerCameraManager 0))) "0, 0, 0" "1.000000,1.000000,1.000000") "AlwaysSpawn" "MultiplyWithRoot" 0 (Utilities|Struct|MakeDataTableRowHandle "/Game/DarknessGame/Blueprint/GameBlueprint/Actor/MechanismBox/OrganDataTable.OrganDataTable" "符文3") "0.000000,0.000000,-1500.000000" false 0))
                    (bind _output_get (Variables|Default|SetLly%20Animatio%20Actor _returnvalue))
                    (Variables|BP_Organ_C|SetOrgan%20Data _returnvalue (Utilities|Struct|MakeOrganDataStruct (.mesh (Variables|BP_Organ_C|GetOrgan%20Data _returnvalue)) (.content (Variables|BP_Organ_C|GetOrgan%20Data _returnvalue)) false false (.soundtips (Variables|BP_Organ_C|GetOrgan%20Data _returnvalue))))
                    (CallFunction|FlyAnimatioEvent)))
                (elif (.Value (Utilities|Map|Find _unlock_organ_box "NewEnumerator3"))
                  (Utilities|FlowControl|DoOnce false
                    (:Completed
                      (bind _returnvalue_2 (Game|SpawnActorfromClass "BP_Organ_C" (Math|Transform|MakeTransform (.location (Transformation|GetActorTransform (Game|GetPlayerCameraManager 0))) "0, 0, 0" "1.000000,1.000000,1.000000") "AlwaysSpawn" "MultiplyWithRoot" 0 (Utilities|Struct|MakeDataTableRowHandle "/Game/DarknessGame/Blueprint/GameBlueprint/Actor/MechanismBox/OrganDataTable.OrganDataTable" "符文2") "0.000000,0.000000,-1500.000000" false 0))
                      (Variables|Default|SetLly%20Animatio%20Actor _returnvalue_2)
                      (Variables|BP_Organ_C|SetOrgan%20Data _returnvalue_2 (Utilities|Struct|MakeOrganDataStruct (.mesh (Variables|BP_Organ_C|GetOrgan%20Data _returnvalue_2)) (.content (Variables|BP_Organ_C|GetOrgan%20Data _returnvalue_2)) false false (.soundtips (Variables|BP_Organ_C|GetOrgan%20Data _returnvalue_2))))
                      (CallFunction|FlyAnimatioEvent)))
                  (elif (.Value (Utilities|Map|Find _unlock_organ_box "NewEnumerator1"))
                    (Utilities|FlowControl|DoOnce false
                      (:Completed
                        (bind _returnvalue_3 (Game|SpawnActorfromClass "BP_Organ_C" (Math|Transform|MakeTransform (.location (Transformation|GetActorTransform (Game|GetPlayerCameraManager 0))) "0, 0, 0" "1.000000,1.000000,1.000000") "AlwaysSpawn" "MultiplyWithRoot" 0 (Utilities|Struct|MakeDataTableRowHandle "/Game/DarknessGame/Blueprint/GameBlueprint/Actor/MechanismBox/OrganDataTable.OrganDataTable" "符文1") "0.000000,0.000000,-1500.000000" false 0))
                        (bind _output_get_2 (Variables|Default|SetLly%20Animatio%20Actor _returnvalue_3))
                        (Variables|BP_Organ_C|SetOrgan%20Data _returnvalue_3 (Utilities|Struct|MakeOrganDataStruct (.mesh (Variables|BP_Organ_C|GetOrgan%20Data _returnvalue_3)) (.content (Variables|BP_Organ_C|GetOrgan%20Data _returnvalue_3)) false false (.soundtips (Variables|BP_Organ_C|GetOrgan%20Data _returnvalue_3))))
                        (CallFunction|FlyAnimatioEvent)))))))
            (:拉杆
              (Audio|PlaySound2D "/Game/D_SFX/机关盒子/抽屉拉开.抽屉拉开" 1.0 1.0 0.0 0 0)
              (CallFunction|PullRodAnimation))))))))

(event Custom|Fly%20Animatio%20Event
  (Default|UpdataOrganData (Variables|Default|GetOrgan%20Collercton))
  (Variables|Drawer|SetFlay%20Actor%20Initial%20Postion (Transformation|GetActorLocation (Variables|Default|GetLly%20Animatio%20Actor)))
  (bind _新建轨道_0 (Timeline|Fly%20Into%20Animation PlayFromStart)
    (:Update
      (Transformation|SetActorLocation (Variables|Default|GetLly%20Animatio%20Actor) (Math|Interpolation|VInterpTo (Variables|Drawer|GetFlay%20Actor%20Initial%20Postion) (Transformation|GetSocketLocation (Variables|Default|GetStaticMesh) (.rowname (Variables|BP_Organ_C|GetItem%20Table%20Data (Variables|Default|GetLly%20Animatio%20Actor)))) _新建轨道_0 2.0) false false))
    (:Finished
      (switch name (.rowname (Variables|BP_Organ_C|GetItem%20Table%20Data (Variables|Default|GetLly%20Animatio%20Actor)))
        (:符文1
          (Default|SubmitDecryptionTask (Variables|Default|GetOrgan%20Collercton) (Utilities|Enum|LiteralenumDecryptionTaskEnum "NewEnumerator2") true)
          (Rendering|Material|SetMaterial (Variables|BP_Organ_C|GetStaticMesh (Variables|Default|GetLly%20Animatio%20Actor)) 0 "/Game/DarknessGame/ArtAssets/Materials/M_Basic_Wall.M_Basic_Wall")
          (Variables|Default|SetLly%20Animatio%20Actor 0)
          (bind _outrownames (DataTable|GetDataTableRowNames "/Game/DarknessGame/Blueprint/GameBlueprint/Actor/MechanismBox/OrganDataTable.OrganDataTable"))
          (for _array_element _outrownames
            (if (Math|Boolean|ORBoolean (== _array_element "提示1") (== _array_element "提示2") (== _array_element "提示3"))
              (Game|SpawnActorfromClass "BP_Organ_C" (Math|Transform|MakeTransform (Transformation|GetActorLocation) "0, 0, 0" "1.000000,1.000000,1.000000") "AlwaysSpawn" "MultiplyWithRoot" 0 (Utilities|Struct|MakeDataTableRowHandle "/Game/DarknessGame/Blueprint/GameBlueprint/Actor/MechanismBox/OrganDataTable.OrganDataTable" _array_element) "0.000000,0.000000,0.000000" false 0))))
        (:符文2
          (Default|SubmitDecryptionTask (Variables|Default|GetOrgan%20Collercton) (Utilities|Enum|LiteralenumDecryptionTaskEnum "NewEnumerator4") true)
          (Rendering|Material|SetMaterial (Variables|BP_Organ_C|GetStaticMesh (Variables|Default|GetLly%20Animatio%20Actor)) 0 "/Game/DarknessGame/ArtAssets/Materials/M_Basic_Wall.M_Basic_Wall")
          (Variables|Default|SetLly%20Animatio%20Actor 0)
          (Utilities|FlowControl|Delay 1.5)
          (Default|SinkingAnimation (Variables|Default|GetOrgan%20Collercton))
          (Audio|PlaySound2D "/Game/D_SFX/机关盒子/抽屉解锁.抽屉解锁" 1.0 1.0 0.0 0 0))
        (:符文3
          (Default|SubmitDecryptionTask (Variables|Default|GetOrgan%20Collercton) (Utilities|Enum|LiteralenumDecryptionTaskEnum "NewEnumerator5") true)
          (Rendering|Material|SetMaterial (Variables|BP_Organ_C|GetStaticMesh (Variables|Default|GetLly%20Animatio%20Actor)) 0 "/Game/DarknessGame/ArtAssets/Materials/M_Basic_Wall.M_Basic_Wall")
          (Variables|Default|SetLly%20Animatio%20Actor 0)
          (Default|符文3动画 (Variables|Default|GetOrgan%20Collercton))
          (Audio|PlaySound2D "/Game/D_SFX/机关盒子/抽屉解锁.抽屉解锁" 1.0 1.0 0.0 0 0))))))

(event Custom|Pull%20Rod%20Animation
  (Utilities|FlowControl|DoOnce false :!label _label
    (:Completed
      (if (not (Variables|Default|GetSlider%20pulled))
        (Variables|Default|SetSlider%20pulled true)
        (bind (_direction _新建轨道_0) (Timeline|时间轴_0 PlayFromStart)
          (:Update
            (Transformation|SetActorLocation (Math|Vector|Lerp(Vector) (Variables|Drawer|GetDrawer%20Initial%20Postion) (+ (Variables|Drawer|GetDrawer%20Initial%20Postion) "0.000000,0.000000,-24.000000") _新建轨道_0) false false))
          (:Finished
            (Default|UnlockDetection (Variables|Default|GetOrgan%20Collercton))
            (goto _label Reset)))
        (else
          (Variables|Default|SetSlider%20pulled false)
          (Timeline|时间轴_0 ReverseFromEnd))))))

(event Custom|Reset%20Pulled
  (if (Variables|Default|GetSlider%20pulled)
    (Variables|Default|SetSlider%20pulled false)
    (bind (_direction _新建轨道_0) (Timeline|时间轴_0 ReverseFromEnd)
      (:Update
        (Transformation|SetActorLocation (Math|Vector|Lerp(Vector) (Variables|Drawer|GetDrawer%20Initial%20Postion) (+ (Variables|Drawer|GetDrawer%20Initial%20Postion) "0.000000,0.000000,-24.000000") _新建轨道_0) false false))
      (:Finished
        (Default|UnlockDetection (Variables|Default|GetOrgan%20Collercton))
        (Utilities|FlowControl|DoOnce false) ; enters at Reset
      ))))

(event Custom|Animation%20Event
  (bind _tags (Variables|Actor|GetTags))
  (bind _output (Utilities|Array|Get(acopy) _tags))
  (Variables|Drawer|SetDrawer%20Initial%20Postion (Transformation|GetActorLocation))
  (switch name (.RowName (Utilities|Struct|BreakDataTableRowHandle (Variables|Default|GetItem%20Table%20Data)))
    (:Default
      (Variables|Drawer|SetAnimation%20End%20Postion (+ (Variables|Drawer|GetDrawer%20Initial%20Postion) "45.000000,0.000000,0.000000"))
      (bind _新建轨道_1 (Timeline|Animation%20Timer PlayFromStart)
        (:Update
          (Transformation|SetActorLocation (Math|Vector|Lerp(Vector) (Variables|Drawer|GetDrawer%20Initial%20Postion) (Variables|Drawer|GetAnimation%20End%20Postion) _新建轨道_1) false false))
        (:Finished
          (if (> (Utilities|Array|Length (Variables|Actor|GetTags)) 0)
            (if (not (Utilities|Struct|BreakOrganDataStruct (Variables|Default|GetOrgan%20Data)))
              (bind _returnvalue (Game|SpawnActorfromClass "BP_Organ_C" (Transformation|GetActorTransform) "AdjustIfPossibleButAlwaysSpawn" "MultiplyWithRoot" 0 (Utilities|Struct|MakeDataTableRowHandle "/Game/DarknessGame/Blueprint/GameBlueprint/Actor/MechanismBox/OrganDataTable.OrganDataTable" _output) "0.000000,0.000000,0.000000" false 0))
              (Utilities|Array|Add (Variables|/Script/Engine.Actor|GetTags _returnvalue) _output)
              (Utilities|Array|Clear (Variables|Actor|GetTags)))))))
    (:符文1
      (Variables|Drawer|SetAnimation%20End%20Postion (+ (Variables|Drawer|GetDrawer%20Initial%20Postion) "0.000000,0.000000,45.000000") :!label _label)
      (Timeline|Animation%20Timer PlayFromStart))
    (:符文2
      (goto _label))
    (:符文3
      (goto _label))))

(fn ConstructionScript
  (bind _item_table_data (Variables|Default|GetItem%20Table%20Data))
  (bind _returnvalue (Utilities|GetDataTableRow (.datatable _item_table_data) (.rowname _item_table_data))
    (:then
      (Variables|Default|SetOrgan%20Data _returnvalue)
      (Components|StaticMesh|SetStaticMesh (Variables|Default|GetStaticMesh) (.Mesh (Utilities|Struct|BreakOrganDataStruct _returnvalue)))
      (Transformation|SetWorldScale3D (Variables|Default|GetStaticMesh) (Math|Conversions|ToVector(Float) 1.7))
      (Transformation|SetRelativeLocation (Variables|Default|GetItem%20Tips%20Component) (Variables|Default|GetTips%20Location) false false)
      (for (_ _array_index) (Rendering|Material|GetMaterials (Variables|Default|GetStaticMesh))
        (Rendering|Material|SetMaterial (Variables|Default|GetStaticMesh) _array_index "/Game/DarknessGame/Blueprint/SphereMaskBlueprints/m_detection.m_detection"))
      (if (not (.NoContent (Utilities|Struct|BreakOrganDataStruct (Variables|Default|GetOrgan%20Data))))
        (CallFunction|SetTipsStyle false)))))

(fn SetTipsStyle
  (params (Interaction%20Tips :type Boolean))
  (Utilities|IsValid (Variables|Default|GetItem%20Tips%20Component)
    (:Is%20Valid
      (Components|StaticMesh|SetStaticMesh (Variables|Default|GetItem%20Tips%20Component) (select Interaction%20Tips "/Game/DarknessGame/ArtAssets/Mesh/SM_SM_TipsStaticMesh02.SM_SM_TipsStaticMesh02" "/Game/DarknessGame/ArtAssets/Mesh/SM_TipsStaticMesh01.SM_TipsStaticMesh01"))
      (Rendering|Material|SetMaterial (Variables|Default|GetItem%20Tips%20Component) 0 (select Interaction%20Tips "/Game/DarknessGame/ArtAssets/Materials/M_ItemTipsMaterial.M_ItemTipsMaterial" "/Game/DarknessGame/ArtAssets/Materials/M_Basic_Wall.M_Basic_Wall")))))

(fn GetItemData
  (return "" ""))