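; BP_OrganBox is a mechanism box actor whose mesh is driven by a data table row.
; The construction script looks up that row, assigns its mesh and applies a uniform scale.
; On BeginPlay it stores a reference to BP_OrganBoxManager and overrides every material slot on its child static meshes with M_detection.
; MouseClickEvent and GetItemData are empty stubs.
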(event EventBeginPlay
  (bind _returnvalue (Actor|GetActorOfClass "/Game/DarknessGame/Blueprint/GameBlueprint/Actor/MechanismBox/OrganBox/BP_OrganBoxManager.BP_OrganBoxManager_C"))
  (Variables|Default|SetOrganBoxManager _returnvalue)
  (for _array_element (Components|GetChildrenComponents (Variables|Default|GetDefaultSceneRoot) true)
    (bind _as静态网格体组件 (Utilities|Casting|CastToStaticMeshComponent _array_element))
    (for (_ _array_index) (Rendering|Material|GetMaterials _as静态网格体组件)
      (Rendering|Material|SetMaterial _as静态网格体组件 _array_index "/Game/DarknessGame/Blueprint/SphereMaskBlueprints/m_detection.m_detection"))))

(event Collision|EventActorBeginOverlap
  (params (OtherActor :type Actor%20Object%20Reference)))

(event EventTick
  (params (DeltaSeconds :type Float%20%28single-precision%29)))

(event EventMouseClickEvent
  (params (Hand%20Actor :type Actor%20Object%20Reference)))

(fn ConstructionScript
  (bind _box_table_data (Variables|Default|GetBox%20Table%20Data))
  (bind _returnvalue (Utilities|GetDataTableRow (.datatable _box_table_data) (.rowname _box_table_data))
    (:then
      (Components|StaticMesh|SetStaticMesh (Variables|Default|GetStaticMesh) (Utilities|Struct|BreakOrganBox_Struct _returnvalue))
      (Transformation|SetWorldScale3D (Variables|Default|GetStaticMesh) (Math|Conversions|ToVector(Float) 1.2)))))

(fn GetItemData
  (return "" ""))