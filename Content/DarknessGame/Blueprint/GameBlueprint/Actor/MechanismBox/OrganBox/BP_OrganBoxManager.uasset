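; BP_OrganBoxManager runs a mechanism-box puzzle, raising and lowering itself and relaying button presses to nearby boxes.
; On BeginPlay a sphere trace caches nearby BP_OrganBox actors, and 按钮通知 passes the button ID to the BP_OrganBox_Left ones for unlock animations.
; 机关盒上升动画 shakes the camera and lifts the manager by timeline.
; OverAnmation shakes again and reverses it, then triggers 机关上升 on BP_OrganColleront when finished.
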(event Custom|Over%20Anmation
  (bind _初始位置 (Variables|Default|Get初始位置))
  (bind _asbp_darkenss_player_pawn (Utilities|Casting|CastToBP_DarkenssPlayerPawn (Game|GetPlayerCharacter 0)))
  (Default|PlayCameraShake _asbp_darkenss_player_pawn)
  (bind (_direction _新建轨道_0) (Timeline|机关盒动画 ReverseFromEnd)
    (:Update
      (Transformation|SetActorLocation (Math|Vector|Lerp(Vector) _初始位置 (+ _初始位置 "0.000000,0.000000,500.000000") _新建轨道_0) false false))
    (:Finished
      (switch Utilities|FlowControl|Switch|SwitchonETimelineDirection _direction
        (:Backward
          (bind _returnvalue (Actor|GetActorOfClass "/Game/DarknessGame/Blueprint/GameBlueprint/Actor/MechanismBox/BP_OrganColleront.BP_OrganColleront_C"))
          (Default|机关上升 _returnvalue))))))

(event Custom|机关盒上升动画
  (Variables|Default|Set初始位置 (Transformation|GetActorLocation))
  (bind _asbp_darkenss_player_pawn (Utilities|Casting|CastToBP_DarkenssPlayerPawn (Game|GetPlayerCharacter 0)))
  (Default|PlayCameraShake _asbp_darkenss_player_pawn)
  (bind (_direction _新建轨道_0) (Timeline|机关盒动画 PlayFromStart)
    (:Update
      (Transformation|SetActorLocation (Math|Vector|Lerp(Vector) (Variables|Default|Get初始位置) (+ (Variables|Default|Get初始位置) "0.000000,0.000000,500.000000") _新建轨道_0) false false))
    (:Finished
      (switch Utilities|FlowControl|Switch|SwitchonETimelineDirection _direction
        (:Backward
          (bind _returnvalue (Actor|GetActorOfClass "/Game/DarknessGame/Blueprint/GameBlueprint/Actor/MechanismBox/BP_OrganColleront.BP_OrganColleront_C"))
          (Default|机关上升 _returnvalue))))))

(event EventBeginPlay
  (bind _returnvalue (Transformation|GetActorLocation))
  (Utilities|Array|Clear (Variables|Default|GetOut%20Actors))
  (bind _outhits (Collision|MultiSphereTraceForObjects _returnvalue _returnvalue (Variables|/Script/Engine.SphereComponent|GetSphereRadius (Variables|Default|GetSphere)) (Utilities|Array|MakeArray "ObjectTypeQuery8") false 0 "None"))
  (for _array_element _outhits
    (bind _asbp_organ_box (Utilities|Casting|CastToBP_OrganBox (.HitActor (Collision|BreakHitResult _array_element))))
    (Utilities|Array|Add (Variables|Default|GetOut%20Actors) _asbp_organ_box)))

(event Collision|EventActorBeginOverlap
  (params (OtherActor :type Actor%20Object%20Reference)))

(event EventTick
  (params (DeltaSeconds :type Float%20%28single-precision%29)))

(fn ConstructionScript)

(fn 按钮通知
  (params (ID :type Integer))
  (for _array_element (Variables|Default|GetOut%20Actors)
    (bind _asbp_organ_box_left (Utilities|Casting|CastToBP_OrganBox_Left _array_element))
    (Default|解锁动画 _asbp_organ_box_left ID)))