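; Black puzzle box actor with buttons, sliding compartments, a collectable hour hand and a clock lock.
; Hand clicks dispatch on component tags to timeline animations, while OrganBoxManager tracks collected items and receives button notifications.
; A looping hover timer previews translucent clock-hand slots until both hands are installed.
; Two controllers then step the hands by 30 degrees, and a tolerance check on their rotations unlocks and reveals a hidden component.
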(event Custom|重置触发逻辑
  (Variables|Default|Set正在触发逻辑 false))

(event Custom|时针条件检测
  (if (and (Math|Float|NearlyEqual(Float) (.Roll (Math|Rotator|BreakRotator (Variables|/Script/Engine.SceneComponent|GetRelativeRotation (Variables|Default|Get时针预设体)))) -9e+01 1e+01) (Math|Float|NearlyEqual(Float) (.Roll (Math|Rotator|BreakRotator (Variables|/Script/Engine.SceneComponent|GetRelativeRotation (Variables|Default|Get分针预设体)))) 9e+01 1e+01))
    (Variables|Default|Set已解锁 true)
    (Development|PrintString "解锁")
    (Utilities|FlowControl|DoOnce false
      (:Completed
        (Development|SetHiddeninGame (Variables|Default|Get11) false false)
        (bind _新建轨道_0 (Timeline|时间轴_0 PlayFromStart)
          (:Update
            (Transformation|SetRelativeLocation (Variables|Default|Get11) (Math|Vector|Lerp(Vector) "0.000000,-76.000000,82.000000" "0.000000,-76.000000,65.000000" _新建轨道_0) false false)))))
    (else
      (Development|PrintString "时间错误" true true "(R=0.000000,G=0.660000,B=1.000000,A=1.000000)" 213.0))))

(event EventBeginPlay
  (|CallParentFunction)
  (bind _returnvalue (Utilities|Time|SetTimerbyFunctionName 0 "时针检测" 0.1 true))
  (Variables|Default|Set时针检测定时器 _returnvalue)
  (Collision|SetCollisionEnabled (Variables|Default|Get时针) "NoCollision")
  (Development|SetHiddeninGame (Variables|Default|Get11) true true))

(event Collision|EventActorBeginOverlap
  (params (OtherActor :type Actor%20Object%20Reference))
  (|CallParentFunction OtherActor) ; 此节点被禁用，将不会被调用。\n从引脚连出引线来编译功能。
)

(event EventTick
  (params (DeltaSeconds :type Float%20%28single-precision%29))
  (|CallParentFunction DeltaSeconds)
  (Variables|Default|SetMouse%20Value%20X (Class|Actor|GetInputAxisKeyValue)))

(event EventMouseClickEvent
  (params (Hand%20Actor :type Actor%20Object%20Reference))
  (Variables|Default|SetHand%20Actor Hand%20Actor)
  (bind _hit_compcont (Class|HandDataandMerhodCommunicationInterface|GetHandTouchItem(Message) (Variables|Default|GetHand%20Actor)))
  (if (not (Variables|Default|Get正在触发逻辑))
    (if (> (Utilities|Array|Length (Variables|/Script/Engine.ActorComponent|GetComponentTags _hit_compcont)) 0)
      (Variables|Default|Set正在触发逻辑 true)
      (Utilities|FlowControl|Sequence
        (:then_0
          (switch name (Utilities|Array|Get(acopy) (Variables|/Script/Engine.ActorComponent|GetComponentTags _hit_compcont))
            (:时钟
              (if (Variables|/Game/DarknessGame/Blueprint/GameBlueprint/Actor/MechanismBox/OrganBox/BP_OrganBoxManager.BP_OrganBoxManager_C|GetGet%20Key? (Variables|Default|GetOrganBoxManager))
                (Utilities|FlowControl|DoOnce false
                  (:Completed
                    (CallFunction|钥匙插入时钟动画)))))
            (:旋钮
              (CallFunction|三角形旋钮动画))
            (:时钟分针
              (CallFunction|分针盒子动画))
            (:时针
              (Components|DestroyComponent (Variables|Default|Get时针))
              (Variables|/Game/DarknessGame/Blueprint/GameBlueprint/Actor/MechanismBox/OrganBox/BP_OrganBoxManager.BP_OrganBoxManager_C|Set获取时针 (Variables|Default|GetOrganBoxManager) true)
              (Audio|PlaySound2D "/Game/D_SFX/交互/获取道具音效.获取道具音效" 1.0 1.0 0.0 0 0))
            (:时针预设体
              (if (Variables|/Game/DarknessGame/Blueprint/GameBlueprint/Actor/MechanismBox/OrganBox/BP_OrganBoxManager.BP_OrganBoxManager_C|Get获取时针 (Variables|Default|GetOrganBoxManager))
                (Utilities|FlowControl|DoOnce false
                  (:Completed
                    (for (_ _array_index) (Rendering|Material|GetMaterials (Variables|Default|Get时针预设体))
                      (Rendering|Material|SetMaterial (Variables|Default|Get时针预设体) _array_index "/Game/DarknessGame/Blueprint/SphereMaskBlueprints/m_detection.m_detection"))
                    (Utilities|Array|SetArrayElem (Variables|Default|Get时钟安装) 0 true)
                    (Audio|PlaySound2D "/Game/D_SFX/机关盒子/指针运动.指针运动" 1.0 1.0 0.0 0 0)))))
            (:圆形旋钮
              (CallFunction|圆形按钮))
            (:分针预设体
              (if (Variables|/Game/DarknessGame/Blueprint/GameBlueprint/Actor/MechanismBox/OrganBox/BP_OrganBoxManager.BP_OrganBoxManager_C|Get获取分针 (Variables|Default|GetOrganBoxManager))
                (Utilities|FlowControl|DoOnce false
                  (:Completed
                    (for (_ _array_index_2) (Rendering|Material|GetMaterials (Variables|Default|Get分针预设体))
                      (Rendering|Material|SetMaterial (Variables|Default|Get分针预设体) _array_index_2 "/Game/DarknessGame/Blueprint/SphereMaskBlueprints/m_detection.m_detection"))
                    (Utilities|Array|SetArrayElem (Variables|Default|Get时钟安装) 1 true)
                    (Audio|PlaySound2D "/Game/D_SFX/机关盒子/指针运动.指针运动" 1.0 1.0 0.0 0 0)))))
            (:分针控制器
              (if (Variables|Default|Get时钟完成安装)
                (CallFunction|钟表时间控制器 true)
                (CallFunction|分针动画)
                (Audio|PlaySound2D "/Game/D_SFX/机关盒子/指针运动.指针运动" 1.0 1.0 0.0 0 0 :!label _label)))
            (:时针控制器
              (if (Variables|Default|Get时钟完成安装)
                (CallFunction|钟表时间控制器 false)
                (CallFunction|时针动画)
                (goto _label)))))
        (:then_1
          (Utilities|FlowControl|Delay 1.0)
          (CallFunction|重置触发逻辑))))))

(event Custom|时针动画
  (Variables|Default|Set时针初始旋转 (Variables|/Script/Engine.SceneComponent|GetRelativeRotation (Variables|Default|Get时针预设体)))
  (bind _新建轨道_0 (Timeline|时针时间轴 PlayFromStart)
    (:Update
      (Transformation|SetRelativeRotation (Variables|Default|Get时针预设体) (Math|Rotator|Lerp(Rotator) (Variables|Default|Get时针初始旋转) (Math|Rotator|MakeRotator (+ (.roll (Variables|Default|Get时针初始旋转)) -3e+01) (.pitch (Variables|Default|Get时针初始旋转)) (.yaw (Variables|Default|Get时针初始旋转))) _新建轨道_0) false false))))

(event Custom|分针动画
  (Variables|Default|Set分针初始旋转 (Variables|/Script/Engine.SceneComponent|GetRelativeRotation (Variables|Default|Get分针预设体)))
  (bind _新建轨道_0 (Timeline|分针时间轴 PlayFromStart)
    (:Update
      (Transformation|SetRelativeRotation (Variables|Default|Get分针预设体) (Math|Rotator|Lerp(Rotator) (Variables|Default|Get分针初始旋转) (Math|Rotator|MakeRotator (+ (.roll (Variables|Default|Get分针初始旋转)) -3e+01) (.pitch (Variables|Default|Get分针初始旋转)) (.yaw (Variables|Default|Get分针初始旋转))) _新建轨道_0) false false))))

(event Custom|钟表时间控制器
  (params (Left :type Boolean))
  (Audio|PlaySound2D "/Game/D_SFX/机关盒子/按钮.按钮" 1.0 1.0 0.0 0 0)
  (bind _新建轨道_0 (Timeline|控制器动画 PlayFromStart)
    (:Update
      (Transformation|SetRelativeLocation (select Left (Variables|Default|Get分针控制器) (Variables|Default|Get时针控制器)) (Math|Vector|Lerp(Vector) "0, 0, 0" (select Left "0.000000,0.000000,-4.000000" "0.000000,0.000000,4.000000") _新建轨道_0) false false))
    (:Finished
      (CallFunction|时针条件检测))))

(event Custom|点击旋钮事件
  (Development|PrintString "点击旋钮" true true "(R=0.000000,G=0.660000,B=1.000000,A=1.000000)" 122.0))

(event Custom|钥匙插入时钟动画
  (bind _returnvalue (AddComponent|AddStaticMeshComponent true (Transformation|GetSocketTransform (Variables|Default|GetStaticMesh1) "钥匙孔" "RTS_Actor")))
  (bind _output_get (Variables|Default|Set钥匙模型 _returnvalue))
  (Variables|Default|Set动画初始位置 (Variables|/Script/Engine.SceneComponent|GetRelativeLocation _output_get))
  (Audio|PlaySound2D "/Game/D_SFX/门/插入钥匙.插入钥匙" 1.0 1.0 0.0 0 0)
  (bind _新建轨道_0 (Timeline|时间轴 PlayFromStart)
    (:Update
      ;[0.15 0.15 0.15 0.5] 插入钥匙
      (Transformation|SetRelativeLocation (Variables|Default|Get钥匙模型) (Math|Vector|Lerp(Vector) (Variables|Default|Get动画初始位置) (+ (Variables|Default|Get动画初始位置) "0.000000,7.000000,0.000000") _新建轨道_0) false false))
    (:Finished
      (Audio|PlaySound2D "/Game/D_SFX/机关盒子/抽屉拉开.抽屉拉开" 1.0 1.0 0.0 0 0)
      (bind _新建轨道_0_2 (Timeline|钥匙旋转动画时间轴 PlayFromStart)
        (:Update
          ;[0.15 0.15 0.15 0.5] 旋转钥匙
          (Transformation|SetRelativeRotation (Variables|Default|Get钥匙模型) (Math|Rotator|Lerp(Rotator) "0, 0, 0" "80.000000,0.000000,0.000000" _新建轨道_0_2) false false))
        (:Finished
          (Transformation|AttachComponentToComponent (Variables|Default|Get钥匙模型) (Variables|Default|GetStaticMesh1) "None" "KeepWorld" "KeepWorld" "KeepWorld" true)
          (CallFunction|拉出时钟动画))))))

(event Custom|拉出时钟动画
  (Utilities|FlowControl|DoOnce false
    (:Completed
      (Audio|PlaySound2D "/Game/D_SFX/机关盒子/抽屉拉开.抽屉拉开" 1.0 1.0 0.0 0 0)
      (bind _新建轨道_0 (Timeline|拉出时间轴 PlayFromStart)
        (:Update
          ;[0.15 0.15 0.15 0.5] 拉出BOX
          (Transformation|SetRelativeLocation (Variables|Default|GetStaticMesh1) (Math|Vector|Lerp(Vector) "0.000000,39.000000,0.000000" "0, 0, 0" _新建轨道_0) false false))
        (:Finished
          (Collision|SetCollisionEnabled (Variables|Default|GetStaticMesh1) "NoCollision"))))))

(event Custom|三角形旋钮动画
  (Audio|PlaySound2D "/Game/D_SFX/机关盒子/按钮.按钮" 1.0 1.0 0.0 0 0)
  (bind _新建轨道_0 (Timeline|钥匙动画 PlayFromStart)
    (:Update
      ;[0.15 0.15 0.15 0.5] 旋钮动画
      (Transformation|SetRelativeLocation (Variables|Default|Get三角形旋钮) (Math|Vector|Lerp(Vector) "0.000000,-45.000000,57.000000" "0.000000,-42.000000,57.000000" _新建轨道_0) false false))
    (:Finished
      (Default|按钮通知 (Variables|Default|GetOrganBoxManager)))))

(event Custom|分针盒子动画
  (Audio|PlaySound2D "/Game/D_SFX/机关盒子/抽屉拉开.抽屉拉开" 1.0 1.0 0.0 0 0)
  (bind _新建轨道_0 (Timeline|分针机关盒子动画 PlayFromStart)
    (:Update
      (Transformation|SetRelativeLocation (Variables|Default|Get带钥匙孔box) (Math|Vector|Lerp(Vector) "0.000000,0.000000,-15.000000" "0, 0, 0" _新建轨道_0) false false))
    (:Finished
      (Collision|SetCollisionEnabled (Variables|Default|Get带钥匙孔box) "NoCollision")
      (Collision|SetCollisionEnabled (Variables|Default|Get时针) "QueryAndPhysics"))))

(event Custom|圆形按钮
  (Utilities|FlowControl|DoOnce false :!label _label
    (:Completed
      (Audio|PlaySound2D "/Game/D_SFX/机关盒子/按钮.按钮" 1.0 1.0 0.0 0 0)
      (bind _新建轨道_0 (Timeline|圆形按钮动画 PlayFromStart)
        (:Update
          (Transformation|SetRelativeLocation (Variables|Default|Get圆形旋钮) (Math|Vector|Lerp(Vector) "7.000000,-64.000000,115.000000" "5.500000,-64.000000,115.000000" _新建轨道_0) false false))
        (:Finished
          (Default|按钮通知 (Variables|Default|GetOrganBoxManager) 1)
          (goto _label Reset))))))

(fn ConstructionScript
  (|CallParentFunction)
  (Transformation|SetRelativeTransform (Variables|Default|GetScene2) (Variables|Default|Get三角形按钮变换) false false))

(fn 时针检测
  (bind _时钟安装 (Variables|Default|Get时钟安装))
  (bind _时钟安装_2 (Variables|Default|Get时钟安装))
  (bind _hit_compcont (Class|HandDataandMerhodCommunicationInterface|GetHandTouchItem(Message) (Variables|Default|GetHand%20Actor)))
  (Utilities|IsValid _hit_compcont
    (:Is%20Valid
      (if (or (Components|ComponentHasTag _hit_compcont "时针预设体") (Components|ComponentHasTag _hit_compcont "分针预设体"))
        (if (and (Variables|/Game/DarknessGame/Blueprint/GameBlueprint/Actor/MechanismBox/OrganBox/BP_OrganBoxManager.BP_OrganBoxManager_C|Get获取分针 (Variables|Default|GetOrganBoxManager)) (Variables|/Game/DarknessGame/Blueprint/GameBlueprint/Actor/MechanismBox/OrganBox/BP_OrganBoxManager.BP_OrganBoxManager_C|Get获取时针 (Variables|Default|GetOrganBoxManager)))
          (Rendering|Material|SetMaterial (Variables|Default|Get分针预设体) 0 "/Game/DarknessGame/Blueprint/SphereMaskBlueprints/m_detection.m_detection")
          (if (and (Utilities|Array|Get(acopy) _时钟安装_2) (Utilities|Array|Get(acopy) _时钟安装_2 1))
            (Utilities|Time|PauseTimerbyHandle (Variables|Default|Get时针检测定时器))
            (Utilities|Time|ClearandInvalidateTimerbyHandle (Variables|Default|Get时针检测定时器))
            (Variables|Default|Set时钟完成安装 true))
          (else
            (if (Components|ComponentHasTag _hit_compcont "时针预设体")
              (Rendering|Material|SetMaterial (Variables|Default|Get时针预设体) 0 (select (Variables|/Game/DarknessGame/Blueprint/GameBlueprint/Actor/MechanismBox/OrganBox/BP_OrganBoxManager.BP_OrganBoxManager_C|Get获取时针 (Variables|Default|GetOrganBoxManager)) "/Game/DarknessGame/Blueprint/SphereMaskBlueprints/m_detection.m_detection" "/Game/DarknessGame/ArtAssets/Materials/M_TranslucentMaterial_Inst.M_TranslucentMaterial_Inst")))
            (if (Components|ComponentHasTag _hit_compcont "分针预设体")
              (Rendering|Material|SetMaterial (Variables|Default|Get分针预设体) 0 (select (Variables|/Game/DarknessGame/Blueprint/GameBlueprint/Actor/MechanismBox/OrganBox/BP_OrganBoxManager.BP_OrganBoxManager_C|Get获取分针 (Variables|Default|GetOrganBoxManager)) "/Game/DarknessGame/Blueprint/SphereMaskBlueprints/m_detection.m_detection" "/Game/DarknessGame/ArtAssets/Materials/M_TranslucentMaterial_Inst.M_TranslucentMaterial_Inst")))))))
    (:Is%20Not%20Valid
      (if (Utilities|Array|Get(acopy) _时钟安装)
        _
        (else
          (Rendering|Material|SetMaterial (Variables|Default|Get时针预设体) 0 "/Game/DarknessGame/ArtAssets/Materials/M_TranslucentMaterial_Inst.M_TranslucentMaterial_Inst")))
      (if (not (Utilities|Array|Get(acopy) _时钟安装 1))
        (Rendering|Material|SetMaterial (Variables|Default|Get分针预设体) 0 "/Game/DarknessGame/ArtAssets/Materials/M_TranslucentMaterial_Inst.M_TranslucentMaterial_Inst")))))