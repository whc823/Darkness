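; Front face of a puzzle box with a square knob button and a four-dial rotary combination lock, worked by the player's hand actor.
; Clicking the tagged button animates the knob, then notifies the OrganBoxManager.
; During left-click notifications, a short hand trace picks a dial, and accumulated vertical mouse movement turns it one 30-degree step either way, gated until release.
; Each step checks all dial rolls within tolerance, triggering BP_OrganBoxManager's finishing animation on a match.
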(event Custom|Left%20Click%20Notification_事件
  (params (Hand :type Actor%20Object%20Reference))
  (Variables|Default|SetHand%20Actor Hand)
  (Input|EnableInput (Game|GetPlayerController 0))
  (bind (_outhit _returnvalue) (Collision|LineTraceForObjects (Transformation|GetActorLocation (Variables|Default|GetHand%20Actor)) (+ (Transformation|GetActorLocation (Variables|Default|GetHand%20Actor)) (* (Transformation|GetActorForwardVector (Variables|Default|GetHand%20Actor)) (Math|Conversions|ToVector(Float) 4e+01))) (Utilities|Array|MakeArray "ObjectTypeQuery8") false 0 "None" false))
  (if _returnvalue
    (Variables|Default|SetAnimation%20Component (.HitComponent (Collision|BreakHitResult _outhit)))
    (bind _output_get (Variables|Default|SetMouse%20Move%20Cumlative%20Value (+ (Variables|Default|GetMouse%20Value%20Y) (Variables|Default|GetMouse%20Move%20Cumlative%20Value))))
    (if (> _output_get 1e+01)
      (Utilities|FlowControl|DoOnce false
        (:Completed
          (CallFunction|PlayRouletteAnimation true)))
      (elif (and (!= _output_get 0.0) (< _output_get -1e+01))
        (Utilities|FlowControl|DoOnce false
          (:Completed
            (CallFunction|PlayRouletteAnimation false)))))))

(event Custom|Up%20Left%20Click%20Notification_事件
  (bind _asbp_darkenss_player_controller (Utilities|Casting|CastToBP_DarkenssPlayerController (Game|GetPlayerController 0)))
  (EventDispatchers|UnbindallEventsfromLeftClickNotification _asbp_darkenss_player_controller)
  (EventDispatchers|UnbindallEventsfromUpLeftClickNotification _asbp_darkenss_player_controller)
  (Variables|Default|SetHand%20Actor 0)
  (Variables|Default|SetMouse%20Move%20Cumlative%20Value 0.0)
  (Input|DisableInput (Game|GetPlayerController 0))
  (CallFunction|ResetAniamtion))

(event Custom|Play%20Roulette%20Animation
  (params (Up%20Animation :type Boolean))
  (Utilities|FlowControl|DoOnce false :!label _label
    (:Completed
      (Variables|Default|SetUp%20Animation Up%20Animation)
      (Variables|Default|SetCurrent%20Rotation (Variables|/Script/Engine.SceneComponent|GetRelativeRotation (Variables|Default|GetAnimation%20Component)))
      (bind _新建轨道_0 (Timeline|Aniamtion PlayFromStart)
        (:Update
          (Transformation|SetRelativeRotation (Variables|Default|GetAnimation%20Component) (Math|Rotator|Lerp(Rotator) (Variables|Default|GetCurrent%20Rotation) (Math|Rotator|MakeRotator (+ (.roll (Variables|Default|GetCurrent%20Rotation)) (select (Variables|Default|GetUp%20Animation) 3e+01 -3e+01)) (.pitch (Variables|Default|GetCurrent%20Rotation)) (.yaw (Variables|Default|GetCurrent%20Rotation))) _新建轨道_0) false false))
        (:Finished
          (Utilities|FlowControl|Sequence
            (:then_0
              (Utilities|FlowControl|Delay 0.5)
              (if (Math|Boolean|ANDBoolean (Math|Float|NearlyEqual(Float) (.Roll (Math|Rotator|BreakRotator (Variables|/Script/Engine.SceneComponent|GetRelativeRotation (Variables|Default|GetRoulette%20Static%20Mesh%2001)))) -1.5e+02 1e+01) (Math|Float|NearlyEqual(Float) (.Roll (Math|Rotator|BreakRotator (Variables|/Script/Engine.SceneComponent|GetRelativeRotation (Variables|Default|GetRoulette%20Static%20Mesh%2002)))) -6e+01 1e+01) (Math|Float|NearlyEqual(Float) (.Roll (Math|Rotator|BreakRotator (Variables|/Script/Engine.SceneComponent|GetRelativeRotation (Variables|Default|GetRoulette%20Static%20Mesh%2003)))) 1.2e+02 1e+01) (Math|Float|NearlyEqual(Float) (.Roll (Math|Rotator|BreakRotator (Variables|/Script/Engine.SceneComponent|GetRelativeRotation (Variables|Default|GetRoulette%20Static%20Mesh%2004)))) 3e+01 1e+01))
                (Development|PrintString "密码正确！" true true "(R=0.189999,G=1.000000,B=0.000000,A=1.000000)" 123.0)
                (bind _returnvalue (Actor|GetActorOfClass "/Game/DarknessGame/Blueprint/GameBlueprint/Actor/MechanismBox/OrganBox/BP_OrganBoxManager.BP_OrganBoxManager_C"))
                (Default|OverAnmation _returnvalue)
                (else
                  (Development|PrintString "密码错误！" true true "(R=1.000000,G=0.000000,B=0.000000,A=1.000000)" 123.0))))
            (:then_1
              (goto _label Reset))))))))

(event Custom|Reset%20Aniamtion
  (Utilities|FlowControl|Sequence
    (:then_0
      (Utilities|FlowControl|DoOnce false) ; enters at Reset
    )
    (:then_1
      (Utilities|FlowControl|DoOnce false) ; enters at Reset
    )))

(event Custom|正方形旋钮动画
  (bind _旋钮 (Timeline|时间轴 PlayFromStart)
    (:Update
      ;[0.15 0.15 0.15 0.5] 旋钮动画
      (Transformation|SetRelativeLocation (Variables|Default|GetStaticMesh1) (Math|Vector|Lerp(Vector) "0.000000,43.000000,56.000000" "0.000000,38.000000,56.000000" _旋钮) false false))
    (:Finished
      (Default|按钮通知 (Variables|Default|GetOrganBoxManager) 2)
      (Utilities|FlowControl|DoOnce false ; enters at Reset
        (:Completed
          (bind _hit_compcont (Class|HandDataandMerhodCommunicationInterface|GetHandTouchItem(Message) (Variables|Default|GetHand%20Actor)))
          (if (Components|ComponentHasTag _hit_compcont "按钮")
            (CallFunction|正方形旋钮动画)))))))

(event EventBeginPlay
  (|CallParentFunction) ; 此节点被禁用，将不会被调用。\n从引脚连出引线来编译功能。
)

(event Collision|EventActorBeginOverlap
  (params (OtherActor :type Actor%20Object%20Reference))
  (|CallParentFunction OtherActor) ; 此节点被禁用，将不会被调用。\n从引脚连出引线来编译功能。
)

(event EventTick
  (params (DeltaSeconds :type Float%20%28single-precision%29))
  (|CallParentFunction DeltaSeconds)
  (Variables|Default|SetMouse%20Value%20Y (* (Class|Actor|GetInputAxisKeyValue) -1.0)))

(event EventMouseClickEvent
  (params (Hand%20Actor :type Actor%20Object%20Reference))
  (Variables|Default|SetHand%20Actor Hand%20Actor)
  (bind _asbp_darkenss_player_controller (Utilities|Casting|CastToBP_DarkenssPlayerController (Game|GetPlayerController 0)))
  (EventDispatchers|AssignLeftClickNotification _asbp_darkenss_player_controller (delegate Custom|Left%20Click%20Notification_事件))
  (EventDispatchers|AssignUpLeftClickNotification _asbp_darkenss_player_controller (delegate Custom|Up%20Left%20Click%20Notification_事件))
  (bind _hit_compcont (Class|HandDataandMerhodCommunicationInterface|GetHandTouchItem(Message) (Variables|Default|GetHand%20Actor)))
  (if (Components|ComponentHasTag _hit_compcont "按钮")
    (CallFunction|正方形旋钮动画)))

(fn ConstructionScript
  (|CallParentFunction))