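; BP_OrganBox_Left is the left part of an organ-box puzzle: three rotatable knobs guard a minute-hand item.
; The unlock animation event turns the selected knob 90 degrees in roll by timeline, then checks whether all three sit at zero rotation.
; On success, chained timelines slide two meshes to present the minute hand and mark the puzzle solved.
; Clicking the tagged hand then flags it acquired on OrganBoxManager and destroys it.
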(event Custom|解锁动画
  (params (ID :type Integer))
  (if (not (Variables|Default|Get解开旋钮))
    (Audio|PlaySound2D "/Game/D_SFX/机关盒子/转动类机关1_沉重.转动类机关1_沉重" 1.0 1.0 0.0 0 0)
    (Variables|Default|Set正在进行解锁的ID ID)
    (Variables|Default|Set当前旋转 (Utilities|Select :Index (Variables|Default|Get正在进行解锁的ID) :Option%200 (Variables|/Script/Engine.SceneComponent|GetRelativeRotation (Variables|组件|Get旋钮01)) :Option%201 (Variables|/Script/Engine.SceneComponent|GetRelativeRotation (Variables|组件|Get旋钮02)) :Option%202 (Variables|/Script/Engine.SceneComponent|GetRelativeRotation (Variables|组件|Get旋钮04))))
    (bind _新建轨道_0 (Timeline|时间轴 PlayFromStart)
      (:Update
        (Transformation|SetRelativeRotation (Utilities|Select :Index (Variables|Default|Get正在进行解锁的ID) :Option%200 (Variables|组件|Get旋钮01) :Option%201 (Variables|组件|Get旋钮02) :Option%202 (Variables|组件|Get旋钮04)) (Math|Rotator|Lerp(Rotator) (Variables|Default|Get当前旋转) (Math|Rotator|MakeRotator (+ (.roll (Variables|Default|Get当前旋转)) 9e+01) (.pitch (Variables|Default|Get当前旋转)) (.yaw (Variables|Default|Get当前旋转))) _新建轨道_0) false false))
      (:Finished
        (if (Math|Boolean|ANDBoolean (Utilities|Operators|EqualEqual :A (Variables|/Script/Engine.SceneComponent|GetRelativeRotation (Variables|组件|Get旋钮01)) :ErrorTolerance 1.0) (Utilities|Operators|EqualEqual :A (Variables|/Script/Engine.SceneComponent|GetRelativeRotation (Variables|组件|Get旋钮02)) :ErrorTolerance 1.0) (Utilities|Operators|EqualEqual :A (Variables|/Script/Engine.SceneComponent|GetRelativeRotation (Variables|组件|Get旋钮04)) :ErrorTolerance 1.0))
          (Development|PrintString "解开密码")
          (bind _新建轨道_1 (Timeline|解开动画 PlayFromStart)
            (:Update
              (Transformation|SetRelativeLocation (Variables|组件|GetStaticMesh2) (Math|Vector|Lerp(Vector) "4.000000,0.000000,0.000000" "-17.000000,0.000000,0.000000" _新建轨道_1) false false))
            (:Finished
              (bind _新建轨道_0_2 (Timeline|分针出现动画 PlayFromStart)
                (:Update
                  (Transformation|SetRelativeLocation (Variables|组件|GetStaticMesh1) (Math|Vector|Lerp(Vector) "0, 0, 0" "0.000000,0.000000,10.000000" _新建轨道_0_2) false false))
                (:Finished
                  (Variables|Default|Set解开旋钮 true)
                  (Collision|SetCollisionEnabled (Variables|组件|GetStaticMesh1) "NoCollision"))))))))))

(event EventBeginPlay
  (|CallParentFunction) ; 此节点被禁用，将不会被调用。\n从引脚连出引线来编译功能。
)

(event Collision|EventActorBeginOverlap
  (params (OtherActor :type Actor%20Object%20Reference))
  (|CallParentFunction OtherActor) ; 此节点被禁用，将不会被调用。\n从引脚连出引线来编译功能。
)

(event EventTick
  (params (DeltaSeconds :type Float%20%28single-precision%29))
  (|CallParentFunction DeltaSeconds) ; 此节点被禁用，将不会被调用。\n从引脚连出引线来编译功能。
)

(event EventMouseClickEvent
  (params (Hand%20Actor :type Actor%20Object%20Reference))
  (Variables|Default|SetHand%20Actor Hand%20Actor)
  (if (Variables|Default|Get解开旋钮)
    (bind _hit_compcont (Class|HandDataandMerhodCommunicationInterface|GetHandTouchItem(Message) (Variables|Default|GetHand%20Actor)))
    (if (Components|ComponentHasTag _hit_compcont "分针")
      (Variables|/Game/DarknessGame/Blueprint/GameBlueprint/Actor/MechanismBox/OrganBox/BP_OrganBoxManager.BP_OrganBoxManager_C|Set获取分针 (Variables|Default|GetOrganBoxManager) true)
      (Components|DestroyComponent (Variables|Default|Get分针))
      (Audio|PlaySound2D "/Game/D_SFX/交互/获取道具音效.获取道具音效" 1.0 1.0 0.0 0 0))))

(fn ConstructionScript
  (|CallParentFunction))