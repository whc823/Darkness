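; BP_OrganBox_Right is a mechanism box actor with a gear the player turns by mouse.
; MouseClickEvent stores the hand actor and binds to the player controller's left-click notifications, with release unbinding them and disabling input.
; Each click notification traces forward from the hand; hitting a component tagged "齿轮" (gear) rolls StaticMesh2 by the inverted axis value cached on Tick and plays a rotation sound.
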(event Custom|Left%20Click%20Notification_事件
  (params (Hand :type Actor%20Object%20Reference))
  (bind _hand_actor (Variables|Default|GetHand%20Actor))
  (bind _returnvalue (Transformation|GetActorLocation _hand_actor))
  (Input|EnableInput (Game|GetPlayerController 0))
  (bind (_outhit _returnvalue_2) (Collision|LineTraceForObjects _returnvalue (+ _returnvalue (* (Transformation|GetActorForwardVector (Variables|Default|GetHand%20Actor)) (Math|Conversions|ToVector(Float) 1.5e+02))) (Utilities|Array|MakeArray "ObjectTypeQuery8") false (Utilities|Array|MakeArray (Variables|Default|GetHand%20Actor) (Game|GetPlayerCharacter 0)) "ForOneFrame" false))
  (if _returnvalue_2
    (if (Components|ComponentHasTag (.HitComponent (Collision|BreakHitResult _outhit)) "齿轮")
      (Transformation|AddWorldRotation (Variables|Default|GetStaticMesh2) (Math|Rotator|MakeRotator (Variables|Default|GetMouse%20Value%20Y) 0.0 0.0) false false)
      (Audio|PlaySound2D "/Game/D_SFX/机关盒子/转动类机关2_快速.转动类机关2_快速" 1.0 1.0 0.0 0 0))))

(event Custom|CustomEvent
  (bind _asbp_ov_player_controller (Utilities|Casting|CastToBP_OV_PlayerController (Game|GetPlayerController 0)))
  (EventDispatchers|UnbindallEventsfromLeftClickNotification _asbp_ov_player_controller)
  (EventDispatchers|UnbindallEventsfromUpLeftClickNotification _asbp_ov_player_controller)
  (Variables|Default|SetHand%20Actor 0)
  (Input|DisableInput (Game|GetPlayerController 0)))

(event EventBeginPlay
  (|CallParentFunction) ; 此节点被禁用，将不会被调用。\n从引脚连出引线来编译功能。
)

(event Collision|EventActorBeginOverlap
  (params (OtherActor :type Actor%20Object%20Reference))
  (|CallParentFunction OtherActor) ; 此节点被禁用，将不会被调用。\n从引脚连出引线来编译功能。
)

(event EventTick
  (params (DeltaSeconds :type Float%20%28single-precision%29))
  (|CallParentFunction DeltaSeconds)
  (Variables|Default|SetMouse%20Value%20Y (* (Class|Actor|GetInputAxisKeyValue) -1.0)))

(event EventMouseClickEvent
  (params (Hand%20Actor :type Actor%20Object%20Reference))
  (Variables|Default|SetHand%20Actor Hand%20Actor)
  (bind _asbp_ov_player_controller (Utilities|Casting|CastToBP_OV_PlayerController (Game|GetPlayerController 0)))
  (EventDispatchers|AssignLeftClickNotification _asbp_ov_player_controller (delegate Custom|Left%20Click%20Notification_事件))
  (EventDispatchers|AssignUpLeftClickNotification _asbp_ov_player_controller (delegate Custom|CustomEvent)))

(fn ConstructionScript
  (|CallParentFunction))