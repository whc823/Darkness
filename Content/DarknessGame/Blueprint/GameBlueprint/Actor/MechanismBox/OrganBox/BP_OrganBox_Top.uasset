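; Top section of the organ box puzzle, where sliding a soldier piece and a car piece reveals a collectible key.
; A hand click binds to player controller left-click events, and the hit component's tag picks the action, once per press until release.
; Each piece follows its spline by timeline; when both finish, the key rises and gains collision.
; Clicking the key flags it on BP_OrganBoxManager, destroys the mesh and plays a pickup sound.
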(event Custom|Left%20Click%20Notification_事件
  (params (Hand :type Actor%20Object%20Reference))
  (Utilities|FlowControl|DoOnce false
    (:Completed
      (bind _hit_compcont (Class|HandDataandMerhodCommunicationInterface|GetHandTouchItem(Message) (Variables|Default|GetHand%20Actor)))
      (Utilities|IsValid _hit_compcont
        (:Is%20Valid
          (if (Components|ComponentHasTag _hit_compcont "Soldier")
            (Collision|SetCollisionEnabled (Variables|Default|GetSoldier%20Pieces%20StaticMesh) "NoCollision")
            (bind _新建轨道_0 (Timeline|Soldier%20Animation PlayFromStart)
              (:Update
                (Transformation|SetRelativeLocation (Variables|Default|GetSoldier%20Pieces%20StaticMesh) (Spline|GetLocationatTime (Variables|Default|GetSoldier%20Spline) _新建轨道_0 "Local" false) false false))
              (:Finished
                (Variables|Default|SetSoldier%20Animation%20Over true)
                (CallFunction|UnlockKeyAnimation)))
            (elif (Components|ComponentHasTag _hit_compcont "Car")
              (Collision|SetCollisionEnabled (Variables|Default|GetCar%20Pieces%20StaticMesh) "NoCollision")
              (bind _新建轨道_0_2 (Timeline|Car%20Pieces%20Animation PlayFromStart)
                (:Update
                  (Transformation|SetRelativeLocation (Variables|Default|GetCar%20Pieces%20StaticMesh) (Spline|GetLocationatTime (Variables|Default|GetCar%20Spline) _新建轨道_0_2 "Local" false) false false))
                (:Finished
                  (Variables|Default|SetCar%20Pieces%20Aimation%20Over true)
                  (CallFunction|UnlockKeyAnimation)))
              (elif (Components|ComponentHasTag _hit_compcont "Key")
                (bind _returnvalue (Actor|GetActorOfClass "/Game/DarknessGame/Blueprint/GameBlueprint/Actor/MechanismBox/OrganBox/BP_OrganBoxManager.BP_OrganBoxManager_C"))
                (Variables|/Game/DarknessGame/Blueprint/GameBlueprint/Actor/MechanismBox/OrganBox/BP_OrganBoxManager.BP_OrganBoxManager_C|SetGet%20Key? _returnvalue true)
                (Components|DestroyComponent (Variables|Default|GetKey%20Static%20Mesh))
                (Audio|PlaySound2D "/Game/D_SFX/交互/获取道具音效.获取道具音效" 1.0 1.0 0.0 0 0)))))))))

(event Custom|Up%20Left%20Click%20Notification_事件
  (bind _asbp_darkenss_player_controller (Utilities|Casting|CastToBP_DarkenssPlayerController (Game|GetPlayerController 0)))
  (EventDispatchers|UnbindallEventsfromLeftClickNotification _asbp_darkenss_player_controller)
  (EventDispatchers|UnbindallEventsfromUpLeftClickNotification _asbp_darkenss_player_controller)
  (Variables|Default|SetHand%20Actor 0)
  (CallFunction|ResetMouseClick))

(event Custom|Unlock%20Key%20Animation
  (if (and (Variables|Default|GetCar%20Pieces%20Aimation%20Over) (Variables|Default|GetSoldier%20Animation%20Over))
    (bind _新建轨道_0 (Timeline|Key%20Animation PlayFromStart)
      (:Update
        (Transformation|SetRelativeLocation (Variables|Default|GetKey%20Static%20Mesh) (Math|Vector|Lerp(Vector) "0.000000,0.000000,130.000000" "0.000000,0.000000,150.000000" _新建轨道_0) false false))
      (:Finished
        (Collision|SetCollisionEnabled (Variables|Default|GetKey%20Static%20Mesh) "QueryAndPhysics")))))

(event Custom|Reset%20Mouse%20Click
  (Utilities|FlowControl|DoOnce false) ; enters at Reset
)

(event EventBeginPlay
  (|CallParentFunction)
  (Collision|SetCollisionEnabled (Variables|Default|GetKey%20Static%20Mesh) "NoCollision"))

(event Collision|EventActorBeginOverlap
  (params (OtherActor :type Actor%20Object%20Reference))
  (|CallParentFunction OtherActor) ; 此节点被禁用，将不会被调用。\n从引脚连出引线来编译功能。
)

(event EventTick
  (params (DeltaSeconds :type Float%20%28single-precision%29))
  (|CallParentFunction DeltaSeconds))

(event EventMouseClickEvent
  (params (Hand%20Actor :type Actor%20Object%20Reference))
  (Variables|Default|SetHand%20Actor Hand%20Actor)
  (bind _asbp_darkenss_player_controller (Utilities|Casting|CastToBP_DarkenssPlayerController (Game|GetPlayerController 0)))
  (EventDispatchers|AssignLeftClickNotification _asbp_darkenss_player_controller (delegate Custom|Left%20Click%20Notification_事件))
  (EventDispatchers|AssignUpLeftClickNotification _asbp_darkenss_player_controller (delegate Custom|Up%20Left%20Click%20Notification_事件)))

(fn ConstructionScript
  (|CallParentFunction))