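; BP_DarkenssGameInstance is the game instance for DarknessGame, holding task and progress state plus the bedroom music.
; It spawns a BP_TaskManager at a given location, mapping the current TaskID to its task enum, and keeps the actor reference.
; Bedroom BGM plays as a UI sound that persists across level transitions until explicitly destroyed.
; ResetGame clears the progress flags, stops the music and optionally opens StartMap.
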(event EventInit)

(fn CreateandPublishTask
  (params (Pulish%20Task%20Location :type Vector))
  (bind _returnvalue (Game|SpawnActorfromClass "/Game/DarknessGame/Blueprint/GameBlueprint/Actor/BP_TaskManager.BP_TaskManager_C" (Math|Transform|MakeTransform Pulish%20Task%20Location "0, 0, 0" "1.000000,1.000000,1.000000") "AdjustIfPossibleButAlwaysSpawn" "MultiplyWithRoot" 0 (Utilities|Select :Index (Variables|Default|GetTask%20ID) :Option%200 "NewEnumerator1" :Option%201 "NewEnumerator2" :Option%202 "NewEnumerator3" :Option%203 "NewEnumerator4") 0))
  (Variables|Default|SetTask%20Actor _returnvalue))

(fn ResetGame
  (params (In%20Level :type Boolean))
  (Variables|Default|SetTask%20ID 0)
  (Variables|Default|SetUnlocked%20Safe false)
  (Variables|Default|SetTask%20Actor 0)
  (Variables|Default|Set通关 false)
  (Variables|Default|SetDo%20One%20Start%20Game false)
  (Variables|Default|SetOne%20Ing%20LivingRoom false)
  (Variables|Default|Set第一次任务 false)
  (Variables|Default|Set第一次进入卧室 false)
  (Variables|Default|Set完成相机任务 false)
  (Variables|Default|Set第一次进入机关 false)
  (CallFunction|StopBedroomBGM)
  (if In%20Level
    (Game|OpenLevel(byName) "StartMap")))

(fn SpawnBedroomBGM
  (params (Sound :type Sound%20Base%20Object%20Reference))
  (bind _returnvalue (Audio|SpawnSound2D Sound 1.0 1.0 0.0 0 true false))
  (bind _output_get (Variables|Default|SetAudio%20Component _returnvalue))
  (Audio|Components|Audio|Play _output_get 0.0)
  (Class|AudioComponent|SetUISound _output_get true))

(fn StopBedroomBGM
  (Utilities|IsValid (Variables|Default|GetAudio%20Component)
    (:Is%20Valid
      (Audio|Components|Audio|Stop (Variables|Default|GetAudio%20Component))
      (Components|DestroyComponent (Variables|Default|GetAudio%20Component))
      (Variables|Default|SetAudio%20Component 0))))