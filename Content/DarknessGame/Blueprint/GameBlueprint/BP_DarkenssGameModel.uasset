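; BP_DarkenssGameModel manages the game's streaming levels through a MapData map of level types to level names.
; LoadStreamLevelEvent recursively preloads each level hidden with short delays, printing progress, then switches to a default level; nothing in this graph triggers it.
; SwitchLevels hides every mapped level, shows the requested one and records it for GetCurrentlyLoadingLevelName to return.
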(event Custom|Load%20Stream%20Level%20Event
  ;[0.15 0.15 0.15 0.5] 关卡预加载
  (bind _values (Utilities|Map|Values (Variables|Level|GetMap%20Data)))
  (Game|LoadStreamLevel(byName) (Utilities|String|StringToName (Utilities|Array|Get(acopy) _values (Variables|关卡|GetLoad%20Level%20ID))) false)
  (Development|PrintString (Utilities|String|Append "关卡：" (Utilities|Array|Get(acopy) _values (Variables|关卡|GetLoad%20Level%20ID)) "---已加载完成") true true "(R=0.046982,G=1.000000,B=0.000000,A=1.000000)" 1e+01)
  (Utilities|FlowControl|Delay 0.2)
  (Math|Integer|IncrementInt (Variables|关卡|GetLoad%20Level%20ID)
    (:%20%20
      (bind _values_2 (Utilities|Map|Values (Variables|Level|GetMap%20Data)))
      (if (< (Variables|关卡|GetLoad%20Level%20ID) (Utilities|Array|Length _values_2))
        (Utilities|FlowControl|Delay 0.2)
        (CallFunction|LoadStreamLevelEvent)
        (else
          (CallFunction|SwitchLevels "NewEnumerator1"))))))

(event EventBeginPlay)

(event EventTick
  (params (DeltaSeconds :type Float%20%28single-precision%29)))

(fn ConstructionScript)

(fn SwitchLevels
  (params (Level%20Tpye :type MapTypeEnum%20Enum :default "NewEnumerator0"))
  ;[0.15 0.15 0.15 0.5] 切换关卡时 关闭所有关卡 并单独显示要加载的关卡 并进行记录
  (bind _values (Utilities|Map|Values (Variables|Level|GetMap%20Data)))
  (for _array_element _values
    (Variables|/Script/Engine.LevelStreaming|SetbShouldBeVisible (Class|GameplayStatics|GetStreamingLevel (Utilities|String|StringToName _array_element)) false))
  (Variables|/Script/Engine.LevelStreaming|SetbShouldBeVisible (Class|GameplayStatics|GetStreamingLevel (Utilities|String|StringToName (.Value (Utilities|Map|Find (Variables|Level|GetMap%20Data) Level%20Tpye)))) true)
  (Variables|Default|SetCurrently%20Loading%20Level Level%20Tpye))

(fn GetCurrentlyLoadingLevelName
  ;[0.15 0.15 0.15 0.5] 获取并返回关卡
  (return (Variables|Default|GetCurrently%20Loading%20Level)))