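; Player pawn for DarknessGame with mouse edge-look camera, crouching, a wake-up animation and inner-monologue text.
; A fast looping timer turns the camera near viewport edges, one direction at a time with limited pitch, scaled by Tick's stored delta.
; A reversible timeline moves the camera for crouch and stand, switching walk speed when finished.
; An Actor Sequence plays waking up and signals completion, while a widget component displays monologue text.
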(event Custom|Squats%20Event
  (bind _charactermovement (Variables|Character|GetCharacterMovement))
  ;[0.15 0.15 0.15 0.5] 角色蹲下和战力逻辑 动画
  (bind (_direction _下蹲 _镜头曲线) (Timeline|时间轴 Play)
    (:Update
      (Transformation|SetRelativeLocation (Variables|Default|GetCamera) (Math|Vector|MakeVector 0.0 _镜头曲线 (Math|Float|Lerp 9e+01 0.0 _下蹲)) false false))
    (:Finished
      (switch Utilities|FlowControl|Switch|SwitchonETimelineDirection _direction
        (:Forward
          (Variables|/Script/Engine.CharacterMovementComponent|SetMaxWalkSpeed _charactermovement 1e+02))
        (:Backward
          (Variables|/Script/Engine.CharacterMovementComponent|SetMaxWalkSpeed _charactermovement 2e+02))))))

(event Custom|Up%20Event
  (bind _charactermovement (Variables|Character|GetCharacterMovement))
  ;[0.15 0.15 0.15 0.5] 角色蹲下和战力逻辑 动画
  (bind (_direction _下蹲 _镜头曲线) (Timeline|时间轴 Reverse)
    (:Update
      (Transformation|SetRelativeLocation (Variables|Default|GetCamera) (Math|Vector|MakeVector 0.0 _镜头曲线 (Math|Float|Lerp 9e+01 0.0 _下蹲)) false false))
    (:Finished
      (switch Utilities|FlowControl|Switch|SwitchonETimelineDirection _direction
        (:Forward
          (Variables|/Script/Engine.CharacterMovementComponent|SetMaxWalkSpeed _charactermovement 1e+02))
        (:Backward
          (Variables|/Script/Engine.CharacterMovementComponent|SetMaxWalkSpeed _charactermovement 2e+02))))))

(event Custom|WakeUp%20Animation
  (Class|ActorSequenceComponent|PlaySequence (Variables|Default|GetActorSequence)))

(event EventBeginPlay
  (Utilities|Time|SetTimerbyFunctionName 0 "Camera Movement Function" 0.001 true))

(event Collision|EventActorBeginOverlap
  (params (OtherActor :type Actor%20Object%20Reference)))

(event EventTick
  (params (DeltaSeconds :type Float%20%28single-precision%29))
  (Variables|CameraData|SetDelta%20Seconds DeltaSeconds))

(event Custom|BP_DarkenssPlayerPawn0_Event
  (params (BP_DarkenssPlayerPawn0 :type Actor%20Object%20Reference))
  (Default|CallWakeUpAnimationOverEvent))

(fn ConstructionScript)

(fn 显示内心独白
  (params (物品内容 :type String))
  (bind _aswbp_物品内容 (Utilities|Casting|CastToWBP_物品内容 (UserInterface|GetWidget (Variables|Default|GetWidget))))
  (Default|更新物品内容 _aswbp_物品内容 物品内容))

(fn CameraMovementFunction
  (bind _returnvalue (Game|GetPlayerController 0))
  (bind _returnvalue_2 (Game|GetPlayerController 0))
  ;[0.15 0.15 0.15 0.5] 相机视角移动功能实现方法 实现方法核心：实时计算鼠标在视口的位置 到设置达边缘时 计算鼠标在视口的方向并向相机添加对应的旋转
  (if (< (.LocationX (Game|Player|GetMousePosition (Game|GetPlayerController 0))) (Variables|CameraData|GetMous%20Screen%20Edge%20Distance))
    ;;[0.15 0.15 0.15 0.5] 在 -Yaw轴时 添加Yaw轴 -1输入
    (Transformation|AddWorldRotation (Variables|Default|GetCamera) (Math|Rotator|MakeRotator 0.0 0.0 (Math|Float|Lerp 0.0 -1.0 (* (Variables|CameraData|GetDelta%20Seconds) (Variables|CameraData|GetCamera%20Speed)))) false false)
    (elif (> (.LocationX (Game|Player|GetMousePosition _returnvalue_2)) (- (.SizeX (HUD|GetViewportSize _returnvalue_2)) (Variables|CameraData|GetMous%20Screen%20Edge%20Distance)))
      ;;[0.15 0.15 0.15 0.5] 在 Yaw轴时 添加Yaw轴 1输入
      (Transformation|AddWorldRotation (Variables|Default|GetCamera) (Math|Rotator|MakeRotator 0.0 0.0 (Math|Float|Lerp 0.0 1.0 (* (Variables|CameraData|GetDelta%20Seconds) (Variables|CameraData|GetCamera%20Speed)))) false false)
      (else
        ;;[0.15 0.15 0.15 0.5] 小于40 且在屏幕边缘 向上看
        (if (and (< (.LocationY (Game|Player|GetMousePosition (Game|GetPlayerController 0))) (Variables|CameraData|GetMous%20Screen%20Edge%20Distance)) (< (.pitch (Variables|/Script/Engine.SceneComponent|GetRelativeRotation (Variables|Default|GetCamera))) 4e+01))
          (Transformation|AddRelativeRotation (Variables|Default|GetCamera) (Math|Rotator|MakeRotator 0.0 (Math|Float|Lerp 0.0 1.0 (* (Variables|CameraData|GetDelta%20Seconds) (Variables|CameraData|GetCamera%20Speed))) 0.0) false false)
          (else
            ;;[0.15 0.15 0.15 0.5] 大于-40 且在屏幕边缘 向下看
            (if (and (> (.LocationY (Game|Player|GetMousePosition _returnvalue)) (- (.SizeY (HUD|GetViewportSize _returnvalue)) (Variables|CameraData|GetMous%20Screen%20Edge%20Distance))) (> (.pitch (Variables|/Script/Engine.SceneComponent|GetRelativeRotation (Variables|Default|GetCamera))) -4e+01))
              (Transformation|AddRelativeRotation (Variables|Default|GetCamera) (Math|Rotator|MakeRotator 0.0 (Math|Float|Lerp 0.0 -1.0 (* (Variables|CameraData|GetDelta%20Seconds) (Variables|CameraData|GetCamera%20Speed))) 0.0) false false))))))))