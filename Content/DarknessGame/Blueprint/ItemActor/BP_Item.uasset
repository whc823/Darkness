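; BP_Item is a configurable item actor with a world-space interaction prompt and a detection material applied to its mesh.
; The construction script applies mesh, size, tip placement and perception radius; a timeline scales the tip in or out as the player crosses that sphere.
; TriggerTouchEvent animates swaps between idle and interaction tip styles via a completion dispatcher, and the interaction tip yaws toward the player.
; SpawnSoundFunction spawns a BP_SoundLigst sound effect actor.
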(event OnComponentBeginOverlap(Sphere)
  (params (OverlappedComponent :type Primitive%20Component%20Object%20Reference) (OtherActor :type Actor%20Object%20Reference) (OtherComp :type Primitive%20Component%20Object%20Reference) (OtherBodyIndex :type Integer) (bFromSweep :type Boolean) (SweepResult :type Hit%20Result%20Structure%20%28by%20ref%29))
  ;[0.15 0.15 0.15 0.5] 玩家进入提示范围进行提示
  (if (Actor|ActorHasTag OtherActor "Player")
    (CallFunction|StartAnimationEvent)))

(event OnComponentEndOverlap(Sphere)
  (params (OverlappedComponent :type Primitive%20Component%20Object%20Reference) (OtherActor :type Actor%20Object%20Reference) (OtherComp :type Primitive%20Component%20Object%20Reference) (OtherBodyIndex :type Integer))
  ;[0.15 0.15 0.15 0.5] 玩家进入提示范围进行提示
  (if (Actor|ActorHasTag OtherActor "Player")
    (CallFunction|ReverseAnimationEnvetn)))

(event Custom|End%20Touch%20%20Prompt%20Completeion
  ;[0.15 0.15 0.15 0.5] 手部触摸 显示交互提示逻辑
  ;;[0.15 0.15 0.15 0.5] 鼠标变成三角形的过程逻辑
  (EventDispatchers|UnbindallEventsfromAnimtionCompletionNotification)
  (CallFunction|SetTipsStyle false)
  (CallFunction|StartAnimationEvent))

(event Custom|Start%20Animation%20Event
  ;[0.15 0.15 0.15 0.5] 提示动画
  (bind _新建轨道_0 (Timeline|时间轴 Play)
    (:Update
      (Transformation|SetRelativeScale3D (Variables|Default|GetItem%20Tips%20Component) (Math|Vector|Lerp(Vector) "0, 0, 0" (Math|Conversions|ToVector(Float) (Variables|ItemData|GetInitial%20Tips%20Size)) _新建轨道_0)))
    (:Finished
      (Default|CallAnimtionCompletionNotification))))

(event Custom|Start%20Touch%20Prompt%20Completeion
  ;[0.15 0.15 0.15 0.5] 手部触摸 显示交互提示逻辑
  ;;[0.15 0.15 0.15 0.5] 三角形变成鼠标的过程逻辑
  (EventDispatchers|UnbindallEventsfromAnimtionCompletionNotification)
  (CallFunction|SetTipsStyle true)
  (CallFunction|StartAnimationEvent))

(event Custom|Reverse%20Animation%20Envetn
  ;[0.15 0.15 0.15 0.5] 提示动画
  (bind _新建轨道_0 (Timeline|时间轴 Reverse)
    (:Update
      (Transformation|SetRelativeScale3D (Variables|Default|GetItem%20Tips%20Component) (Math|Vector|Lerp(Vector) "0, 0, 0" (Math|Conversions|ToVector(Float) (Variables|ItemData|GetInitial%20Tips%20Size)) _新建轨道_0)))
    (:Finished
      (Default|CallAnimtionCompletionNotification))))

(event EventBeginPlay
  (Variables|ItemData|SetInitial%20Tips%20Size (.x (Variables|/Script/Engine.SceneComponent|GetRelativeScale3D (Variables|Default|GetItem%20Tips%20Component))))
  (Transformation|SetRelativeScale3D (Variables|Default|GetItem%20Tips%20Component) "0, 0, 0"))

(event Collision|EventActorBeginOverlap
  (params (OtherActor :type Actor%20Object%20Reference)))

(event EventTick
  (params (DeltaSeconds :type Float%20%28single-precision%29))
  ;[0.15 0.15 0.15 0.5] 交互提示时 进行同步
  (if (== (Variables|/Script/Engine.StaticMeshComponent|GetStaticMesh (Variables|Default|GetItem%20Tips%20Component)) "/Game/DarknessGame/ArtAssets/Mesh/SM_SM_TipsStaticMesh02.SM_SM_TipsStaticMesh02")
    (Transformation|SetWorldRotation (Variables|Default|GetItem%20Tips%20Component) (Math|Rotator|MakeRotator 0.0 0.0 (.Yaw (Math|Rotator|BreakRotator (Math|Rotator|FindLookatRotation (Transformation|GetWorldLocation (Variables|Default|GetItem%20Tips%20Component)) (Transformation|GetActorLocation (Game|Player|GetPlayerPawn 0)))))) false false)))

(event EventTriggerTouchEvent
  (params (Trigger :type Boolean))
  ;[0.15 0.15 0.15 0.5] 手部触摸 显示交互提示逻辑
  (if Trigger
    ;;[0.15 0.15 0.15 0.5] 三角形变成鼠标的过程逻辑
    (Utilities|FlowControl|DoOnce false :!label _label
      (:Completed
        (CallFunction|ReverseAnimationEnvetn)
        (EventDispatchers|AssignAnimtionCompletionNotification (delegate Custom|Start%20Touch%20Prompt%20Completeion))
        (goto _label_2 Reset)))
    (else
      ;;[0.15 0.15 0.15 0.5] 鼠标变成三角形的过程逻辑
      (Utilities|FlowControl|DoOnce false :!label _label_2
        (:Completed
          (CallFunction|ReverseAnimationEnvetn)
          (EventDispatchers|AssignAnimtionCompletionNotification (delegate Custom|End%20Touch%20%20Prompt%20Completeion))
          (goto _label Reset))))))

(event EventSpawnSoundFunction
  ;[0.15 0.15 0.15 0.5] 声音和音波效果生成
  (bind _returnvalue (Game|SpawnActorfromClass "/Game/DarknessGame/Blueprint/BP_SoundLigst.BP_SoundLigst_C" (Math|Transform|MakeTransform (Transformation|GetWorldLocation (Variables|Default|GetC%20Sound%20Lcaiton))) "AlwaysSpawn" "MultiplyWithRoot" 0 (Variables|SoundData|GetItem%20Sound) 0))
  (Variables|SoundData|SetSound%20Actor _returnvalue))

(fn ConstructionScript
  ;[0.15 0.15 0.15 0.5] 实时设置物体模型 和同步探测效果材质
  (Components|StaticMesh|SetStaticMesh (Variables|Default|GetItem%20Static%20Mesh) (Variables|ItemData|GetItem%20Mesh))
  (for (_ _array_index) (Rendering|Material|GetMaterials (Variables|Default|GetItem%20Static%20Mesh))
    (Rendering|Material|SetMaterial (Variables|Default|GetItem%20Static%20Mesh) _array_index "/Game/DarknessGame/Blueprint/SphereMaskBlueprints/m_detection.m_detection"))
  (Transformation|SetRelativeScale3D (Variables|Default|GetItem%20Static%20Mesh) (Math|Conversions|ToVector(Float) (Variables|ItemData|GetItem%20Size)))
  (Transformation|SetRelativeLocation (Variables|Default|GetItem%20Tips%20Component) (Variables|ItemData|GetItem%20Tips%20Location) false false)
  (CallFunction|SetTipsStyle false)
  (Components|Sphere|SetSphereRadius (Variables|Default|GetSphere) (Variables|ItemData|GetPerception%20Player%20Range) true)
  (Transformation|SetRelativeLocation (Variables|Default|GetC%20Sound%20Lcaiton) (Variables|SoundData|GetSound%20Location) false false))

(fn SetTipsStyle
  (params (Interaction%20Tips :type Boolean))
  (Components|StaticMesh|SetStaticMesh (Variables|Default|GetItem%20Tips%20Component) (select Interaction%20Tips "/Game/DarknessGame/ArtAssets/Mesh/SM_SM_TipsStaticMesh02.SM_SM_TipsStaticMesh02" "/Game/DarknessGame/ArtAssets/Mesh/SM_TipsStaticMesh01.SM_TipsStaticMesh01"))
  (Rendering|Material|SetMaterial (Variables|Default|GetItem%20Tips%20Component) 0 (select Interaction%20Tips "/Game/DarknessGame/ArtAssets/Materials/M_ItemTipsMaterial.M_ItemTipsMaterial" "/Game/DarknessGame/ArtAssets/Materials/M_Basic_Wall.M_Basic_Wall")))