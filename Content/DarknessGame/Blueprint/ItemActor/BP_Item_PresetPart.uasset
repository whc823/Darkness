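; BP_Item_PresetPart is a part item actor that the player can grab, drop or install.
; On a click, if the player controller permits grabbing, it attaches to the hand actor and updates the controller's crawling (grab) permission.
; Clicking while held either installs it, firing an installation notification and destroying the actor, or detaches it when installation is not allowed.
; BeginPlay hides its tips, sphere and location components and disables sphere collision.
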(event Custom|进行安装
  (Default|CallInstallingOntifiction self)
  (Variables|Default|SetInstalling true)
  (Class|IBPControllerCommunicationInterface|UpdateCrawlingPermission(Message) (Game|GetPlayerController 0) true)
  (Actor|DestroyActor))

(event EventBeginPlay
  (|CallParentFunction)
  (Rendering|SetVisibility (Variables|Default|GetItem%20Tips%20Component) false false)
  (Collision|SetCollisionEnabled (Variables|Default|GetSphere) "NoCollision"))

(event Collision|EventActorBeginOverlap
  (params (OtherActor :type Actor%20Object%20Reference))
  (|CallParentFunction OtherActor) ; 此节点被禁用，将不会被调用。\n从引脚连出引线来编译功能。
)

(event EventTick
  (params (DeltaSeconds :type Float%20%28single-precision%29))
  (|CallParentFunction DeltaSeconds) ; 此节点被禁用，将不会被调用。\n从引脚连出引线来编译功能。
)

(event EventMouseClickEvent
  (params (Hand%20Actor :type Actor%20Object%20Reference))
  (if (Variables|Default|GetBeing%20Crawled)
    (if (Variables|Default|GetAllow%20Installation)
      (CallFunction|进行安装)
      (else
        (Transformation|DetachFromActor "KeepWorld" "KeepWorld" "KeepWorld")
        (Class|IBPControllerCommunicationInterface|UpdateCrawlingPermission(Message) (Game|GetPlayerController 0) true)
        (Variables|Default|SetBeing%20Crawled false)))
    (else
      (bind _allow_ (Class|IBPControllerCommunicationInterface|QueryWhetherItemCanGrabbed(Message) (Game|GetPlayerController 0)))
      (if _allow_
        (Transformation|AttachActorToActor Hand%20Actor "None" "KeepWorld" "KeepWorld" "KeepWorld" false)
        (Class|IBPControllerCommunicationInterface|UpdateCrawlingPermission(Message) (Game|GetPlayerController 0) false)
        (Variables|Default|SetBeing%20Crawled true)))))

(fn ConstructionScript
  (|CallParentFunction))