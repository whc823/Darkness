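; BP_Item_Story is an item actor that shows story text through a widget component when its mouse click event fires.
; The click event passes its story string to the WBP_物品内容 widget on StoryContentWidget, then destroys the linked SoundActor if it is valid.
; The construction script positions the widget component from a transform variable, after running the parent's construction logic.
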(event EventBeginPlay
  (|CallParentFunction))

(event Collision|EventActorBeginOverlap
  (params (OtherActor :type Actor%20Object%20Reference))
  (|CallParentFunction OtherActor) ; 此节点被禁用，将不会被调用。\n从引脚连出引线来编译功能。
)

(event EventTick
  (params (DeltaSeconds :type Float%20%28single-precision%29))
  (|CallParentFunction DeltaSeconds) ; 此节点被禁用，将不会被调用。\n从引脚连出引线来编译功能。
)

(event EventMouseClickEvent
  (params (Hand%20Actor :type Actor%20Object%20Reference))
  ;[0.15 0.15 0.15 0.5] 鼠标点击事件
  (bind _aswbp_物品内容 (Utilities|Casting|CastToWBP_物品内容 (UserInterface|GetWidget (Variables|Default|GetStory%20Content%20Widget))))
  (Default|更新物品内容 _aswbp_物品内容 (Variables|Default|GetStroy%20Content%20String))
  (Utilities|IsValid (Variables|Default|GetSound%20Actor)
    (:Is%20Valid
      (Actor|DestroyActor (Variables|Default|GetSound%20Actor)))))

(fn ConstructionScript
  (|CallParentFunction)
  (Transformation|SetRelativeTransform (Variables|Default|GetStory%20Content%20Widget) (Variables|Default|GetStroy%20Widget%20Transform) false false))