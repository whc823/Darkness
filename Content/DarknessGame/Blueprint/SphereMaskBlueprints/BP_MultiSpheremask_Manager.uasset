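; Manager that arbitrates priority between overlapping sphere-mask world changers, deciding which one may hide an item.
; BeginPlay builds a mask-tag list from the world changer array, whose index gives each sphere's priority ID.
; Spheres ask to override or release items; the manager compares their ID with the item's tag-derived ID and calls back.
; Duplicate override component tags act as a counter, one added per override and one removed per release.
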(event EventBeginPlay
  (bind _bp_world_changer_list (Variables|Default|GetBp_World_Changer_List))
  ;[0.06447 0.1855 1] Get all worldchanger tag and put it in a list in ID order
  (for (_array_element _array_index) _bp_world_changer_list
    (Utilities|Array|Insert (Variables|Default|GetWorldChangerListTag) (Variables|/Game/DarknessGame/Blueprint/SphereMaskBlueprints/BP_WorldChanger.BP_WorldChanger_C|GetTag%20In%20Mask _array_element) _array_index))
  (Variables|Default|SetNumber%20of%20World%20changer (- (Utilities|Array|Length _bp_world_changer_list) 1)))

(event EventAskHasBeenOverride
  (params (ItemToCheck :type Primitive%20Component%20Object%20Reference) (From :type BP%20World%20Changer%20Object%20Reference))
  (bind _componenttags (Variables|/Script/Engine.ActorComponent|GetComponentTags ItemToCheck))
  ;[0.06447 0.1855 1] Check if the item is colliding with higher sphere priority than it should be
  ;;[0.1406 0.1406 0.1406] Has not been overriden
  (if (Components|ComponentHasTag ItemToCheck (Variables|Default|GetOverrideTag))
    ;;[0.1406 0.1406 0.1406] Get the id (spheremask) of the item by comparing the tag in the list
    (bind _array_element (Utilities|Array|ForEachLoopwithBreak _componenttags :!label _label)
      (:LoopBody
        (for (_array_element_2 _array_index) (Variables|Default|GetWorldChangerListTag)
          (if (== _array_element _array_element_2)
            (Variables|Default|SetTag%20To%20ID%20Sphere _array_index)
            (goto _label Break))))
      (:Completed
        ;;[0.1406 0.1406 0.1406] if sphere id is greater than item sphere id
        (if (> (Variables|/Game/DarknessGame/Blueprint/SphereMaskBlueprints/BP_WorldChanger.BP_WorldChanger_C|GetIDSphere From) (Variables|Default|GetTag%20To%20ID%20Sphere))
          ;;[0.1406 0.1406 0.1406] Remove a "Override tag" occurence (if 1 is still here then the item is still override"
          (bind (_array_element_3 _array_index_2) (Utilities|Array|ForEachLoopwithBreak _componenttags :!label _label_2)
            (:LoopBody
              (if (== _array_element_3 (Variables|Default|GetOverrideTag))
                (Utilities|Array|RemoveIndex _componenttags _array_index_2)
                (goto _label_2 Break)))
            (:Completed
              (Default|AnswerHasBeenOverride From true ItemToCheck))))))
    (else
      (Default|AnswerHasBeenOverride From false ItemToCheck))))

(event EventAskOverride
  (params (Item%20to%20override :type Primitive%20Component%20Object%20Reference) (From :type BP%20World%20Changer%20Object%20Reference))
  (bind _componenttags (Variables|/Script/Engine.ActorComponent|GetComponentTags Item%20to%20override))
  ;[0.06447 0.1855 1] Check if a spheremask has priority to hide the item. Example : id : 4 has priority on id : 0,1,2,3. but not on id : 5
  ;;[0.1406 0.1406 0.1406] Get the id (spheremask) of the item by comparing the tag in the list
  (bind _array_element (Utilities|Array|ForEachLoopwithBreak (Variables|/Script/Engine.ActorComponent|GetComponentTags Item%20to%20override) :!label _label)
    (:LoopBody
      (for (_array_element_2 _array_index) (Variables|Default|GetWorldChangerListTag)
        (if (== _array_element _array_element_2)
          (Variables|Default|SetTag%20To%20ID%20Sphere _array_index)
          (goto _label Break))))
    (:Completed
      ;;[0.1406 0.1406 0.1406] if sphere id is greater than item sphere id
      (if (> (Variables|/Game/DarknessGame/Blueprint/SphereMaskBlueprints/BP_WorldChanger.BP_WorldChanger_C|GetIDSphere From) (Variables|Default|GetTag%20To%20ID%20Sphere))
        ;;[0.1406 0.1406 0.1406] If overriden Add a tag to identifie later
        (Utilities|Array|Insert _componenttags (Variables|Default|GetOverrideTag) (Utilities|Array|Length _componenttags))
        (Default|AnswerOverride From true Item%20to%20override)
        (else
          (Default|AnswerOverride From false Item%20to%20override))))))

(fn ConstructionScript)