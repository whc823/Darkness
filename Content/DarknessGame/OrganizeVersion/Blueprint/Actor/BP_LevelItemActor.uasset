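; BP_LevelItemActor is a placeable level item with an interaction tip that swaps between a triangle and a mouse prompt on hand touch.
; Construction loads the item mesh from a data table, overrides its materials with M_detection and positions sound, story widget and tip components.
; DoOnce-gated touch events reverse a scale timeline, swap tip mesh and material via a completion dispatcher, then replay it.
; Tick yaws the mouse prompt toward the player.
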(event Custom|End%20Touch%20%20Prompt%20Completeion
  ;[0.15 0.15 0.15 0.5] 手部触摸 显示交互提示逻辑
  ;;[0.15 0.15 0.15 0.5] 鼠标变成三角形的过程逻辑
  (EventDispatchers|UnbindallEventsfromAnimtionCompletionNotification)
  (CallFunction|SetTipsStyle false)
  (CallFunction|StartAnimationEvent))

(event Custom|Show%20Triangle
  ;[0.15 0.15 0.15 0.5] 手部触摸 显示交互提示逻辑
  ;;[0.15 0.15 0.15 0.5] 鼠标变成三角形的过程逻辑
  (CallFunction|ReverseAnimationEnvetn)
  (EventDispatchers|BindEventtoAnimtionCompletionNotification (delegate Custom|End%20Touch%20%20Prompt%20Completeion))
  ;;[0.15 0.15 0.15 0.5] 三角形变成鼠标的过程逻辑
  (Utilities|FlowControl|DoOnce false) ; enters at Reset
)

(event Custom|Start%20Animation%20Event
  (bind _item_tips_component (Variables|Default|GetItem%20Tips%20Component))
  ;[0.15 0.15 0.15 0.5] 提示动画
  (bind _新建轨道_0 (Timeline|时间轴 PlayFromStart)
    (:Update
      (Utilities|IsValid _item_tips_component
        (:Is%20Valid
          (Transformation|SetRelativeScale3D _item_tips_component (Math|Vector|Lerp(Vector) "0, 0, 0" (Math|Conversions|ToVector(Float) (Variables|ItemBasicData|GetInitial%20Tips%20Size)) _新建轨道_0)))))
    (:Finished
      (Default|CallAnimtionCompletionNotification))))

(event Custom|Start%20Touch%20Prompt%20Completeion
  ;[0.15 0.15 0.15 0.5] 手部触摸 显示交互提示逻辑
  ;;[0.15 0.15 0.15 0.5] 三角形变成鼠标的过程逻辑
  (EventDispatchers|UnbindallEventsfromAnimtionCompletionNotification)
  (CallFunction|SetTipsStyle true)
  (CallFunction|StartAnimationEvent))

(event Custom|Reverse%20Animation%20Envetn
  (bind _item_tips_component (Variables|Default|GetItem%20Tips%20Component))
  ;[0.15 0.15 0.15 0.5] 提示动画
  (bind _新建轨道_0 (Timeline|时间轴 ReverseFromEnd)
    (:Update
      (Utilities|IsValid _item_tips_component
        (:Is%20Valid
          (Transformation|SetRelativeScale3D _item_tips_component (Math|Vector|Lerp(Vector) "0, 0, 0" (Math|Conversions|ToVector(Float) (Variables|ItemBasicData|GetInitial%20Tips%20Size)) _新建轨道_0)))))
    (:Finished
      (Default|CallAnimtionCompletionNotification))))

(event Custom|Show%20Mouse
  ;[0.15 0.15 0.15 0.5] 手部触摸 显示交互提示逻辑
  ;;[0.15 0.15 0.15 0.5] 三角形变成鼠标的过程逻辑
  (CallFunction|ReverseAnimationEnvetn)
  (EventDispatchers|BindEventtoAnimtionCompletionNotification (delegate Custom|Start%20Touch%20Prompt%20Completeion))
  ;;[0.15 0.15 0.15 0.5] 鼠标变成三角形的过程逻辑
  (Utilities|FlowControl|DoOnce false) ; enters at Reset
)

(event EventBeginPlay)

(event Collision|EventActorBeginOverlap
  (params (OtherActor :type Actor%20Object%20Reference)))

(event EventTick
  (params (DeltaSeconds :type Float%20%28single-precision%29))
  ;[0.15 0.15 0.15 0.5] 交互提示时 进行同步
  (if (== (Variables|/Script/Engine.StaticMeshComponent|GetStaticMesh (Variables|Default|GetItem%20Tips%20Component)) "/Game/DarknessGame/ArtAssets/Mesh/SM_SM_TipsStaticMesh02.SM_SM_TipsStaticMesh02")
    (Transformation|SetWorldRotation (Variables|Default|GetItem%20Tips%20Component) (Math|Rotator|MakeRotator 0.0 0.0 (.Yaw (Math|Rotator|BreakRotator (Math|Rotator|FindLookatRotation (Transformation|GetWorldLocation (Variables|Default|GetItem%20Tips%20Component)) (Transformation|GetActorLocation (Game|Player|GetPlayerPawn 0)))))) false false)))

(event EventTriggerTouchEvent
  (params (Trigger :type Boolean))
  ;[0.15 0.15 0.15 0.5] 手部触摸 显示交互提示逻辑
  (if Trigger
    ;;[0.15 0.15 0.15 0.5] 三角形变成鼠标的过程逻辑
    (Utilities|FlowControl|DoOnce false :!label _label
      (:Completed
        (CallFunction|ReverseAnimationEnvetn)
        (EventDispatchers|BindEventtoAnimtionCompletionNotification (delegate Custom|Start%20Touch%20Prompt%20Completeion))
        (goto _label_2 Reset)))
    (else
      ;;[0.15 0.15 0.15 0.5] 鼠标变成三角形的过程逻辑
      (Utilities|FlowControl|DoOnce false :!label _label_2
        (:Completed
          (CallFunction|ReverseAnimationEnvetn)
          (EventDispatchers|BindEventtoAnimtionCompletionNotification (delegate Custom|End%20Touch%20%20Prompt%20Completeion))
          (goto _label Reset))))))

(fn ConstructionScript
  (bind _item_table_data (Variables|ItemBasicData|GetItem%20Table%20Data))
  (bind _returnvalue (Utilities|GetDataTableRow (.datatable _item_table_data) (.rowname _item_table_data))
    (:then
      (Components|StaticMesh|SetStaticMesh (Variables|Default|GetLevel%20Item%20Static%20Mesh) (.ItemStaticMehs (Utilities|Struct|BreakItemStruct _returnvalue)))
      (Transformation|SetRelativeScale3D (Variables|Default|GetLevel%20Item%20Static%20Mesh) (Math|Conversions|ToVector(Float) (Variables|ItemBasicData|GetInitial%20Tips%20Size)))
      (for (_ _array_index) (Rendering|Material|GetMaterials (Variables|Default|GetLevel%20Item%20Static%20Mesh))
        (Rendering|Material|SetMaterial (Variables|Default|GetLevel%20Item%20Static%20Mesh) _array_index "/Game/DarknessGame/Blueprint/SphereMaskBlueprints/m_detection.m_detection"))
      (Transformation|SetRelativeLocation (Variables|Default|GetSound%20Lcaiton) (Variables|ItemBasicData|GetSound%20Location) false false)
      (Transformation|SetRelativeTransform (Variables|Default|GetStory%20Content%20Widget) (Variables|ItemBasicData|GetStroy%20Widget%20Transform) false false)
      (Transformation|SetRelativeLocation (Variables|Default|GetItem%20Tips%20Component) (Variables|Default|GetItem%20Tips%20Location) false false)
      (CallFunction|SetTipsStyle false))))

(fn SetTipsStyle
  (params (Interaction%20Tips :type Boolean))
  (Utilities|IsValid (Variables|Default|GetItem%20Tips%20Component)
    (:Is%20Valid
      (Components|StaticMesh|SetStaticMesh (Variables|Default|GetItem%20Tips%20Component) (select Interaction%20Tips "/Game/DarknessGame/ArtAssets/Mesh/SM_SM_TipsStaticMesh02.SM_SM_TipsStaticMesh02" "/Game/DarknessGame/ArtAssets/Mesh/SM_TipsStaticMesh01.SM_TipsStaticMesh01"))
      (Rendering|Material|SetMaterial (Variables|Default|GetItem%20Tips%20Component) 0 (select Interaction%20Tips "/Game/DarknessGame/ArtAssets/Materials/M_ItemTipsMaterial.M_ItemTipsMaterial" "/Game/DarknessGame/ArtAssets/Materials/M_Basic_Wall.M_Basic_Wall")))))

(fn GetItemData
  (return "" ""))