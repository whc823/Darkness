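; Game-model Blueprint for a dream-escape game, managing streamed levels and player arrival in each.
; In GameMainMap, BeginPlay preloads every MapData level hidden through a delayed recursive event, then shows the start level.
; SwitchLevels toggles level visibility, moves the pawn to the tag-matched PlayerStart, and updates cursor, widget and camera.
; Outside the start level, a wake-up animation leads into first-visit or return monologues; EndPlay runs a delayed unload loop.
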(event Custom|Wake%20Up%20Aniamtion%20Comp%20Event
  ;[0.15 0.15 0.15 0.5] 玩家起身动画完成时
  (bind _firset_entry_level_ (CallFunction|QueryIsFirsetTimeinLevel (Variables|关卡|GetCurrently%20Loading%20Level)))
  (if _firset_entry_level_
    (CallFunction|UpdataIsFiresetTimerinLevel (Variables|关卡|GetCurrently%20Loading%20Level) false)
    ;[0.15 0.15 0.15 0.5] 关卡进入时播放内容
    (switch Utilities|FlowControl|Switch|SwitchonMapTypeEnum (Variables|关卡|GetCurrently%20Loading%20Level)
      (:NewEnumerator2
        (bind _hud (CallFunction|GetGameHUD))
        (Default|PlayPlayerInnerMonologue _hud "Where am I? Wasn’t I in my own bed/"))
      (:NewEnumerator3
        (bind _hud_2 (CallFunction|GetGameHUD))
        (Default|PlayPlayerInnerMonologue _hud_2 "What the hell is going on/ 
 
Why am I still not waking up in my bed? What’s happening/ 
 
.../ 
 
Stay calm, Harrison. Think. There’s got to be a way out of this dream/"))
      (:NewEnumerator4
        (bind _hud_3 (CallFunction|GetGameHUD))
        (Default|PlayPlayerInnerMonologue _hud_3 "Ouch! okay it’s actually not hurt, it’s just a dream/ 
 
.../ 
 
This is... my room/"))
      (:NewEnumerator5
        (bind _hud_4 (CallFunction|GetGameHUD))
        (Default|PlayPlayerInnerMonologue _hud_4 "I am ready/")))
    (else
      (switch Utilities|FlowControl|Switch|SwitchonMapTypeEnum (Variables|关卡|GetCurrently%20Loading%20Level)
        (:NewEnumerator2
          (bind _hud_5 (CallFunction|GetGameHUD))
          (Default|PlayPlayerInnerMonologue _hud_5 "This time… I’m ready to open the door/"))
        (:NewEnumerator3
          (bind _hud_6 (CallFunction|GetGameHUD))
          (Default|PlayPlayerInnerMonologue _hud_6 "I am back/"))))))

(event Custom|Load%20Stream%20Level%20Event
  ;[0.15 0.15 0.15 0.5] 关卡预加载
  (bind _values (Utilities|Map|Values (Variables|Level|GetMap%20Data)))
  (Game|LoadStreamLevel(byName) (Utilities|String|StringToName (Utilities|Array|Get(acopy) _values (Variables|关卡|GetLoad%20Level%20ID))) false)
  (Development|PrintString (Utilities|String|Append "关卡：" (Utilities|Array|Get(acopy) _values (Variables|关卡|GetLoad%20Level%20ID)) "---已加载完成") true true "(R=0.046982,G=1.000000,B=0.000000,A=1.000000)" 2e+01)
  (Utilities|FlowControl|Delay 0.2)
  (Math|Integer|IncrementInt (Variables|关卡|GetLoad%20Level%20ID)
    (:%20%20
      (bind _values_2 (Utilities|Map|Values (Variables|Level|GetMap%20Data)))
      (if (< (Variables|关卡|GetLoad%20Level%20ID) (Utilities|Array|Length _values_2))
        (Utilities|FlowControl|Delay 0.2)
        (CallFunction|LoadStreamLevelEvent)
        (else
          (bind _outactors (Actor|GetAllActorsOfClass "/Script/Engine.PlayerStart"))
          (Variables|关卡|SetPlayer%20Spawn%20Point%20Data _outactors)
          (CallFunction|SwitchLevels "NewEnumerator1"))))))

(event EventBeginPlay
  (bind _returnvalue (Game|GetCurrentLevelName true))
  (if (Utilities|Enum|Equal(Enum) _returnvalue "GameMainMap")
    (CallFunction|LoadStreamLevelEvent)
    (else
      (Utilities|FlowControl|Delay 0.5)
      (CallFunction|SwichGanemWidget "NewEnumerator2")
      (CallFunction|PlayPlayerCameraAniatmion false))))

(event EventTick
  (params (DeltaSeconds :type Float%20%28single-precision%29)))

(event EventEndPlay
  (params (EndPlayReason :type EEndPlayReason%20Enum :default "Destroyed"))
  ;[0.15 0.15 0.15 0.5] 游戏结束卸载所有关卡
  (bind _values (Utilities|Map|Values (Variables|Level|GetMap%20Data) :!label _label))
  (Variables|关卡|SetLoad%20Level%20ID 0)
  (Game|UnloadStreamLevel(byName) (Utilities|String|StringToName (Utilities|Array|Get(acopy) _values (Variables|关卡|GetLoad%20Level%20ID))) false)
  (Utilities|FlowControl|Delay 0.2)
  (Math|Integer|IncrementInt (Variables|关卡|GetLoad%20Level%20ID)
    (:%20%20
      (bind _values_2 (Utilities|Map|Values (Variables|Level|GetMap%20Data)))
      (if (< (Variables|关卡|GetLoad%20Level%20ID) (Utilities|Array|Length _values_2))
        (Utilities|FlowControl|Delay 0.2)
        (goto _label)))))

(fn ConstructionScript)

(fn SwitchLevels
  (params (Level%20Tpye :type MapTypeEnum%20Enum :default "NewEnumerator0"))
  (Variables|关卡|SetCurrently%20Loading%20Level Level%20Tpye)
  (bind _values (Utilities|Map|Values (Variables|Level|GetMap%20Data)))
  (for _array_element _values
    (Variables|/Script/Engine.LevelStreaming|SetbShouldBeVisible (Class|GameplayStatics|GetStreamingLevel (Utilities|String|StringToName _array_element)) false))
  (Variables|/Script/Engine.LevelStreaming|SetbShouldBeVisible (Class|GameplayStatics|GetStreamingLevel (Utilities|String|StringToName (.Value (Utilities|Map|Find (Variables|Level|GetMap%20Data) Level%20Tpye)))) true)
  (CallFunction|LevelCompletesSwitching))

(fn GetCurrentlyLoadingLevelName
  ;[0.15 0.15 0.15 0.5] 获取并返回关卡
  (return (Variables|关卡|GetCurrently%20Loading%20Level)))

(fn LevelCompletesSwitching
  (bind _map_data (Variables|Level|GetMap%20Data))
  (bind _currently_loading_level (Variables|关卡|GetCurrently%20Loading%20Level))
  (bind _value (Utilities|Map|Find _map_data _currently_loading_level))
  (if (Utilities|Enum|NotEqual(Enum) (Variables|关卡|GetCurrently%20Loading%20Level) "NewEnumerator1")
    (bind _player_character (CallFunction|PlayPlayerCameraAniatmion false))
    (Default|WakeUpAnimation _player_character)
    (EventDispatchers|BindEventtoWakeUpAnimationOverEvent _player_character (EventDispatchers|CreateEvent :!event Custom|Wake%20Up%20Aniamtion%20Comp%20Event)))
  (for _array_element (Variables|关卡|GetPlayer%20Spawn%20Point%20Data)
    (Development|PrintString (Utilities|String|Append "玩家出生点标签为：" (Utilities|String|ToString(Name) (Utilities|Array|Get(acopy) (Variables|/Script/Engine.Actor|GetTags _array_element))) "寻找的关卡：" _value) true true "(R=0.000000,G=0.660000,B=1.000000,A=1.000000)" 1.2e+02)
    (if (Actor|ActorHasTag _array_element (Utilities|String|StringToName _value))
      (LocalVariables|SetPlayer%20Generation%20Position _array_element)))
  (Transformation|SetActorTransform (Game|Player|GetPlayerPawn 0) (Math|Transform|MakeTransform (.location (Transformation|GetActorTransform (LocalVariables|GetPlayer%20Generation%20Position))) (.rotation (Transformation|GetActorTransform (LocalVariables|GetPlayer%20Generation%20Position))) "1.000000,1.000000,1.000000"))
  (CallFunction|UpdateGameMouseCursor (Utilities|Select :Index (Variables|关卡|GetCurrently%20Loading%20Level) :NewEnumerator0 "Default" :NewEnumerator1 "CardinalCross" :NewEnumerator2 "Default" :NewEnumerator3 "Default" :NewEnumerator4 "Default" :NewEnumerator5 "Default"))
  (CallFunction|SwichGanemWidget (Variables|关卡|GetCurrently%20Loading%20Level))
  (CallFunction|PlayPlayerCameraAniatmion false))