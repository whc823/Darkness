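; HUD Blueprint that owns the main UI, mouse cursor and player inner-monologue display.
; On BeginPlay it adds the main widget to the viewport, sets a gaming widget as the custom CardinalCross cursor, and selects the initial screen.
; Helper functions toggle the cursor and forward screen switches to the main widget.
; Monologue content passes to its child widget, whose animation-finished event is bound for relaying completion through the HUD's dispatcher.
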(event Custom|Complete%20Player%20Inner%20Monologue%20Animation
  ;[0.15 0.15 0.15 0.5] 玩家内心独白完成时
  (Default|CallCompletePlayerInnerMonologue))

(event EventBeginPlay
  (bind _returnvalue (UserInterface|CreateWidget "/Game/DarknessGame/Blueprint/GameBlueprint/GameUMG/WBP_MainWidget.WBP_MainWidget_C"))
  (bind _output_get (Variables|Default|SetMain%20Widget _returnvalue))
  (UserInterface|Viewport|AddtoViewport _output_get 99)
  (bind _returnvalue_2 (UserInterface|CreateWidget "/Game/DarknessGame/Blueprint/GameBlueprint/GameUMG/WBP_GameingWidget.WBP_GameingWidget_C"))
  (Variables|Default|SetTransparent%20Mouse%20Cursor%20Controls _returnvalue_2)
  (CallFunction|UpdateMouseCursor "Default")
  (CallFunction|SwitchHUDWidget "NewEnumerator0"))

(event Collision|EventActorBeginOverlap
  (params (OtherActor :type Actor%20Object%20Reference)))

(event EventTick
  (params (DeltaSeconds :type Float%20%28single-precision%29)))

(fn ConstructionScript)

(fn UpdateMouseCursor
  (params (当前鼠标光标 :type EMouseCursor%20Enum :default "None"))
  (bind _returnvalue (Game|GetPlayerController 0))
  (if (Utilities|Enum|Equal(Enum) 当前鼠标光标 "Default")
    (Variables|/Script/Engine.PlayerController|SetCurrentMouseCursor _returnvalue "CardinalCross")
    (Class|PlayerController|SetMouseCursorWidget _returnvalue "CardinalCross" (Variables|Default|GetTransparent%20Mouse%20Cursor%20Controls))
    (else
      (Variables|/Script/Engine.PlayerController|SetCurrentMouseCursor (Game|GetPlayerController 0) "Default"))))

(fn SwitchHUDWidget
  (params (Level%20Name :type MapTypeEnum%20Enum :default "NewEnumerator0"))
  (Default|SwitchGanemWidget (Variables|Default|GetMain%20Widget) Level%20Name))

(fn PlayPlayerInnerMonologue
  (params (内容独白整体内容 :type String))
  (bind _main_widget (Variables|Default|GetMain%20Widget))
  (bind _wbp_内心独白 (Variables|/Game/DarknessGame/Blueprint/GameBlueprint/GameUMG/WBP_MainWidget.WBP_MainWidget_C|GetWBP_内心独白 _main_widget))
  (Default|更新物品内容 _wbp_内心独白 内容独白整体内容)
  (EventDispatchers|BindEventto完成动画 _wbp_内心独白 (EventDispatchers|CreateEvent :!event Custom|Complete%20Player%20Inner%20Monologue%20Animation)))