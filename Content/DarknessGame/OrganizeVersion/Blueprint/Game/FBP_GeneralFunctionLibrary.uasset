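; Blueprint function library of global shortcuts to the game's mode, HUD and player pawn.
; Each function casts the game mode, player 0's HUD or player 0's character to its BP_OV class and forwards a call or returns a value.
; It covers level switching, the loading level name, mouse cursor updates, HUD widget switching, forward or reverse camera animation, and HUD access.
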(fn SwitchGameLevels
  (params (Map :type MapTypeEnum%20Enum :default "NewEnumerator0"))
  (bind _asbp_ov_game_model (Utilities|Casting|CastToBP_OV_GameModel (Game|GetGameMode)))
  (Default|SwitchLevels _asbp_ov_game_model Map))

(fn GetGameLoadingLevelName
  (bind _asbp_ov_game_model (Utilities|Casting|CastToBP_OV_GameModel (Game|GetGameMode)))
  (return (Variables|/Game/DarknessGame/OrganizeVersion/Blueprint/Game/BP_OV_GameModel.BP_OV_GameModel_C|GetCurrently%20Loading%20Level _asbp_ov_game_model)))

(fn UpdateGameMouseCursor
  (params (当前鼠标光标 :type EMouseCursor%20Enum :default "None"))
  (bind _asbp_ov_hud (Utilities|Casting|CastToBP_OV_HUD (HUD|GetHUD (Game|GetPlayerController 0))))
  (Default|UpdateMouseCursor _asbp_ov_hud 当前鼠标光标))

(fn SwichGanemWidget
  (params (Level%20Name :type MapTypeEnum%20Enum :default "NewEnumerator0"))
  (bind _asbp_ov_hud (Utilities|Casting|CastToBP_OV_HUD (HUD|GetHUD (Game|GetPlayerController 0))))
  (Default|SwitchHUDWidget _asbp_ov_hud Level%20Name))

(fn PlayPlayerCameraAniatmion
  (params (Play? :type Boolean))
  (bind _asbp_ov_player_pawn (Utilities|Casting|CastToBP_OV_PlayerPawn (Game|GetPlayerCharacter 0)))
  (if Play?
    (Default|StartCameraAnimation _asbp_ov_player_pawn)
    (else
      (Default|ReverseCamerAnimation _asbp_ov_player_pawn))))

(fn GetGameHUD
  (bind _asbp_ov_hud (Utilities|Casting|CastToBP_OV_HUD (HUD|GetHUD (Game|GetPlayerController 0))))
  (return _asbp_ov_hud))