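; BP_Ligst is an interactable actor that plays a configurable sound and shows a 3D icon turned toward the player.
; BeginPlay assigns the sound-effect variable to its Audio component and starts playback.
; Tick yaws the icon toward the player pawn with a -90 degree offset, preserving its pitch and roll.
; The actor destroys itself when the audio finishes or when its interaction event (进行交互) fires.
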(event OnAudioFinished(Audio)
  (Actor|DestroyActor))

(event Custom|进行交互
  (Actor|DestroyActor))

(event EventBeginPlay
  (Variables|/Script/Engine.AudioComponent|SetSound (Variables|Default|GetAudio) (Variables|Default|Get音效))
  (Audio|Components|Audio|Play (Variables|Default|GetAudio) 0.0))

(event Collision|EventActorBeginOverlap
  (params (OtherActor :type Actor%20Object%20Reference)))

(event EventTick
  (params (DeltaSeconds :type Float%20%28single-precision%29))
  (bind _ns_icon3d_ting (Variables|Default|GetNS_Icon3D_Ting))
  (bind _returnvalue (Transformation|GetWorldRotation _ns_icon3d_ting))
  (Transformation|SetWorldRotation (Variables|Default|GetNS_Icon3D_Ting) (Math|Rotator|MakeRotator (.roll _returnvalue) (.pitch _returnvalue) (+ (.yaw (Math|Rotator|FindLookatRotation (Transformation|GetActorLocation) (Transformation|GetActorLocation (Game|Player|GetPlayerPawn 0)))) -9e+01)) false false))

(fn ConstructionScript)