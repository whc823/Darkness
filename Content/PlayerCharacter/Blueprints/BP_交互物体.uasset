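; Interactable world item with a configurable model, a floating prompt, an item-content widget and optional looping-agnostic sound actor.
; The construction script applies the mesh and component placements; BeginPlay can spawn BP_Ligst at the sound location.
; A timeline scales the prompt in and out, swapping mesh marker and mouse-icon widget between reverse and replay, while Tick yaws the widget toward the player.
; Showing content fills the item widget and destroys the sound actor.
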(event Custom|显示鼠标
  (Variables|Default|Set正在显示鼠标 true)
  (CallFunction|隐藏提示))

(event Custom|隐藏鼠标
  (Variables|Default|Set正在隐藏鼠标 true)
  (CallFunction|隐藏提示))

(event Custom|显示内容
  (bind _aswbp_物品内容 (Utilities|Casting|CastToWBP_物品内容 (UserInterface|GetWidget (Variables|Default|GetWidget1)))
    (:then
      (Default|更新物品内容 _aswbp_物品内容 (Variables|Default|Get物品内容)))
    (:CastFailed
      _))
  (Utilities|IsValid (Variables|Default|Get音效对象)
    (:Is%20Valid
      (Actor|DestroyActor (Variables|Default|Get音效对象)))))

(event Custom|显示提示
  ;[1 0 0 0.5] 提示UI 的缩放动画时间轴
  (bind (_direction _新建轨道_0) (Timeline|时间轴 Play)
    (:Update
      (Transformation|SetRelativeScale3D (Variables|Default|GetTips%20Statcic%20Mesh) (Math|Vector|Lerp(Vector) "0, 0, 0" (Variables|Default|Get提示控件默认缩放) _新建轨道_0)))
    (:Finished
      (switch Utilities|FlowControl|Switch|SwitchonETimelineDirection _direction
        (:Forward
          (Variables|Default|Set同步提示 true))
        (:Backward
          (Variables|Default|Set同步提示 false)
          (if (Variables|Default|Get正在显示鼠标)
            (Rendering|SetVisibility (Variables|Default|GetWidget) true true)
            (Rendering|SetVisibility (Variables|Default|GetTips%20Statcic%20Mesh) false false)
            (CallFunction|更新图标 "/Game/PlayerCharacter/Texture/T_Mouse_Left_Key_Dark.T_Mouse_Left_Key_Dark")
            (Variables|Default|Set正在显示鼠标 false)
            (CallFunction|显示提示)
            (elif (Variables|Default|Get正在隐藏鼠标)
              (Rendering|SetVisibility (Variables|Default|GetWidget) false false)
              (Rendering|SetVisibility (Variables|Default|GetTips%20Statcic%20Mesh) true true)
              (CallFunction|更新图标 "/Game/PlayerCharacter/Texture/圆形.圆形")
              (Variables|Default|Set正在隐藏鼠标 false)
              (CallFunction|显示提示))))))))

(event Custom|隐藏提示
  ;[1 0 0 0.5] 提示UI 的缩放动画时间轴
  (bind (_direction _新建轨道_0) (Timeline|时间轴 Reverse)
    (:Update
      (Transformation|SetRelativeScale3D (Variables|Default|GetTips%20Statcic%20Mesh) (Math|Vector|Lerp(Vector) "0, 0, 0" (Variables|Default|Get提示控件默认缩放) _新建轨道_0)))
    (:Finished
      (switch Utilities|FlowControl|Switch|SwitchonETimelineDirection _direction
        (:Forward
          (Variables|Default|Set同步提示 true))
        (:Backward
          (Variables|Default|Set同步提示 false)
          (if (Variables|Default|Get正在显示鼠标)
            (Rendering|SetVisibility (Variables|Default|GetWidget) true true)
            (Rendering|SetVisibility (Variables|Default|GetTips%20Statcic%20Mesh) false false)
            (CallFunction|更新图标 "/Game/PlayerCharacter/Texture/T_Mouse_Left_Key_Dark.T_Mouse_Left_Key_Dark")
            (Variables|Default|Set正在显示鼠标 false)
            (CallFunction|显示提示)
            (elif (Variables|Default|Get正在隐藏鼠标)
              (Rendering|SetVisibility (Variables|Default|GetWidget) false false)
              (Rendering|SetVisibility (Variables|Default|GetTips%20Statcic%20Mesh) true true)
              (CallFunction|更新图标 "/Game/PlayerCharacter/Texture/圆形.圆形")
              (Variables|Default|Set正在隐藏鼠标 false)
              (CallFunction|显示提示))))))))

(event EventBeginPlay
  (Variables|Default|Set提示控件默认缩放 (Variables|/Script/Engine.SceneComponent|GetRelativeScale3D (Variables|Default|GetTips%20Statcic%20Mesh)))
  (Rendering|SetVisibility (Variables|Default|GetWidget) false false)
  (if (Variables|Default|Get拥有默认音效)
    (CallFunction|生成音效)))

(event Collision|EventActorBeginOverlap
  (params (OtherActor :type Actor%20Object%20Reference)))

(event EventTick
  (params (DeltaSeconds :type Float%20%28single-precision%29))
  (if (Variables|Default|Get同步提示)
    (Transformation|SetWorldRotation (Variables|Default|GetWidget) (Math|Rotator|MakeRotator 0.0 0.0 (.Yaw (Math|Rotator|BreakRotator (Math|Rotator|FindLookatRotation (Transformation|GetWorldLocation (Variables|Default|GetWidget)) (Transformation|GetActorLocation (Game|Player|GetPlayerPawn 0)))))) false false)))

(fn ConstructionScript
  (Transformation|SetRelativeLocation (Variables|Default|GetTips%20Statcic%20Mesh) (Variables|Default|GetWidget%20Location) false false)
  (Transformation|SetRelativeTransform (Variables|Default|GetWidget1) (Variables|Default|Get物品内容变换) false false)
  (Components|StaticMesh|SetStaticMesh (Variables|Default|GetStaticMesh) (Variables|Default|Get物品模型))
  (Transformation|SetRelativeLocation (Variables|Default|GetSound%20Location%20Cmp) (Variables|Default|GetSound%20Location) false false))

(fn 更新图标
  (params (图像 :type Texture%202D%20Object%20Reference))
  (bind _aswbp_tips_widget (Utilities|Casting|CastToWBP_TipsWidget (UserInterface|GetWidget (Variables|Default|GetWidget))))
  (Default|更新图标 _aswbp_tips_widget 图像))

(fn 生成音效
  (bind _returnvalue (Game|SpawnActorfromClass "/Game/PlayerCharacter/Blueprints/BP_Ligst.BP_Ligst_C" (Math|Transform|MakeTransform (Transformation|GetWorldLocation (Variables|Default|GetSound%20Location%20Cmp))) "AlwaysSpawn" "MultiplyWithRoot" 0 (Variables|Default|Get音效) 0))
  (Variables|Default|Set音效对象 _returnvalue))