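; BP_WorldChanger is a sphere-mask volume that switches "WorldChange"-tagged actors between inside-only and outside-only states.
; Overlaps toggle their Pawn/Camera collision and shadows, with initial collision set on BeginPlay.
; Tick writes location, scale and an active flag to ID-suffixed Material Parameter Collection entries.
; Optional multi-sphere mode resolves priority through BP_MultiSpheremask_Manager and component tags; event 消失 (disappear) shrinks the sphere, then destroys it.
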(event Custom|消失
  (Variables|Default|Set初始大小 (Transformation|GetActorScale3D))
  (bind _新建轨道_0 (Timeline|时间轴 Play)
    (:Update
      (Transformation|SetActorScale3D (Math|Vector|Lerp(Vector) (Variables|Default|Get初始大小) "0, 0, 0" _新建轨道_0)))
    (:Finished
      (Actor|DestroyActor))))

(event EventBeginPlay
  (Utilities|FlowControl|Sequence
    (:then_0
      ;[1 0.08938 0] On start (if multiple sphere mask the manager is required in the lvl)
      (if (Variables|Default|GetMultipleSphereMask)
        (bind _returnvalue (Actor|GetActorOfClass "/Game/SphereMask/Multiple_Spheremask_Map/Blueprints/BP_MultiSpheremask_Manager.BP_MultiSpheremask_Manager_C"))
        (Variables|Default|SetMultiSphereManager _returnvalue)))
    (:then_1
      ;[1 1 1] Setup collision into trigger when hidden ands outside of the sphere at the beginning
      (bind _outactors (Actor|GetAllActorswithTag "WorldChange"))
      (for _array_element _outactors
        (if (not (Collision|IsOverlappingActor _array_element :!class /Script/Engine.Actor))
          (if (Actor|ActorHasTag _array_element (Variables|Default|GetTag%20Out%20Mask))
            (for _array_element_2 (Actor|GetComponentsByClass _array_element "/Script/Engine.PrimitiveComponent")
              (Collision|SetCollisionResponsetoChannel _array_element_2 "ECC_Pawn" "ECR_Block")
              (Collision|SetCollisionResponsetoChannel _array_element_2 "ECC_Camera" "ECR_Block"))
            (else
              (for _array_element_3 (Actor|GetComponentsByClass _array_element "/Script/Engine.PrimitiveComponent")
                (Collision|SetCollisionResponsetoChannel _array_element_3 "ECC_Pawn" "ECR_Ignore")
                (Collision|SetCollisionResponsetoChannel _array_element_3 "ECC_Camera" "ECR_Ignore")))))))))

(event Collision|EventActorBeginOverlap
  (params (OtherActor :type Actor%20Object%20Reference))
  (bind _returnvalue (Actor|GetComponentsByClass OtherActor "/Script/Engine.PrimitiveComponent"))
  ;[0.06447 0.1855 1 1 30] Start collision with a item affected by a Spheremask
  ;;[0.2031 0.2031 0.2031] Detect if the item is affected by a sphere
  (if (Actor|ActorHasTag OtherActor "WorldChange")
    ;;[0.2031 0.2031 0.2031] Detect if the item is affected by this sphere
    (if (Actor|ActorHasTag OtherActor (Variables|Default|GetTag%20In%20Mask))
      ;;[0.2031 0.2031 0.2031] Overlap Item with the right sphere tag (Item collision and shadow apear)
      (for _array_element _returnvalue
        (if (Variables|Default|GetMultipleSphereMask)
          ;;;[0.02851 0.1927 0.01945] Multiple Sphere Mask (need more tag system for priority when a sphere overlap another)
          (if (Components|ComponentHasTag _array_element (Variables|Default|GetOverrideTag))
            _
            (else
              (Collision|SetCollisionResponsetoChannel _array_element "ECC_Pawn" "ECR_Block")
              (Collision|SetCollisionResponsetoChannel _array_element "ECC_Camera" "ECR_Block")
              (Rendering|SetCastShadow _array_element true)))
          (Utilities|Array|Insert (Variables|/Script/Engine.ActorComponent|GetComponentTags _array_element) (Variables|Default|GetGoodSphereTag) (Utilities|Array|Length (Variables|/Script/Engine.ActorComponent|GetComponentTags _array_element)))
          (else
            ;;;[0.02851 0.1927 0.01945] Single Sphere mask
            (Collision|SetCollisionResponsetoChannel _array_element "ECC_Pawn" "ECR_Block")
            (Collision|SetCollisionResponsetoChannel _array_element "ECC_Camera" "ECR_Block")
            (Rendering|SetCastShadow _array_element true))))
      (else
        ;;[0.2031 0.2031 0.2031] Detect if the item should be only outside of all sphere
        (if (Actor|ActorHasTag OtherActor (Variables|Default|GetTag%20Out%20Mask))
          ;;[0.2031 0.2031 0.2031] Overlap Item outside of all the spheremask and have to diseapear
          (for _array_element_2 _returnvalue
            (Collision|SetCollisionResponsetoChannel _array_element_2 "ECC_Pawn" "ECR_Ignore")
            (Collision|SetCollisionResponsetoChannel _array_element_2 "ECC_Camera" "ECR_Ignore")
            (Rendering|SetCastShadow _array_element_2 false))
          (elif (Variables|Default|GetMultipleSphereMask)
            ;;[0.1406 0.1406 0.1406] Overlap a item already overlaped by his spheremask
            ;;;[0.02851 0.1927 0.01945] Ask To Manager if we override the item (if the sphere has the priority)
            (for _array_element_3 _returnvalue
              (Class|BPIMultiSpheremaskInterface|AskOverride(Message) (Variables|Default|GetMultiSphereManager) _array_element_3 self))))))))

(event EventTick
  (params (DeltaSeconds :type Float%20%28single-precision%29))
  (bind _worldspheredatas (Variables|Default|GetWorldSphereDatas))
  ;[0.1125 0.2193 0.7448 1 25] Setup Parametter collection : Based on Sphere ID number (send Location/Scale/Mask to the sphere mask)
  ;;[0.1406 0.1406 0.1406] setup Material collection parametter Location Example : VariableName+idSphere = Location0
  (Rendering|Material|SetVectorParameterValue _worldspheredatas (Utilities|String|StringToName (Utilities|String|Append (Variables|Default|GetParameter%20Name%20Location) (Utilities|String|ToString(Integer) (Variables|Default|GetIDSphere)))) (Math|Conversions|ToLinearColor(Vector) (Transformation|GetActorLocation)) :!class /Script/Engine.KismetMaterialLibrary)
  ;;[0.1406 0.1406 0.1406] setup Material collection parametter Scale Example : VariableName+idSphere = Scale0
  (Rendering|Material|SetVectorParameterValue _worldspheredatas (Utilities|String|StringToName (Utilities|String|Append (Variables|Default|GetParameter%20Name%20Scale) (Utilities|String|ToString(Integer) (Variables|Default|GetIDSphere)))) (Math|Conversions|ToLinearColor(Vector) (Transformation|GetWorldScale (Variables|Default|GetBP_W_Reveal_A))) :!class /Script/Engine.KismetMaterialLibrary)
  ;;[0.1406 0.1406 0.1406] setup Material collection parametter World Example : VariableName+idSphere = World0
  (Rendering|Material|SetScalarParameterValue _worldspheredatas (Utilities|String|StringToName (Utilities|String|Append (Variables|Default|GetWorld) (Utilities|String|ToString(Integer) (Variables|Default|GetIDSphere)))) 1.0 :!class /Script/Engine.KismetMaterialLibrary))

(event EventAnswerHasBeenOverride
  (params (OverrideStatus :type Boolean) (item :type Primitive%20Component%20Object%20Reference))
  ;[0.06447 0.1855 1] End collision with a item affected by a Spheremask
  ;;[0.2031 0.2031 0.2031] Overlap a item already overlaped by his spheremask
  ;;;[0.02851 0.1927 0.01945] We get the answer from the manager and make action
  (if OverrideStatus
    (if (Components|ComponentHasTag item (Variables|Default|GetGoodSphereTag))
      (Collision|SetCollisionResponsetoChannel item "ECC_Pawn" "ECR_Block")
      (Collision|SetCollisionResponsetoChannel item "ECC_Camera" "ECR_Block")
      (Rendering|SetCastShadow item true))))

(event Collision|EventActorEndOverlap
  (params (OtherActor :type Actor%20Object%20Reference))
  (bind _returnvalue (Actor|GetComponentsByClass OtherActor "/Script/Engine.PrimitiveComponent"))
  (bind _goodspheretag (Variables|Default|GetGoodSphereTag))
  ;[0.06447 0.1855 1] End collision with a item affected by a Spheremask
  ;;[0.2031 0.2031 0.2031] Detect if the item is affected by a sphere
  (if (Actor|ActorHasTag OtherActor "WorldChange")
    ;;[0.2031 0.2031 0.2031] Detect if the item is affected by this sphere
    (if (Actor|ActorHasTag OtherActor (Variables|Default|GetTag%20In%20Mask))
      ;;[0.2031 0.2031 0.2031] Overlap good sphere
      (for _array_element _returnvalue
        ;;;[0.02851 0.1927 0.01945] Hide the item (colision and shadow)
        (Collision|SetCollisionResponsetoChannel _array_element "ECC_Pawn" "ECR_Ignore")
        (Collision|SetCollisionResponsetoChannel _array_element "ECC_Camera" "ECR_Ignore")
        (Rendering|SetCastShadow _array_element false)
        ;;;[0.02851 0.1927 0.01945] If multiple sphere mask (tag manipulation)
        (if (Variables|Default|GetMultipleSphereMask)
          (if (Components|ComponentHasTag _array_element _goodspheretag)
            (Utilities|Array|RemoveItem (Variables|/Script/Engine.ActorComponent|GetComponentTags _array_element) _goodspheretag))))
      (else
        ;;[0.2031 0.2031 0.2031] Detect if the item should be only outside of all sphere
        (if (Actor|ActorHasTag OtherActor (Variables|Default|GetTag%20Out%20Mask))
          ;;[0.2031 0.2031 0.2031] Outside the sphere
          (for _array_element_2 _returnvalue
            (if (Utilities|Array|IsEmpty (Collision|GetOverlappingActors _array_element_2 "BP_WorldChanger_C" :!class /Script/Engine.PrimitiveComponent))
              (Collision|SetCollisionResponsetoChannel _array_element_2 "ECC_Pawn" "ECR_Block")
              (Collision|SetCollisionResponsetoChannel _array_element_2 "ECC_Camera" "ECR_Block")
              (Rendering|SetCastShadow _array_element_2 true)))
          (elif (Variables|Default|GetMultipleSphereMask)
            ;;[0.2031 0.2031 0.2031] Overlap a item already overlaped by his spheremask
            ;;;[0.02851 0.1927 0.01945] Ask To Manager if the item has been override (to not show the item if a higher priority sphere is already colliding)
            (for _array_element_3 _returnvalue
              (Default|AskHasBeenOverride (Variables|Default|GetMultiSphereManager) _array_element_3 self))))))))

(event EventAnswerOverride
  (params (Overriden :type Boolean) (item%20to%20override :type Primitive%20Component%20Object%20Reference))
  ;[0.06447 0.1855 1 1 30] Start collision with a item affected by a Spheremask
  ;;[0.1406 0.1406 0.1406] Overlap a item already overlaped by his spheremask
  ;;;[0.02851 0.1927 0.01945] We get the answer from the manager and make action
  (if Overriden
    (Collision|SetCollisionResponsetoChannel item%20to%20override "ECC_Pawn" "ECR_Ignore")
    (Collision|SetCollisionResponsetoChannel item%20to%20override "ECC_Camera" "ECR_Ignore")
    (Rendering|SetCastShadow item%20to%20override false)))

(fn ConstructionScript)