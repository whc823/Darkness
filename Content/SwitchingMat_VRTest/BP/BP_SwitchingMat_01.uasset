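; BP_SwitchingMat_01 is a test actor that drives a location-based material switch or dissolve on Cube, Cone and Sphere meshes.
; The construction script creates one dynamic instance of MI_SwitchingMatTest01 from Cube, shares it with Cone and Sphere, and seeds "Dissolve Location" from the Location component's relative position.
; Each tick feeds that component's world position and bounds radius into the material's probe-sphere parameters (探测球位置, 探测球半径).
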(event EventTick
  (params (DeltaSeconds :type Float%20%28single-precision%29))
  (Rendering|Material|SetVectorParameterValue (Variables|Default|GetDynamicMaterial) "探测球位置" (Math|Conversions|ToLinearColor(Vector) (Transformation|GetWorldLocation (Variables|Default|GetLocation))) :!class /Script/Engine.MaterialInstanceDynamic)
  (Rendering|Material|SetScalarParameterValue (Variables|Default|GetDynamicMaterial) "探测球半径" (.SphereRadius (Collision|GetComponentBounds (Variables|Default|GetLocation))) :!class /Script/Engine.MaterialInstanceDynamic))

(fn ConstructionScript
  (bind _returnvalue (Rendering|Material|CreateDynamicMaterialInstance (Variables|Default|GetCube) 0 "/Game/SwitchingMat_VRTest/Material/MI_SwitchingMatTest01.MI_SwitchingMatTest01" "None" :!class /Script/Engine.PrimitiveComponent))
  (bind _output_get (Variables|Default|SetDynamicMaterial _returnvalue))
  (Rendering|Material|SetMaterial (Variables|Default|GetCone) 0 _output_get)
  (Rendering|Material|SetVectorParameterValue _output_get "Dissolve Location" (Math|Conversions|ToLinearColor(Vector) (Variables|/Script/Engine.SceneComponent|GetRelativeLocation (Variables|Default|GetLocation))) :!class /Script/Engine.MaterialInstanceDynamic))